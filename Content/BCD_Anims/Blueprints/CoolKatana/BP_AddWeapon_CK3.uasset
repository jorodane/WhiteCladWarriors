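; Helper Blueprint that equips every Skeletal Mesh Actor in the level with a katana when play begins.
; On BeginPlay it gathers all SkeletalMeshActors and spawns a movable, collision-free StaticMeshActor using SM_Katana for each valid one.
; Each katana is attached to its skeletal actor at the S_KatanaR socket, snapping location and rotation while keeping relative scale.
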(event EventBeginPlay
  (bind _outactors (Actor|GetAllActorsOfClass "/Script/Engine.SkeletalMeshActor"))
  (if (Utilities|Array|IsValidIndex _outactors)
    (for _array_element _outactors
      (Utilities|IsValid _array_element
        (:Is%20Valid
          ;[1 1 1] Add Weapon
          (bind _returnvalue (Game|SpawnActorfromClass "/Script/Engine.StaticMeshActor" (Math|Transform|MakeTransform "0, 0, 0" "0, 0, 0" "1.000000,1.000000,1.000000") "AlwaysSpawn" "MultiplyWithRoot" 0 0))
          (Transformation|SetMobility _returnvalue "Movable")
          (Collision|SetActorEnableCollision _returnvalue false)
          (Components|StaticMesh|SetStaticMesh (Variables|/Script/Engine.StaticMeshActor|GetStaticMeshComponent _returnvalue) "/Game/BCD_Anims/Weapons/CoolKatana/SM_Katana.SM_Katana")
          (Transformation|AttachActorToActor _returnvalue _array_element "S_KatanaR" "SnapToTarget" "SnapToTarget" "KeepRelative" true))))))

(fn ConstructionScript)