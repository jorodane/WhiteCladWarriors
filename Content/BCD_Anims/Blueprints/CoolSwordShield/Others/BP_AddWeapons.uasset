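; BP_AddWeapons is a helper actor that equips skeletal mesh actors in the level with katanas and shields on BeginPlay, likely for an animation showcase.
; It scans every SkeletalMeshActor, skips names containing "throw", "arm" or "with", and picks a big or regular shield by checking for "BigShield" in the display name.
; AttachWeaponsToCharacter spawns a movable, collision-free StaticMeshActor per weapon and snaps it to the given socket.
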(event EventBeginPlay
  (bind _outactors (Actor|GetAllActorsOfClass "/Script/Engine.SkeletalMeshActor"))
  (if (Utilities|Array|IsValidIndex _outactors)
    (for _array_element _outactors
      (Utilities|IsValid _array_element
        (:Is%20Valid
          (if (Math|Boolean|ANDBoolean (not (Utilities|String|Contains (Utilities|GetDisplayName _array_element) "throw")) (not (Utilities|String|Contains (Utilities|GetDisplayName _array_element) "arm")) (not (Utilities|String|Contains (Utilities|GetDisplayName _array_element) "with")))
            (CallFunction|AttachWeaponstoCharacter _array_element "S_KatanaR" "/Game/BCD_Anims/Weapons/CoolSwordShield/SM_Katana.SM_Katana")
            (if (Utilities|String|Contains (Utilities|GetDisplayName _array_element) "BigShield")
              (CallFunction|AttachWeaponstoCharacter _array_element "S_BigShieldL" "/Game/BCD_Anims/Weapons/CoolSwordShield/SM_BigShield.SM_BigShield")
              (else
                (CallFunction|AttachWeaponstoCharacter _array_element "S_ShieldL" "/Game/BCD_Anims/Weapons/CoolSwordShield/SM_Shield.SM_Shield")))))))))

(fn ConstructionScript)

(fn AttachWeaponstoCharacter
  (params (ParentActor :type Actor%20Object%20Reference) (SocketName :type Name) (NewMesh :type Static%20Mesh%20Object%20Reference))
  ;[1 1 1] Add Weapon
  (bind _returnvalue (Game|SpawnActorfromClass "/Script/Engine.StaticMeshActor" (Math|Transform|MakeTransform "0, 0, 0" "0, 0, 0" "1.000000,1.000000,1.000000") "AlwaysSpawn" "MultiplyWithRoot" 0 0))
  (Transformation|SetMobility _returnvalue "Movable")
  (Collision|SetActorEnableCollision _returnvalue false)
  (Components|StaticMesh|SetStaticMesh (Variables|/Script/Engine.StaticMeshActor|GetStaticMeshComponent _returnvalue) NewMesh)
  (Transformation|AttachActorToActor _returnvalue ParentActor SocketName "SnapToTarget" "SnapToTarget" "KeepRelative" true))