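; BP_AddWeapons_CTS is a helper actor that equips every SkeletalMeshActor in the level with twin swords when play begins, in the CoolTwinSword animation content.
; BeginPlay gathers those actors and calls AttachWeaponsToCharacter for the left and right sword sockets.
; That function spawns a movable, collision-free StaticMeshActor with the sword mesh and snaps it to the socket's location and rotation, keeping relative scale.
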(event EventBeginPlay
  (bind _outactors (Actor|GetAllActorsOfClass "/Script/Engine.SkeletalMeshActor"))
  (if (Utilities|Array|IsValidIndex _outactors)
    (for _array_element _outactors
      (Utilities|IsValid _array_element
        (:Is%20Valid
          (CallFunction|AttachWeaponstoCharacter _array_element "S_TwinSwordL" "/Game/BCD_Anims/Weapons/CoolTwinSword/S_TwinSword.S_TwinSword")
          (CallFunction|AttachWeaponstoCharacter _array_element "S_TwinSwordR" "/Game/BCD_Anims/Weapons/CoolTwinSword/S_TwinSword.S_TwinSword"))))))

(fn ConstructionScript)

(fn AttachWeaponstoCharacter
  (params (ParentActor :type Actor%20Object%20Reference) (SocketName :type Name) (NewMesh :type Static%20Mesh%20Object%20Reference))
  ;[1 1 1] Add Weapon
  (bind _returnvalue (Game|SpawnActorfromClass "/Script/Engine.StaticMeshActor" (Math|Transform|MakeTransform "0, 0, 0" "0, 0, 0" "1.000000,1.000000,1.000000") "AlwaysSpawn" "MultiplyWithRoot" 0 0))
  (Transformation|SetMobility _returnvalue "Movable")
  (Collision|SetActorEnableCollision _returnvalue false)
  (Components|StaticMesh|SetStaticMesh (Variables|/Script/Engine.StaticMeshActor|GetStaticMeshComponent _returnvalue) NewMesh)
  (Transformation|AttachActorToActor _returnvalue ParentActor SocketName "SnapToTarget" "SnapToTarget" "KeepRelative" true))