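; BP_AddWeapons is a helper actor that puts knives in the hands of animation showcase characters at BeginPlay.
; It scans all SkeletalMeshActors in the level and keeps those whose display name contains "Run" or "Walk".
; For each, it spawns collisionless, movable StaticMeshActors with the SM_CoolKnife mesh and snaps them to the left and right knife sockets.
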(event EventBeginPlay
  (bind _outactors (Actor|GetAllActorsOfClass "/Script/Engine.SkeletalMeshActor"))
  (if (Utilities|Array|IsValidIndex _outactors)
    (for _array_element _outactors
      (Utilities|IsValid _array_element
        (:Is%20Valid
          (if (or (Utilities|String|Contains (Utilities|GetDisplayName _array_element) "Run") (Utilities|String|Contains (Utilities|GetDisplayName _array_element) "Walk"))
            (CallFunction|AttachWeaponstoCharacter _array_element "S_KnifeL")
            (CallFunction|AttachWeaponstoCharacter _array_element "S_KnifeR")))))))

(fn ConstructionScript)

(fn AttachWeaponstoCharacter
  (params (ParentActor :type Actor%20Object%20Reference) (SocketName :type Name))
  ;[1 1 1] Add Weapon
  (bind _returnvalue (Game|SpawnActorfromClass "/Script/Engine.StaticMeshActor" (Math|Transform|MakeTransform "0, 0, 0" "0, 0, 0" "1.000000,1.000000,1.000000") "AlwaysSpawn" "MultiplyWithRoot" 0 0))
  (Transformation|SetMobility _returnvalue "Movable")
  (Collision|SetActorEnableCollision _returnvalue false)
  (Components|StaticMesh|SetStaticMesh (Variables|/Script/Engine.StaticMeshActor|GetStaticMeshComponent _returnvalue) "/Game/BCD_Anims/Weapons/CoolThrowing/SM_CoolKnife.SM_CoolKnife")
  (Transformation|AttachActorToActor _returnvalue ParentActor SocketName "SnapToTarget" "SnapToTarget" "KeepRelative" true))