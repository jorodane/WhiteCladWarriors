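; Monster spawn component that hands out monster actors at requested locations, apparently on top of an instance queue defined outside this file.
; SpawnInstance creates an actor from TemplateClass, always spawning regardless of collision.
; SpawnMonster takes an instance via DequeueInstance and, if valid, teleports it to the wanted location without sweep and returns it.
; BeginPlay and Tick are unused.
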(event EventBeginPlay)

(event EventTick
  (params (DeltaSeconds :type Float%20%28single-precision%29)))

(fn SpawnInstance
  (bind _templateclass (Variables|Default|GetTemplateClass)
    (:then
      (bind _returnvalue (Game|SpawnActorfromClass _templateclass (Math|Transform|MakeTransform "0, 0, 0" "0, 0, 0" "1.000000,1.000000,1.000000") "AlwaysSpawn" "MultiplyWithRoot" 0 0))
      (return _returnvalue))
    (:else)))

(fn SpawnMonster
  (params (WantLocation :type Vector))
  (bind _returnvalue (Class|PoolComponent|DequeueInstance))
  (Utilities|IsValid _returnvalue
    (:Is%20Valid
      (bind _output_get (LocalVariables|SetResult _returnvalue))
      (Transformation|SetActorLocation _output_get WantLocation false true)
      (return (LocalVariables|GetResult)))
    (:Is%20Not%20Valid
      (return 0))))