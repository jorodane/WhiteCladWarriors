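; Health component that supplies an HP readout to connected info widgets.
; When a widget connects, it sends the current and max values, an "HP :" label and a green bar color scheme through widget message calls.
; CurrentValue and MaxValue are not changed by any live logic here; an unconnected chain would add health and refresh every "HP" widget.
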(event EventBeginPlay)

(event EventTick
  (params (DeltaSeconds :type Float%20%28single-precision%29)))

(event EventOnConnectInfoWidget
  (params (TargetWidget :type Widget%20Object%20Reference) (ClaimedTag :type Name :default "None"))
  (Class|ContainFloat2Value|SetFloat2(Message) TargetWidget (Variables|Default|GetCurrentValue) (Variables|Default|GetMaxValue))
  (Class|ContainTagValue|SetTag(Message) TargetWidget (Utilities|Text|ToText(String) "HP : "))
  (Class|ContainBackgroundColorPaint|SetBackgroundColor(Message) TargetWidget "(R=0.001097,G=0.015625,B=0.000743,A=1.000000)")
  (Class|ContainContentColorPaint|SetContentColor(Message) TargetWidget "(R=1.000000,G=1.000000,B=1.000000,A=1.000000)")
  (Class|ContainFillColorPaint|SetFillColor(Message) TargetWidget "(R=0.035328,G=0.303125,B=0.044371,A=1.000000)"))