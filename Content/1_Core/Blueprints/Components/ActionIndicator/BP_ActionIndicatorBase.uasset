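; Base action indicator that shows a ground decal at the mouse's terrain position, oriented toward the owning operator's hero.
; BeginPlay pre-spawns pools of arrow, circle and quad shower actors through ShowerCreate and ShowerPush.
; InputClaim toggles the decal's visibility by claim validity, and Tick redraws it at a fixed size while active.
; The pooled showers are not used in this graph, and an alternative hero-to-mouse line draw is disconnected.
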(event EventBeginPlay
  (for _index (range 1 (Variables|Default|GetIndicatorPoolCount))
    (CallFunction|ShowerCreate "/Game/1_Core/Blueprints/Actors/ActionIndicatorShower/BP_AIS_Arrow.BP_AIS_Arrow_C" "Arrow" true)
    (CallFunction|ShowerCreate "/Game/1_Core/Blueprints/Actors/ActionIndicatorShower/BP_AIS_Circle.BP_AIS_Circle_C" "Circle" true)
    (CallFunction|ShowerCreate "/Game/1_Core/Blueprints/Actors/ActionIndicatorShower/BP_AIS_Quad.BP_AIS_Quad_C" "Quad" true)))

(event EventTick
  (params (DeltaSeconds :type Float%20%28single-precision%29))
  (Variables|Default|GetbIsActivated
    (:then
      (bind _owneroperator (Variables|Default|GetOwnerOperator)
        (:then
          (Default|Drawfrom (Variables|Default|GetDecal) (.mouseterrainposition (Class|Operator|GetInputPackage _owneroperator)) 3e+02 1e+02 (Math|Rotator|FindLookatRotation (.mouseterrainposition (Class|Operator|GetInputPackage _owneroperator)) (Transformation|GetActorLocation (Variables|/Script/WhiteCladWarriors.Operator|GetHeroActor _owneroperator)))))
        (:else)))
    (:else)))

(event EventInputClaim
  (params (NewClaim :type Input%20Claim%20Structure%20%28by%20ref%29) (ValidClaim :type Boolean))
  (if ValidClaim
    (Class|ActionIndicatorBase|SetVisible)
    (else
      (Class|ActionIndicatorBase|SetInvisible))))

(event EventSetVisible
  (Variables|Default|SetbIsActivated true)
  (Rendering|SetActorHiddenInGame (Variables|Default|GetDecal) (not (Variables|Default|GetbIsActivated))))

(event EventSetInvisible
  (Variables|Default|SetbIsActivated false)
  (Rendering|SetActorHiddenInGame (Variables|Default|GetDecal) (not (Variables|Default|GetbIsActivated))))

(fn ShowerCreate
  (params (WantClass :type Action%20Indicator%20Shower%20Base%20Class%20Reference) (WantType :type EInputIndicatorType%20Enum :default "Arrow") (AddToQueue :type Boolean))
  (LocalVariables|SetTargetClass WantClass)
  (LocalVariables|SetTargetType WantType)
  (LocalVariables|SetNeedToAdd AddToQueue)
  (Utilities|FlowControl|Sequence
    (:then_0
      (bind _returnvalue (Game|SpawnActorfromClass (LocalVariables|GetTargetClass) (Math|Transform|MakeTransform "0, 0, 0" "0, 0, 0" "1.000000,1.000000,1.000000") "Undefined" "MultiplyWithRoot" 0 (Variables|Default|GetOwnerOperator)))
      (LocalVariables|SetInstance _returnvalue))
    (:then_1
      (bind _instance (LocalVariables|GetInstance)
        (:then
          (if (LocalVariables|GetNeedToAdd)
            (Class|ActionIndicatorBase|ShowerPush (LocalVariables|GetTargetType) _instance)))
        (:else)))
    (:then_2
      (return (LocalVariables|GetInstance)))))