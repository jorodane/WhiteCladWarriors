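; Status component for a fillable current/max value on a unit, such as a health-style bar.
; On BeginPlay it registers with its owner unit under its tag, then declares ordered UI widget claims instead of creating widgets directly.
; It claims a detailed bar with a child text widget and a simple fill bar.
; Connect and update events send values and colors to the bars through messages.
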(event Custom|ValueUpdate
  (params (NewWidget :type Generic%20Widget%20Base%20Object%20Reference))
  (Class|ContainFloat2Value|SetFloat2(Message) NewWidget (Variables|Default|GetCurrentValue) (Variables|Default|GetMaxValue)))

(event Custom|BarConnect
  (params (NewParam :type Generic%20Widget%20Base%20Object%20Reference))
  (CallFunction|ValueUpdate NewParam)
  (Class|ContainBackgroundColorPaint|SetBackgroundColor(Message) NewParam (Variables|Default|GetBackgroundColor))
  (Class|ContainFillColorPaint|SetFillColor(Message) NewParam (Variables|Default|GetFillColor)))

(event EventBeginPlay
  (|CallParentFunction)
  (bind _resultunit (Class|UnitComponentBase|TryGetOwnerUnit)
    (:True
      (Class|UnitMainComponent|AddFillValue _resultunit (Variables|Default|GetTag) self)
      (CallFunction|CreateWidgetClaimers))))

(fn BroadcastDirty
  (bind _returnvalue (|CallParentFunction))
  (return _returnvalue))

(fn CreateWidgetClaimers
  (bind _returnvalue (Utilities|CreateWidgetClaimwithUpdater (Variables|Default|GetTextWidgetName) 0 (EventDispatchers|CreateEvent :!event Custom|ValueUpdate)))
  (Variables|/Script/WhiteCladWarriors.GenericWidgetClaim|SetWidgetTransform _returnvalue (Utilities|Map|MakeMap "VerticalAlignment" 0.5))
  (bind _returnvalue_2 (Utilities|CreateOrderedWidgetClaimwithEvent (Variables|Default|GetUIOrder) "HP_Type1" (Utilities|Array|MakeArray _returnvalue) (EventDispatchers|CreateEvent :!event Custom|BarConnect) (EventDispatchers|CreateEvent :!event Custom|ValueUpdate)))
  (bind _output_get (Variables|Default|SetDetailBar _returnvalue_2))
  (Variables|/Script/WhiteCladWarriors.GenericWidgetClaim|SetWidgetTransform _output_get (Utilities|Map|MakeMap "VerticalSize" (Variables|Default|GetDetailHeight)))
  (bind _returnvalue_3 (Utilities|CreateOrderedWidgetClaimwithEvent (Variables|Default|GetUIOrder) "FillBar" 0 (EventDispatchers|CreateEvent :!event Custom|BarConnect) (EventDispatchers|CreateEvent :!event Custom|ValueUpdate)))
  (bind _output_get_2 (Variables|Default|SetSimpleBar _returnvalue_3))
  (Variables|/Script/WhiteCladWarriors.GenericWidgetClaim|SetWidgetTransform _output_get_2 (Utilities|Map|MakeMap "VerticalSize" (Variables|Default|GetSimpleHeight))))