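; BP_LevelComponent is a status component that tracks a unit's progress toward its next level.
; The level lives on the owner unit as a tagged float, set to a starting value on connect.
; A full bar resets to zero, raises its maximum by 25% and adds a level, while overflow is re-added.
; Its widget shows level, class name and percent, offering the detail bar for owned units or when no owner is found.
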(event EventValueUpdate
  (params (NewWidget :type Generic%20Widget%20Base%20Object%20Reference))
  (|CallParentFunction NewWidget)
  (bind _resultunit (Class|UnitComponentBase|TryGetOwnerUnit)
    (:True
      (Class|ContainTextValue|SetText(Message) NewWidget (Utilities|Text|FormatText "LV.{Level} {ClassName} ({Percent}%)" (Variables|/Script/WhiteCladWarriors.UnitMainComponent|GetClassName _resultunit) (Utilities|Text|ToText(Float) (* (Class|FillableValueComponent|GetPercent) 1e+02) "HalfToEven" false true 1 324 0 1) (Class|UnitMainComponent|GetFloatValue _resultunit (Variables|Default|GetLevelTag) 1.0))))
    (:False
      (Class|ContainTextValue|SetText(Message) NewWidget (Utilities|Text|FormatText "LV.{Level} ({Percent}%)" (Class|FillableValueComponent|GetPercent) (Class|UnitMainComponent|GetFloatValue _resultunit (Variables|Default|GetLevelTag) 1.0))))))

(fn GetInfoWidget
  (params (WantType :type EInfoWidgetType%20Enum :default "Minimal") (Operator :type Operator%20Object%20Reference))
  (bind _resultunit (Class|UnitComponentBase|TryGetOwnerUnit)
    (:True
      (if (Utilities|Enum|Equal(Enum) (Class|UnitMainComponent|GetAllyTypefromOperator _resultunit Operator) "Own")
        _
        (else
          (return 0))))
    (:False
      _))
  (return (Utilities|Array|MakeArray (Utilities|Select :Index WantType :Minimal 0 :Hover 0 :Detail (Variables|Default|GetDetailBar) :Inspector 0))))

(fn OnConnectUnit
  (params (NewUnit :type Unit%20Main%20Component%20Object%20Reference))
  (|CallParentFunction NewUnit)
  (Class|UnitMainComponent|SetFloatValue NewUnit (Variables|Default|GetLevelTag) (Variables|Default|GetStartLevel)))

(fn OnValueFull
  (|CallParentFunction)
  (bind _returnvalue (Class|FillableValueComponent|SetValue 0.0 (* (Variables|Default|GetMaxValue) 1.25)))
  (CallFunction|LevelUp 1)
  (return _returnvalue))

(fn LevelUp
  (params (Amount :type Integer))
  (bind _resultunit (Class|UnitComponentBase|TryGetOwnerUnit)
    (:True
      (Class|UnitMainComponent|AddFloatValue _resultunit (Variables|Default|GetLevelTag) (Math|Conversions|ToFloat(Integer) Amount)))))

(fn OnValueOverflow
  (params (AbsoluteValue :type Float%20%28single-precision%29))
  (bind _returnvalue (Class|FillableValueComponent|AddValue AbsoluteValue))
  (return _returnvalue))