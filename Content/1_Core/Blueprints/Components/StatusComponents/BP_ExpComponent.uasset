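; BP_ExpComponent is a status component that presents experience (XP) as a bar in info widgets.
; When a widget connects, it pushes current and max values, an "XP :" tag and an amber-on-dark color scheme through message calls.
; GetInfoWidget supplies the detail bar for Hero and Detail views only, leaving the other view types empty.
; It holds no XP gain or leveling logic.
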(event EventBeginPlay)

(event EventOnConnectInfoWidget
  (params (NewType :type EInfoWidgetType%20Enum :default "Minimal") (TargetWidget :type Widget%20Object%20Reference) (ClaimedTag :type Name :default "None"))
  (Class|ContainFloat2Value|SetFloat2(Message) TargetWidget (Variables|Default|GetCurrentValue) (Variables|Default|GetMaxValue))
  (Class|ContainTagValue|SetTag(Message) TargetWidget (Utilities|Text|ToText(String) "XP : "))
  (Class|ContainBackgroundColorPaint|SetBackgroundColor(Message) TargetWidget "(R=0.119792,G=0.054715,B=0.000000,A=1.000000)")
  (Class|ContainContentColorPaint|SetContentColor(Message) TargetWidget "(R=1.000000,G=1.000000,B=1.000000,A=1.000000)")
  (Class|ContainFillColorPaint|SetFillColor(Message) TargetWidget "(R=0.657292,G=0.409931,B=0.000000,A=1.000000)"))

(fn GetInfoWidget
  (params (WantType :type EInfoWidgetType%20Enum :default "Minimal"))
  (bind _detailbar (Variables|Default|GetDetailBar))
  (return (Utilities|Select :Index WantType :Minimal 0 :Hover 0 :Hero _detailbar :Detail _detailbar :Inspector 0)))