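; Hero unit component that supplies hero UI widgets and rewards whoever kills the hero.
; On BeginPlay it builds ordered widget claims with updater callbacks: a name header for Hover and Detail info, plus a separately stored portrait claim.
; GetInfoWidget appends the list matching the requested info type to the parent's result.
; On death it grants the damage causer EXP, then Gold once that completes.
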(event Custom|NameUpdate
  (params (NewWidget :type Generic%20Widget%20Base%20Object%20Reference))
  (bind _returnvalue (Class|Selectable|GetSelectedName))
  (Class|ContainTextValue|SetText(Message) NewWidget _returnvalue))

(event Custom|ConstructWidgets
  (bind _returnvalue (Utilities|CreateOrderedWidgetClaimwithUpdater 50 "Text_Header" 0 (delegate Custom|NameUpdate)))
  (Variables|/Script/WhiteCladWarriors.GenericWidgetClaim|SetWidgetTransform _returnvalue (Utilities|Map|MakeMap "VerticalAlignment" 1.0))
  (Variables|Default|SetSimpleWidgets (Utilities|Array|MakeArray _returnvalue))
  (bind _returnvalue_2 (Utilities|CreateOrderedWidgetClaimwithUpdater 25 "Image" 0 (delegate Custom|UpdatePortrait)))
  (Variables|/Script/WhiteCladWarriors.GenericWidgetClaim|SetWidgetTransform _returnvalue_2 (Utilities|Map|MakeMap "Size" 4e+02 "AspectRatio" 0.77 "HorizontalAlignment" 0.0))
  (Variables|Default|SetDetailWidgets (Utilities|Array|MakeArray _returnvalue))
  (Variables|Default|SetHeroPortraitClaim _returnvalue_2))

(event Custom|UpdatePortrait
  (params (NewWidget :type Generic%20Widget%20Base%20Object%20Reference))
  (Class|ContainImageValue|SetImage(Message) NewWidget (Variables|Default|GetPortrait)))

(event EventBeginPlay
  (CallFunction|ConstructWidgets))

(event EventOnDie
  (params (LastAttackDamageInfo :type Damage%20Info%20Structure%20%28by%20ref%29) (LastDamageMap :type Map%20of%20Unit%20Main%20Component%20Object%20References%20to%20Reals) (LastTotalDamage :type Float%20%28single-precision%29))
  (Utilities|AddFillValueforDamageCauser "EXP" 6e+01
    (:Completed
      (Utilities|AddFloatValueforDamageCauser "Gold" 3e+02))))

(fn GetInfoWidget
  (params (WantType :type EInfoWidgetType%20Enum :default "Minimal") (Operator :type Operator%20Object%20Reference))
  (bind _output_get (LocalVariables|SetResult (|CallParentFunction WantType Operator)))
  (Utilities|Array|AppendArray _output_get (Utilities|Select :Index WantType :Minimal 0 :Hover (Variables|Default|GetSimpleWidgets) :Detail (Variables|Default|GetDetailWidgets) :Inspector 0))
  (return (LocalVariables|GetResult)))