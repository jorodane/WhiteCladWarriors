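; Unit component that supplies a header text widget showing the unit's selected name to info panels.
; BeginPlay builds an ordered widget claim, whose updater writes GetSelectedName into the text.
; GetInfoWidget offers that claim for the Hover, Detail and Inspector views.
; CheckSelectable always returns false, so the component never reports itself as selectable.
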(event Custom|NameUpdate
  (params (NewWidget :type Generic%20Widget%20Base%20Object%20Reference))
  (bind _returnvalue (Class|Selectable|GetSelectedName))
  (Class|ContainTextValue|SetText(Message) NewWidget _returnvalue))

(event Custom|ConstructWidgets
  (bind _returnvalue (Utilities|CreateOrderedWidgetClaimwithUpdater 50 "Text_Header" 0 (delegate Custom|NameUpdate)))
  (Variables|/Script/WhiteCladWarriors.GenericWidgetClaim|SetWidgetTransform _returnvalue (Utilities|Map|MakeMap "VerticalAlignment" 1.0))
  (Variables|Default|SetSimpleWidgets (Utilities|Array|MakeArray _returnvalue)))

(event EventBeginPlay
  (|CallParentFunction)
  (CallFunction|ConstructWidgets))

(event EventTick
  (params (DeltaSeconds :type Float%20%28single-precision%29)))

(fn GetInfoWidget
  (params (WantType :type EInfoWidgetType%20Enum :default "Minimal") (Operator :type Operator%20Object%20Reference))
  (bind _simplewidgets (Variables|Default|GetSimpleWidgets))
  (bind _returnvalue (Utilities|Select :Index WantType :Minimal 0 :Hover _simplewidgets :Detail _simplewidgets :Inspector _simplewidgets))
  (bind _output_get (LocalVariables|SetResult (|CallParentFunction WantType Operator)))
  (Utilities|Array|AppendArray _output_get _returnvalue)
  (return _returnvalue))

(fn CheckSelectable
  (params (Operator :type Operator%20Object%20Reference) (bIsSingleSelection :type Boolean))
  (return false))