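; Fillable value component that holds a current and max value for a unit and feeds it to widgets.
; On BeginPlay it registers itself with its owning UnitBase under its Tag, and stops if the owner is not one.
; Its BroadcastDirty sends the current and max values as a two-float message to every widget matching that Tag, then calls the parent implementation.
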(event EventBeginPlay
  (bind _asunit_base (Utilities|Casting|CastToUnitBase (Components|GetOwner)))
  (Class|UnitBase|AddFillValue _asunit_base (Variables|Default|GetTag) self))

(event EventTick
  (params (DeltaSeconds :type Float%20%28single-precision%29)))

(fn BroadcastDirty
  (bind _array_element (Utilities|ForEachWidget (Variables|Default|GetTag))
    (:LoopBody
      (Class|ContainFloat2Value|SetFloat2(Message) _array_element (Variables|Default|GetCurrentValue) (Variables|Default|GetMaxValue)))
    (:Completed
      (bind _returnvalue (|CallParentFunction))
      (return _returnvalue))))