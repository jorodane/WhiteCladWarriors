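; Actor component that gives its owning Pawn simple move and stop actions.
; On BeginPlay it caches the owner as a Pawn along with that Pawn's movement component.
; SetMove issues an AI MoveTo toward a destination or target actor, and SetStop halts movement immediately, both only while the movement component is valid.
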(event Custom|SetStop
  (bind _movement (Variables|Default|GetMovement)
    (:then
      (Components|Movement|StopMovementImmediately _movement))
    (:else)))

(event Custom|SetMove
  (params (Destination :type Vector) (TargetActor :type Actor%20Object%20Reference))
  (Variables|Default|GetMovement
    (:then
      (AI|AIMoveTo (Variables|Default|GetOwnerAsPawn) Destination TargetActor 5.0 false))
    (:else)))

(event EventBeginPlay
  (|CallParentFunction)
  (bind _as폰 (Utilities|Casting|CastToPawn (Components|GetOwner)))
  (Variables|Default|SetOwnerAsPawn _as폰)
  (Variables|Default|SetMovement (Pawn|GetMovementComponent _as폰)))