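; Attack action component for units that handles target detection, attackability checks, movement orders and retaliation against damage causers.
; It spawns a toggleable overlap sphere on BeginPlay and runs an attack check each tick.
; Attackability combines a target message, horizontal range and no active montage, while damaged player-controlled units without a main action attack the causer.
; It binds to owner unit events and supports pooling by toggling tick and resetting attack data on enqueue.
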(event Custom|CreateDetectionSphere
  (bind _returnvalue (Game|AddComponentbyClass (Components|GetOwner) "/Script/Engine.SphereComponent" false))
  (bind _output_get (Variables|Default|SetDetectionSphere _returnvalue))
  (Collision|BindEventtoOnComponentBeginOverlap _output_get (EventDispatchers|CreateEvent :!event OnActorDetected))
  (Collision|BindEventtoOnComponentEndOverlap _output_get (EventDispatchers|CreateEvent :!event OnActorUndetected))
  (Utilities|FlowControl|Delay 0.2)
  (Class|UnitAttackComponent|ResetAttackDatas))

(event EventBeginPlay
  (|CallParentFunction)
  (CallFunction|CreateDetectionSphere))

(event EventTick
  (params (DeltaSeconds :type Float%20%28single-precision%29))
  (|CallParentFunction DeltaSeconds)
  (Class|UnitAttackComponent|TickAttackCheck DeltaSeconds))

(event EventSetStop
  (Class|UnitAttackComponent|ResetAttackDatas))

(event EventOnPoolEnqueue
  (params (EnqueueTo :type Pool%20Component%20Object%20Reference))
  (Components|Tick|SetComponentTickEnabled false)
  (CallFunction|SetStop))

(event EventOnPoolDequeue
  (params (DequeueFrom :type Pool%20Component%20Object%20Reference))
  (Components|Tick|SetComponentTickEnabled true))

(event EventMovetoTarget
  (params (WantTarget :type Actor%20Object%20Reference))
  (bind _resultunit (Class|UnitComponentBase|TryGetOwnerUnit)
    (:True
      (Default|CallOnMovementStart _resultunit (Variables|Default|GetAttackFocusLocation) WantTarget (Class|UnitAttackComponent|GetAttackRange) (Variables|Default|GetActionClaimer)))))

(event EventMovetoLocation
  (params (WantLocation :type Vector :default "0, 0, 0"))
  (bind _resultunit (Class|UnitComponentBase|TryGetOwnerUnit)
    (:True
      (Default|CallOnMovementStart _resultunit WantLocation 0 1e+01 (Variables|Default|GetActionClaimer)))))

(event EventSetDetectionEnable
  (params (bWantDetectAround :type Boolean))
  (Collision|SetCollisionEnabled (Variables|Default|GetDetectionSphere) (select bWantDetectAround "QueryOnly" "NoCollision")))

(fn CheckAttackable
  (params (Target :type Actor%20Object%20Reference) (TargetUnit :type Unit%20Main%20Component%20Object%20Reference))
  (bind _output_get (LocalVariables|SetCurrentTarget Target))
  (bind _returnvalue (Class|Damageable|GetIsAttackable(Message) _output_get TargetUnit))
  (return (and _returnvalue (and (not (Class|UnitMainComponent|HasActionMontage TargetUnit)) (< (Transformation|GetHorizontalDistanceTo (Components|GetOwner) (LocalVariables|GetCurrentTarget)) (Class|UnitAttackComponent|GetAttackRange)))) _returnvalue (and (not (Class|UnitMainComponent|HasActionMontage TargetUnit)) (< (Transformation|GetHorizontalDistanceTo (Components|GetOwner) (LocalVariables|GetCurrentTarget)) (Class|UnitAttackComponent|GetAttackRange)))))

(fn GetDetectionEnabled
  (return (Class|PrimitiveComponent|IsCollisionEnabled (Variables|Default|GetDetectionSphere))))

(fn OnDamaged
  (params (TargetUnit :type Unit%20Main%20Component%20Object%20Reference) (Info :type Damage%20Info%20Structure%20%28by%20ref%29))
  (bind _output_get (LocalVariables|SetDamagedUnit TargetUnit))
  (Utilities|IsValid _output_get
    (:Is%20Valid
      (bind _output_get_2 (LocalVariables|SetCauser (.DamageCauser (Utilities|Struct|BreakDamageInfo Info))))
      (Utilities|IsValid _output_get_2
        (:Is%20Valid
          (if (not (Class|UnitMainComponent|HasMainAction (LocalVariables|GetDamagedUnit)))
            (bind _playercontroller (Variables|/Script/WhiteCladWarriors.UnitMainComponent|GetPlayerController (LocalVariables|GetDamagedUnit))
              (:then
                (bind _output_get_3 (LocalVariables|SetOperator (Variables|/Script/WhiteCladWarriors.IngameController|GetConnectedOperator _playercontroller)))
                (Class|UnitAttackComponent|CommandAttackTarget _output_get_3 (LocalVariables|GetCauser)))
              (:else))))))))

(fn GetChaseAction
  (bind _returnvalue (Class|ActionSetting|GetAction "ChaseAttack"))
  (return _returnvalue))

(fn GetAttackAction
  (bind _resultunit (Class|UnitComponentBase|TryGetOwnerUnit)
    (:True
      (bind _returnvalue (Class|ActionSetting|GetAction (Class|UnitMainComponent|GetActionfromTag _resultunit "Attack")))
      (return _returnvalue))))

(fn SetOwnerUnit
  (params (NewUnit :type Unit%20Main%20Component%20Object%20Reference))
  (bind _output_get (LocalVariables|SetNewOwner (|CallParentFunction NewUnit)))
  (Utilities|IsValid _output_get
    (:Is%20Valid
      (EventDispatchers|BindEventtoOnUnitDamage (LocalVariables|GetNewOwner) (EventDispatchers|CreateEvent :!event OnDamaged))
      (EventDispatchers|BindEventtoOnUnitDie (LocalVariables|GetNewOwner) (EventDispatchers|CreateEvent :!event OnUnitDied))
      (EventDispatchers|BindEventtoOnMainActionChanged (LocalVariables|GetNewOwner) (EventDispatchers|CreateEvent :!event OnMainActionChanged))
      (EventDispatchers|BindEventtoOnMovementStop (LocalVariables|GetNewOwner) (EventDispatchers|CreateEvent :!event OnMoveCompleted))
      (return (LocalVariables|GetNewOwner)))
    (:Is%20Not%20Valid
      (return 0))))