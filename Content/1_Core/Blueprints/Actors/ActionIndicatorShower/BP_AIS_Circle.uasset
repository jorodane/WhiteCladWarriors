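; Circular action indicator actor that implements the sizing events of an action indicator shower by changing its actor scale.
; Scale X acts as height, while Y and Z share one radius value passed through RemapWidth, which is not defined here.
; Length and width requests collapse into that uniform radius, using the larger value when two are given, so the shape stays round.
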(event Custom|SetHeightRadius
  (params (NewHeight :type Float%20%28double-precision%29) (NewRadius :type Float%20%28double-precision%29))
  (bind _returnvalue (CallFunction|RemapWidth NewRadius))
  (Transformation|SetActorScale3D (Math|Vector|MakeVector NewHeight _returnvalue _returnvalue)))

(event EventBeginPlay)

(event Collision|EventActorBeginOverlap
  (params (OtherActor :type Actor%20Object%20Reference)))

(event EventTick
  (params (DeltaSeconds :type Float%20%28single-precision%29)))

(event EventSetSize
  (params (NewSize :type Vector :default "0, 0, 0"))
  (CallFunction|SetHeightRadius (.x NewSize) (Math|Float|Max(Float) (.y NewSize) (.z NewSize))))

(event EventSetWidth
  (params (NewWidth :type Float%20%28double-precision%29))
  (bind _returnvalue (CallFunction|RemapWidth NewWidth))
  (Transformation|SetActorScale3D (Math|Vector|MakeVector (.x (Transformation|GetActorScale3D)) _returnvalue _returnvalue)))

(event EventSetWidthLength
  (params (Length :type Float%20%28double-precision%29) (Width :type Float%20%28double-precision%29))
  (CallFunction|SetWidth (Math|Float|Max(Float) Length Width)))

(event EventSetLength
  (params (NewLength :type Float%20%28double-precision%29))
  (CallFunction|SetWidth NewLength))

(fn ConstructionScript)