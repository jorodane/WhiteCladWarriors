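; Base actor for action indicators, showing a decal that can be positioned, rotated, sized, colored, textured and filled.
; On BeginPlay it creates a dynamic material from the Shower component, whose parameters drive fill percent, colors and texture.
; Size setters map length to Y scale and width to Z scale through pass-through Remap functions.
; DrawLine and DrawFrom combine these setters to span two points or extend from a start location.
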(event Custom|SetStartLocation
  (params (NewLocation :type Vector))
  (Transformation|SetActorLocation NewLocation false true))

(event Custom|SetLength
  (params (NewLength :type Float%20%28double-precision%29))
  (bind _returnvalue (Transformation|GetActorScale3D))
  (Transformation|SetActorScale3D (Math|Vector|MakeVector (.x _returnvalue) (CallFunction|RemapLength NewLength) (.z _returnvalue))))

(event Custom|DrawLineWithRotation
  (params (StartPosition :type Vector) (EndPosition :type Vector) (Width :type Float%20%28double-precision%29) (Rotation :type Rotator))
  (CallFunction|SetWidthLength (* (Math|Vector|Distance2D(Vector) StartPosition EndPosition) 0.5) Width)
  (Transformation|SetActorRotation Rotation true)
  (CallFunction|SetMiddleLocation StartPosition EndPosition))

(event Custom|SetFillColor
  (params (Color :type Linear%20Color%20Structure))
  (bind _decalmaterial (Variables|Default|GetDecalMaterial)
    (:then
      (Rendering|Material|SetVectorParameterValue _decalmaterial "FillColor" Color :!class /Script/Engine.MaterialInstanceDynamic))
    (:else)))

(event Custom|SetColor
  (params (Color :type Linear%20Color%20Structure))
  (bind _decalmaterial (Variables|Default|GetDecalMaterial)
    (:then
      (Rendering|Material|SetVectorParameterValue _decalmaterial "Color" Color :!class /Script/Engine.MaterialInstanceDynamic))
    (:else)))

(event Custom|SetWidthLength
  (params (Length :type Float%20%28double-precision%29) (Width :type Float%20%28double-precision%29))
  (Transformation|SetActorScale3D (Math|Vector|MakeVector (.x (Transformation|GetActorScale3D)) (CallFunction|RemapLength Length) (CallFunction|RemapWidth Width))))

(event Custom|SetTexture
  (params (NewTexture :type Texture%20Object%20Reference))
  (bind _decalmaterial (Variables|Default|GetDecalMaterial)
    (:then
      (Rendering|Material|SetTextureParameterValue _decalmaterial "Texture" NewTexture))
    (:else)))

(event Custom|SetMiddleLocation
  (params (A :type Vector) (B :type Vector))
  (Transformation|SetActorLocation (Math|Vector|Lerp(Vector) A B (Variables|Default|GetLengthLocationOffset)) false true))

(event Custom|DrawFrom
  (params (Location :type Vector) (Length :type Float%20%28double-precision%29) (Width :type Float%20%28double-precision%29) (Rotation :type Rotator))
  (CallFunction|SetStartLocation Location)
  (CallFunction|SetWidthLength Length Width)
  (Transformation|SetActorRotation (Math|Rotator|MakeRotator 0.0 0.0 (.yaw Rotation)) true))

(event Custom|SetWidth
  (params (NewWidth :type Float%20%28double-precision%29))
  (bind _returnvalue (Transformation|GetActorScale3D))
  (Transformation|SetActorScale3D (Math|Vector|MakeVector (.x _returnvalue) (.y _returnvalue) (CallFunction|RemapWidth NewWidth))))

(event Custom|SetSize
  (params (NewSize :type Vector))
  (Transformation|SetActorScale3D (Math|Vector|MakeVector (.x NewSize) (CallFunction|RemapLength (.y NewSize)) (CallFunction|RemapWidth (.z NewSize)))))

(event Custom|SetRotation
  (params (NewRotation :type Rotator))
  (Transformation|SetActorRotation NewRotation true))

(event Custom|SetDirection
  (params (NewDirection :type Vector))
  (CallFunction|SetRotation (Math|Conversions|RotationFromXVector (Class|KismetMathLibrary|VectorNormal2D NewDirection 0.0001))))

(event Custom|DrawLine
  (params (StartPosition :type Vector) (EndPosition :type Vector) (Width :type Float%20%28double-precision%29))
  (CallFunction|DrawLinewithRotation StartPosition EndPosition Width (Math|Rotator|MakeRotator 0.0 0.0 (.yaw (Math|Rotator|FindLookatRotation StartPosition EndPosition)))))

(event Custom|SetPercent
  (params (Value :type Float%20%28single-precision%29))
  (bind _decalmaterial (Variables|Default|GetDecalMaterial)
    (:then
      (Rendering|Material|SetScalarParameterValue _decalmaterial "Fill" Value :!class /Script/Engine.MaterialInstanceDynamic))
    (:else)))

(event EventBeginPlay
  (bind _returnvalue (Rendering|Material|CreateDynamicMaterialInstance (Variables|Default|GetShower) :!class /Script/Engine.DecalComponent))
  (Variables|Default|SetDecalMaterial _returnvalue))

(event Collision|EventActorBeginOverlap
  (params (OtherActor :type Actor%20Object%20Reference)))

(event EventTick
  (params (DeltaSeconds :type Float%20%28single-precision%29)))

(fn ConstructionScript)

(fn RemapLength
  (params (A :type Float%20%28double-precision%29))
  (return A))

(fn RemapWidth
  (params (A :type Float%20%28double-precision%29))
  (return A))