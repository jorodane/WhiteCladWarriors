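; BP_UnitBase is a base actor for selectable units, handling selection and hover feedback and supplying a name widget for UI.
; Selection toggles a decal, hover toggles custom depth on the mesh, and the select effect spawns attached Niagara only for the local operator.
; BeginPlay builds an ordered header-text widget claim that fills itself from the selected name and serves the Hover, Detail and Inspector info views.
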(event Custom|NameUpdate
  (params (NewWidget :type Generic%20Widget%20Base%20Object%20Reference))
  (bind _returnvalue (Class|Selectable|GetSelectedName))
  (Class|ContainTextValue|SetText(Message) NewWidget _returnvalue))

(event EventSelect
  (params (Operator :type Operator%20Object%20Reference) (bIsSingleSelection :type Boolean))
  (Rendering|SetVisibility (Variables|컴포넌트|GetSelectedDecal) true false))

(event Collision|EventActorBeginOverlap
  (params (OtherActor :type Actor%20Object%20Reference)))

(event EventTick
  (params (DeltaSeconds :type Float%20%28single-precision%29)))

(event EventDeselect
  (Rendering|SetVisibility (Variables|컴포넌트|GetSelectedDecal) false false))

(event EventMouseHoverEnd
  (Rendering|SetRenderCustomDepth (Variables|Character|GetMesh) false))

(event EventMouseHoverBegin
  (Rendering|SetRenderCustomDepth (Variables|Character|GetMesh) true))

(event EventBeginPlay
  (|CallParentFunction)
  (bind _returnvalue (Game|ConstructObjectfromClass "/Script/WhiteCladWarriors.OrderedGenericWidgetClaim" 50 "Text_Header"))
  (bind _output_get (Variables|Default|SetNameWidget _returnvalue))
  (Class|GenericWidgetClaim|AssignGenericWidgetEvents _output_get (delegate Custom|NameUpdate) (delegate Custom|NameUpdate)))

(event EventPlaySelectEffect
  (params (Operator :type Operator%20Object%20Reference) (bIsSingleSelection :type Boolean))
  (if (== Operator (Class|Operator|GetLocalOperator))
    (Niagara|SpawnSystemAttached "/Game/1_Core/VisualEffects/Single/NS_MoveEffect.NS_MoveEffect" (Variables|Character|GetMesh) "None" "0, 0, 0" "0, 0, 0" "KeepRelativeOffset" false)))

(fn ConstructionScript)

(fn IsSelectable
  (params (Operator :type Operator%20Object%20Reference))
  (return true))

(fn GetSelectedName
  (return (Variables|Default|GetSelectedName)))

(fn GetUnitInfoWidget
  (params (WantType :type EInfoWidgetType%20Enum :default "Minimal"))
  (bind _namewidget (Variables|Default|GetNameWidget))
  (return (Utilities|Array|MakeArray (Utilities|Select :Index WantType :Minimal 0 :Hover _namewidget :Hero 0 :Detail _namewidget :Inspector _namewidget))))