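; Base Blueprint for selectable hero units, handling selection feedback and info-panel text.
; On BeginPlay it creates ordered widget claims for a name header (player user name, falling back to SelectedName) and a placeholder level-1 line, served to Hover, Detail and Inspector views.
; Selection toggles a decal, hover toggles custom depth on the mesh, and a Niagara select effect spawns only for the local operator.
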(event Custom|NameUpdate
  (params (NewWidget :type Generic%20Widget%20Base%20Object%20Reference))
  (bind _returnvalue (Class|Selectable|GetSelectedName))
  (Class|ContainTextValue|SetText(Message) NewWidget _returnvalue))

(event Custom|UpdateLevel
  (params (NewWidget :type Generic%20Widget%20Base%20Object%20Reference))
  (Class|ContainTextValue|SetText(Message) NewWidget (Utilities|Text|FormatText "LV.{Level} {Name}" (Math|Conversions|ToInteger(Byte) 1) (Variables|Default|GetSelectedName))))

(event EventSelect
  (params (Operator :type Operator%20Object%20Reference) (bIsSingleSelection :type Boolean))
  (Rendering|SetVisibility (Variables|Default|GetSelectedDecal) true false))

(event EventDeselect
  (Rendering|SetVisibility (Variables|Default|GetSelectedDecal) false false))

(event EventMouseHoverEnd
  (Rendering|SetRenderCustomDepth (Variables|Character|GetMesh) false))

(event EventMouseHoverBegin
  (Rendering|SetRenderCustomDepth (Variables|Character|GetMesh) true))

(event EventBeginPlay
  (|CallParentFunction)
  (bind _returnvalue (Game|ConstructObjectfromClass "/Script/WhiteCladWarriors.OrderedGenericWidgetClaim" 50 "Text_Header"))
  (bind _output_get (Variables|Default|SetNameWidget _returnvalue))
  (Class|GenericWidgetClaim|AssignGenericWidgetEvents _output_get (delegate Custom|NameUpdate) (delegate Custom|NameUpdate))
  (bind _returnvalue_2 (Game|ConstructObjectfromClass "/Script/WhiteCladWarriors.OrderedGenericWidgetClaim" 75 "Text_Explain"))
  (bind _output_get_2 (Variables|Default|SetExplainWidget _returnvalue_2))
  (Class|GenericWidgetClaim|AssignGenericWidgetEvents _returnvalue_2 (delegate Custom|UpdateLevel) (delegate Custom|UpdateLevel)))

(event EventPlaySelectEffect
  (params (Operator :type Operator%20Object%20Reference) (bIsSingleSelection :type Boolean))
  (if (== Operator (Class|Operator|GetLocalOperator))
    (Niagara|SpawnSystemAttached "/Game/1_Core/VisualEffects/Single/NS_MoveEffect.NS_MoveEffect" (Variables|Character|GetMesh) "None" "0, 0, 0" "0, 0, 0" "KeepRelativeOffset" false)))

(fn ConstructionScript)

(fn IsSelectable
  (params (Operator :type Operator%20Object%20Reference))
  (return (== Operator Operator)))

(fn GetUnitInfoWidget
  (params (WantType :type EInfoWidgetType%20Enum :default "Minimal"))
  (bind _namewidget (Variables|Default|GetNameWidget))
  (bind _explainwidget (Variables|Default|GetExplainWidget))
  (bind _array (Utilities|Array|MakeArray _namewidget _explainwidget))
  (return (Utilities|Select :Index WantType :Minimal 0 :Hover _array :Hero 0 :Detail _array :Inspector _array)))

(fn GetSelectedName
  (bind _playercontroller (Variables|Default|GetPlayerController)
    (:then
      (return (Variables|/Script/WhiteCladWarriors.IngameController|GetUserName _playercontroller)))
    (:else
      (return (Variables|Default|GetSelectedName)))))