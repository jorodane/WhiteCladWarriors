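; BP_SimpleActorBasedUnit is a simple Actor-based unit that implements a set of selection functions.
; It always reports itself selectable, whatever the operator, and returns a fixed selection order.
; Info widget, selected icon and selected name requests are forwarded to BPUnitMainComponent.
; The event graph and construction script are empty, so the Blueprint adds no runtime logic of its own.
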(event EventBeginPlay)

(event Collision|EventActorBeginOverlap
  (params (OtherActor :type Actor%20Object%20Reference)))

(event EventTick
  (params (DeltaSeconds :type Float%20%28single-precision%29)))

(fn ConstructionScript)

(fn CheckSelectable
  (params (Operator :type Operator%20Object%20Reference))
  (return true))

(fn GetInfoWidget
  (params (WantType :type EInfoWidgetType%20Enum :default "Minimal"))
  (return (Class|InfoConnectable|GetInfoWidget (Variables|Default|GetBP_UnitMainComponent) WantType)))

(fn GetSelectedIcon
  (bind _returnvalue (Class|Selectable|GetSelectedIcon (Variables|Default|GetBP_UnitMainComponent)))
  (return _returnvalue))

(fn GetSelectedName
  (bind _returnvalue (Class|Selectable|GetSelectedName (Variables|Default|GetBP_UnitMainComponent)))
  (return _returnvalue))

(fn GetSelectedorder
  (return 5e+02))