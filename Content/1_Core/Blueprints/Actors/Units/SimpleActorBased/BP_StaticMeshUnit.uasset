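; BP_StaticMeshUnit is an actor Blueprint for units represented by a static mesh, with hover highlighting and selection info.
; On BeginPlay it fills a highlight mesh array with its Mesh, and mouse hover events toggle Render Custom Depth on that array.
; Selected name, selected icon and info widget queries are forwarded to its BPUnitMainComponent.
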(event EventBeginPlay
  (|CallParentFunction)
  (CallFunction|SetHighlightMeshes))

(event Collision|EventActorBeginOverlap
  (params (OtherActor :type Actor%20Object%20Reference))
  (|CallParentFunction OtherActor) ; This node is disabled and will not be called.\nDrag off pins to build functionality.
)

(event EventTick
  (params (DeltaSeconds :type Float%20%28single-precision%29))
  (|CallParentFunction DeltaSeconds) ; This node is disabled and will not be called.\nDrag off pins to build functionality.
)

(event EventMouseHoverBegin
  (Rendering|SetRenderCustomDepth (Variables|Default|GetHighlightMeshArray) true))

(event EventMouseHoverEnd
  (Rendering|SetRenderCustomDepth (Variables|Default|GetHighlightMeshArray) false))

(fn ConstructionScript
  (|CallParentFunction))

(fn GetSelectedName
  (bind _returnvalue (Class|Selectable|GetSelectedName (Variables|Default|GetBP_UnitMainComponent)))
  (return _returnvalue))

(fn GetSelectedIcon
  (bind _returnvalue (Class|Selectable|GetSelectedIcon (Variables|Default|GetBP_UnitMainComponent)))
  (return _returnvalue))

(fn GetInfoWidget
  (params (WantType :type EInfoWidgetType%20Enum :default "Minimal"))
  (return (Class|InfoConnectable|GetInfoWidget (Variables|Default|GetBP_UnitMainComponent) WantType)))

(fn SetHighlightMeshes
  (Variables|Default|SetHighlightMeshArray (Utilities|Array|MakeArray (Variables|Default|GetMesh)))
  (return))