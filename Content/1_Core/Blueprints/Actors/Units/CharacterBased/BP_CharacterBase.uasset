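; BP_CharacterBase is a base character Blueprint for units that can be selected and hovered with the mouse.
; BeginPlay creates a dynamic material for the selection decal, which Select and Deselect show or hide.
; Mouse hover toggles custom depth rendering on the mesh.
; Selection queries return defaults: always selectable, a generic name and a fixed order, with empty icon and info widget returns.
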(event EventBeginPlay
  (|CallParentFunction)
  (bind _returnvalue (Rendering|Material|CreateDynamicMaterialInstance (Variables|Default|GetSelectDecal) :!class /Script/Engine.DecalComponent))
  (Variables|Default|SetSelectDecalMaterial _returnvalue))

(event Collision|EventActorBeginOverlap
  (params (OtherActor :type Actor%20Object%20Reference)))

(event EventTick
  (params (DeltaSeconds :type Float%20%28single-precision%29)))

(event EventDeselect
  (Development|SetHiddeninGame (Variables|Default|GetSelectDecal) true false))

(event EventSelect
  (params (Operator :type Operator%20Object%20Reference) (bIsSingleSelection :type Boolean))
  (Development|SetHiddeninGame (Variables|Default|GetSelectDecal) false false))

(event EventMouseHoverBegin
  (Rendering|SetRenderCustomDepth (Variables|Character|GetMesh) true))

(event EventMouseHoverEnd
  (Rendering|SetRenderCustomDepth (Variables|Character|GetMesh) false))

(fn ConstructionScript)

(fn CheckSelectable
  (params (Operator :type Operator%20Object%20Reference) (bIsSingleSelection :type Boolean))
  (return true))

(fn GetInfoWidget
  (params (WantType :type EInfoWidgetType%20Enum :default "Minimal") (Operator :type Operator%20Object%20Reference))
  (return 0))

(fn GetSelectedIcon
  (return ""))

(fn GetSelectedName
  (return "Character"))

(fn GetSelectedorder
  (return 1e+03))