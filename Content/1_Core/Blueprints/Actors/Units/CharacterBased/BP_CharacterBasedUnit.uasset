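; Character-based unit actor that exposes damage, status, selection and info-widget functions, mostly forwarded to BPUnitMainComponent.
; BeginPlay binds to the component's unit-die event.
; TakeDamage delegates to the component and calls OnDamage only for non-lethal hits that deal positive damage.
; Single selection is always allowed, multi-selection requires the operator's authority, and selection order is fixed.
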(event EventBeginPlay
  (|CallParentFunction)
  (EventDispatchers|BindEventtoOnUnitDie (Variables|Default|GetBP_UnitMainComponent) (EventDispatchers|CreateEvent :!event OnDie)))

(event Collision|EventActorBeginOverlap
  (params (OtherActor :type Actor%20Object%20Reference))
  (|CallParentFunction OtherActor) ; 지금 이 노드는 비활성 상태입니다. \n핀을 끌어서 다른 노드를 연결하면 활성화됩니다.
)

(event EventTick
  (params (DeltaSeconds :type Float%20%28single-precision%29))
  (|CallParentFunction DeltaSeconds) ; 지금 이 노드는 비활성 상태입니다. \n핀을 끌어서 다른 노드를 연결하면 활성화됩니다.
)

(fn ConstructionScript
  (|CallParentFunction))

(fn TakeDamage
  (params (Info :type Damage%20Info%20Structure%20%28by%20ref%29))
  (bind (_biskill _returnvalue) (Class|Damageable|TakeDamage (Variables|Default|GetBP_UnitMainComponent) Info))
  (if (or _biskill (<= _returnvalue 0.0))
    _
    (else
      (CallFunction|OnDamage (Variables|Default|GetBP_UnitMainComponent) Info)))
  (return _biskill _returnvalue))

(fn GetSelectedName
  (return (Variables|/Script/WhiteCladWarriors.UnitMainComponent|GetSelectedName (Variables|Default|GetBP_UnitMainComponent))))

(fn GetSelectedIcon
  (return (Variables|/Script/WhiteCladWarriors.UnitMainComponent|GetSelectedIcon (Variables|Default|GetBP_UnitMainComponent))))

(fn CheckSelectable
  (params (Operator :type Operator%20Object%20Reference) (bIsSingleSelection :type Boolean))
  (return (or bIsSingleSelection (Class|UnitMainComponent|HasOperatorAuthority (Variables|Default|GetBP_UnitMainComponent) Operator))))

(fn GetSelectedorder
  (return 5e+02))

(fn GetInfoWidget
  (params (WantType :type EInfoWidgetType%20Enum :default "Minimal") (Operator :type Operator%20Object%20Reference))
  (return (Class|InfoConnectable|GetInfoWidget (Variables|Default|GetBP_UnitMainComponent) WantType Operator)))

(fn GetIsDie
  (bind _returnvalue (Class|Damageable|GetIsDie (Variables|Default|GetBP_UnitMainComponent)))
  (return _returnvalue))

(fn GetIsDamageable
  (params (From :type Unit%20Main%20Component%20Object%20Reference))
  (bind _returnvalue (Class|Damageable|GetIsDamageable From))
  (return _returnvalue))

(fn GetIsAttackable
  (params (From :type Unit%20Main%20Component%20Object%20Reference))
  (bind _returnvalue (Class|Damageable|GetIsAttackable (Variables|Default|GetBP_UnitMainComponent) From))
  (return _returnvalue))