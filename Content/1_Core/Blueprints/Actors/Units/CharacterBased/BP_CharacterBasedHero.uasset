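; Character-based hero unit that is selectable, hoverable and damageable, delegating most hero logic to BPHeroMainComponent.
; The component supplies selection info, authority checks for multi-selection and death notification, and receives incoming damage.
; Ally type tints the selection decal and sets the hover custom-depth stencil.
; Each tick, unless physics is simulating, the mesh yaws toward the mouse terrain position while an input-ready montage exists, otherwise resetting its relative rotation.
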(event Game|Damage|EventAnyDamage
  (params (Damage :type Float%20%28single-precision%29) (DamageType :type Damage%20Type%20Object%20Reference) (InstigatedBy :type Controller%20Object%20Reference) (DamageCauser :type Actor%20Object%20Reference))
  (|CallParentFunction Damage DamageType InstigatedBy DamageCauser)
  (Class|UnitMainComponent|TakeDamage (Variables|Default|GetBP_HeroMainComponent) (Utilities|Struct|MakeDamageInfo Damage DamageCauser 0)))

(event Collision|EventActorBeginOverlap
  (params (OtherActor :type Actor%20Object%20Reference)))

(event EventTick
  (params (DeltaSeconds :type Float%20%28single-precision%29))
  (bind _mesh (Variables|Character|GetMesh))
  (bind _mesh_2 (Variables|Character|GetMesh))
  (|CallParentFunction DeltaSeconds)
  (if (not (Class|SceneComponent|IsAnySimulatingPhysics _mesh_2))
    (if (Class|UnitMainComponent|HasInputReadyMontage (Variables|Default|GetBP_HeroMainComponent))
      (Transformation|SetWorldRotation _mesh (Math|Rotator|MakeRotator 0.0 0.0 (+ (.yaw (Math|Rotator|FindLookatRotation (Transformation|GetWorldLocation _mesh_2) (.mouseterrainposition (Class|Operator|GetLocalInputPackage)))) -9e+01)) false false)
      (else
        (Transformation|SetRelativeRotation _mesh "0.000000,-90.000000,0.000000" false false)))))

(event EventSelect
  (params (Operator :type Operator%20Object%20Reference) (bIsSingleSelection :type Boolean))
  (|CallParentFunction Operator bIsSingleSelection)
  (Rendering|Material|SetVectorParameterValue (Variables|Default|GetSelectDecalMaterial) "LineColor" (Utilities|Select :Index (Class|UnitMainComponent|GetAllyType (Variables|Default|GetBP_HeroMainComponent) Operator) :Normal "(R=3.000000,G=3.000000,B=3.000000,A=1.000000)" :Own "(R=0.000000,G=3.000000,B=0.000000,A=1.000000)" :Enemy "(R=3.000000,G=0.000000,B=0.000000,A=1.000000)" :Ally "(R=3.000000,G=3.000000,B=0.000000,A=1.000000)") :!class /Script/Engine.MaterialInstanceDynamic))

(event EventMouseHoverBegin
  (|CallParentFunction)
  (Rendering|SetCustomDepthStencilValue (Variables|Character|GetMesh) (Math|Conversions|ToInteger(Byte) (Class|UnitMainComponent|GetAllyType (Variables|Default|GetBP_HeroMainComponent) (Class|Operator|GetLocalOperator)))))

(event EventBeginPlay
  (|CallParentFunction)
  (EventDispatchers|BindEventtoOnUnitDie (Variables|Default|GetBP_HeroMainComponent) (EventDispatchers|CreateEvent :!event OnDie)))

(fn ConstructionScript)

(fn GetSelectedName
  (return (Variables|/Script/WhiteCladWarriors.UnitMainComponent|GetSelectedName (Variables|Default|GetBP_HeroMainComponent))))

(fn GetSelectedIcon
  (return (Variables|/Script/WhiteCladWarriors.UnitMainComponent|GetSelectedIcon (Variables|Default|GetBP_HeroMainComponent))))

(fn CheckSelectable
  (params (Operator :type Operator%20Object%20Reference) (bIsSingleSelection :type Boolean))
  (return (or bIsSingleSelection (Class|UnitMainComponent|HasOperatorAuthority (Variables|Default|GetBP_HeroMainComponent) Operator))))

(fn GetSelectedorder
  (return 1e+02))

(fn GetInfoWidget
  (params (WantType :type EInfoWidgetType%20Enum :default "Minimal") (Operator :type Operator%20Object%20Reference))
  (return (Class|InfoConnectable|GetInfoWidget (Variables|Default|GetBP_HeroMainComponent) WantType Operator)))