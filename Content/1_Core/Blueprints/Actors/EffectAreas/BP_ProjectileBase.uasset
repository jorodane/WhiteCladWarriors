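; Base projectile effect actor that a node spawns with a cursor, taking owner and unit from the cursor's component and excluding that owner from targeting.
; SetProjectileInfo sets particle, position and scale, launches the mesh by physics impulse, and stretches durability to cover Range/Speed.
; Valid mesh hits exclude that target from further hits and report back to the node, replacing hit normals with the reversed, flattened launch direction.
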(event OnComponentHit(Mesh)
  (params (HitComponent :type Primitive%20Component%20Object%20Reference) (OtherActor :type Actor%20Object%20Reference) (OtherComp :type Primitive%20Component%20Object%20Reference) (NormalImpulse :type Vector :default "0, 0, 0") (Hit :type Hit%20Result%20Structure%20%28by%20ref%29))
  (if (CallFunction|TargetCheck OtherActor)
    (CallFunction|OnTargetHit OtherActor OtherComp NormalImpulse Hit)))

(event Custom|AddForce
  (params (Velocity :type Vector) (BoneName :type Name) (bAccelChange :type Boolean))
  (bind _output_get (Variables|Default|SetReceivedForce Velocity))
  (Variables|Default|SetReceivedNormal (* (Class|KismetMathLibrary|VectorNormal2D _output_get 0.0001) -1.0))
  (Physics|AddImpulse (Variables|Character|GetMesh) (Variables|Default|GetReceivedForce) BoneName bAccelChange)
  (Transformation|SetWorldRotation (Variables|Character|GetMesh) (Math|Conversions|RotationFromXVector (Variables|Default|GetReceivedForce)) false false))

(event EventBeginPlay)

(event Collision|EventActorBeginOverlap
  (params (OtherActor :type Actor%20Object%20Reference)))

(event EventTick
  (params (DeltaSeconds :type Float%20%28single-precision%29)))

(event EventSpawnInitialize
  (params (SpawnedNode :type Action%20Spawn%20Node%20Object%20Reference) (Cursor :type Action%20Cursor%20Finder%20Structure%20%28by%20ref%29) (OnDestroyEvent :type Delegate%20%28by%20ref%29))
  (Utilities|FlowControl|Sequence
    (:then_0
      (Variables|Default|SetBaseNode SpawnedNode)
      (bind _output_get (Variables|Default|SetBaseCursor Cursor))
      (Variables|Default|SetOwnerOperator (.CurrentOperator (Utilities|Struct|BreakActionCursorFinder _output_get)))
      (bind _output_get_2 (Variables|Default|SetOwnerComponent (.CurrentComponent (Utilities|Struct|BreakActionCursorFinder _output_get))))
      (Utilities|IsValid _output_get_2
        (:Is%20Valid
          (Actor|SetOwner (Components|GetOwner _output_get_2))
          (Utilities|IsValid (Components|GetOwner _output_get_2)
            (:Is%20Valid
              (Utilities|FlowControl|Sequence
                (:then_0
                  (CallFunction|AddtoExceptTarget (Components|GetOwner _output_get_2)))
                (:then_1
                  (Variables|Default|SetOwnerUnit (Class|UnitComponentBase|GetOwnerUnit _output_get_2) :!label _label))))
            (:Is%20Not%20Valid
              (goto _label))))))
    (:then_1
      (EventDispatchers|UnbindallEventsfromBroadcastDestroy)
      (EventDispatchers|BindEventtoBroadcastDestroy OnDestroyEvent))))

(fn ConstructionScript
  (|CallParentFunction))

(fn SetProjectileInfo
  (params (MainParticle :type Niagara%20System%20Object%20Reference) (StartLocation :type Vector) (Direction :type Vector :default "1.000000,0.000000,0.000000") (Speed :type Float%20%28double-precision%29) (Range :type Float%20%28double-precision%29) (Radius :type Float%20%28double-precision%29) (MaxDurability :type Float%20%28double-precision%29))
  (Class|NiagaraComponent|SetAsset (Variables|Default|GetMainParticle) MainParticle true)
  (Transformation|SetActorLocation StartLocation false true)
  (CallFunction|AddForce (* (Math|Vector|Normalize Direction) Speed) "None" true)
  (Transformation|SetActorScale3D (Math|Conversions|ToVector(Float) (* Radius 0.01)))
  (CallFunction|SetDurability (Math|Float|Max(Float) MaxDurability (Math|Float|SelectFloat (/ Range Speed) MaxDurability (> Speed 0.0)))))

(fn OnTargetHit
  (params (TargetActor :type Actor%20Object%20Reference) (TargetComponent :type Primitive%20Component%20Object%20Reference) (Impulse :type Vector) (Hit :type Hit%20Result%20Structure))
  (bind (_bblockinghit _binitialoverlap _time _distance _location _impactpoint _normal _impactnormal _physmat _hitactor _hitcomponent _hitbonename _bonename _hititem _elementindex _faceindex _tracestart _traceend) (Collision|BreakHitResult Hit))
  (bind _receivednormal (Variables|Default|GetReceivedNormal))
  (CallFunction|AddtoExceptTarget TargetActor)
  (bind _basenode (Variables|Default|GetBaseNode)
    (:then
      (Class|ReceiverHitEvent|OnHitReceived(Message) _basenode self (Variables|Default|GetBaseCursor) (Collision|MakeHitResult _bblockinghit _binitialoverlap _time _distance _location _impactpoint _receivednormal _receivednormal _physmat _hitactor _hitcomponent _hitbonename _bonename _hititem _elementindex _faceindex _tracestart _traceend)))
    (:else)))