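; BP_Operator is the player pawn for RTS-style control: it spawns and follows a hero, drives the camera and issues selection and hotkey commands.
; On player connection it sets up Enhanced Input, the in-game widget and a drag-area actor.
; Shift and Control modify clicks, and Shift also queues hotkey actions as reservations.
; Tick handles edge scrolling and drains accumulated wheel-drag movement into rate-limited pan or rotation, while zoom length sets arm pitch.
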(event Input|EnhancedActionEvents|EnhancedInputActionIA_MouseLeft
  (params (ActionValue :type Boolean) (ElapsedSeconds :type Float%20%28double-precision%29) (TriggeredSeconds :type Float%20%28double-precision%29) (InputAction :type Input%20Action%20Object%20Reference :default "/Game/1_Core/Inputs/IA_MouseLeft.IA_MouseLeft"))
  (bind _currentinputpackage (Variables|Default|GetCurrentInputPackage))
  (bind (_dragstartposition _mouseterrainposition) (Utilities|Struct|BreakInputPackage _currentinputpackage))
  ;[0.15 0.15 0.15 0.5] Click
  (:Triggered
    (if (not (Class|Operator|IsInputClaimed))
      (Class|Operator|DrawDragArea _dragstartposition _mouseterrainposition)))
  (:Started
    (Utilities|Struct|SetmembersinInputPackage _currentinputpackage _mouseterrainposition))
  (:Completed
    (Class|Operator|OnLeftClick false (Variables|Default|GetbIsAdditiveMode) (Variables|Default|GetbIsSelectAllMode))
    (Class|Operator|HideDragArea)))

(event Input|EnhancedActionEvents|EnhancedInputActionIA_Zoom
  (params (ActionValue :type Float%20%28double-precision%29) (ElapsedSeconds :type Float%20%28double-precision%29) (TriggeredSeconds :type Float%20%28double-precision%29) (InputAction :type Input%20Action%20Object%20Reference :default "/Game/1_Core/Inputs/IA_Zoom.IA_Zoom"))
  ;[0.15 0.15 0.15 0.5] Zoom
  (Class|Operator|CameraZoom ActionValue (CallFunction|GetCameraZoomLimitMin) (CallFunction|GetCameraZoomLimitMax) (CallFunction|GetCameraZoomSpeed)))

(event Input|EnhancedActionEvents|EnhancedInputActionIA_Shift
  (params (ActionValue :type Boolean) (ElapsedSeconds :type Float%20%28double-precision%29) (TriggeredSeconds :type Float%20%28double-precision%29) (InputAction :type Input%20Action%20Object%20Reference :default "/Game/1_Core/Inputs/IA_Shift.IA_Shift"))
  ;[0.15 0.15 0.15 0.5] SimpleInput
  (:Started
    (bind _output_get (Variables|Default|SetbIsAdditiveMode ActionValue :!label _label))
    (Variables|Default|SetbIsReservationMode _output_get))
  (:Completed
    (goto _label)))

(event Input|EnhancedActionEvents|EnhancedInputActionIA_KeyboardArrow
  (params (ActionValue :type Vector%202D%20Structure) (ElapsedSeconds :type Float%20%28double-precision%29) (TriggeredSeconds :type Float%20%28double-precision%29) (InputAction :type Input%20Action%20Object%20Reference :default "/Game/1_Core/Inputs/IA_KeyboardArrow.IA_KeyboardArrow"))
  ;[0.15 0.15 0.15 0.5] CameraMove By Keyboard
  (Class|Operator|CameraMove (Math|Conversions|ToVector(Vector2D) ActionValue) (CallFunction|GetCameraMoveSpeedKeyboard))
  (Class|Operator|RemoveFocusActor))

(event Input|EnhancedActionEvents|EnhancedInputActionIA_MouseWheelButton
  (params (ActionValue :type Boolean) (ElapsedSeconds :type Float%20%28double-precision%29) (TriggeredSeconds :type Float%20%28double-precision%29) (InputAction :type Input%20Action%20Object%20Reference :default "/Game/1_Core/Inputs/IA_MouseWheelButton.IA_MouseWheelButton"))
  (bind _playercontroller (Variables|Default|GetPlayerController))
  (bind (_locationx _locationy) (Game|Player|GetMousePosition _playercontroller))
  ;[0.15 0.15 0.15 0.5] SimpleInput
  (:Started
    (Variables|Default|SetMouseWheel true)
    (Variables|Default|SetWheelStartPosition (Math|Vector2D|MakeVector2D _locationx _locationy))
    (Variables|/Script/Engine.PlayerController|SetbShowMouseCursor (Variables|Default|GetPlayerController) (not (Variables|Default|GetMouseWheel)) :!label _label))
  (:Completed
    (Variables|Default|SetMouseWheel false)
    (goto _label)))

(event Input|EnhancedActionEvents|EnhancedInputActionIA_Control
  (params (ActionValue :type Boolean) (ElapsedSeconds :type Float%20%28double-precision%29) (TriggeredSeconds :type Float%20%28double-precision%29) (InputAction :type Input%20Action%20Object%20Reference :default "/Game/1_Core/Inputs/IA_Control.IA_Control"))
  ;[0.15 0.15 0.15 0.5] SimpleInput
  (:Started
    (Variables|Default|SetbIsSelectAllMode ActionValue :!label _label))
  (:Completed
    (goto _label)))

(event Input|EnhancedActionEvents|EnhancedInputActionIA_MouseRight
  (params (ActionValue :type Boolean) (ElapsedSeconds :type Float%20%28double-precision%29) (TriggeredSeconds :type Float%20%28double-precision%29) (InputAction :type Input%20Action%20Object%20Reference :default "/Game/1_Core/Inputs/IA_MouseRight.IA_MouseRight"))
  (:Completed
    (Class|Operator|OnRightClick false)))

(event Input|EnhancedActionEvents|EnhancedInputActionIA_FollowHero
  (params (ActionValue :type Boolean) (ElapsedSeconds :type Float%20%28double-precision%29) (TriggeredSeconds :type Float%20%28double-precision%29) (InputAction :type Input%20Action%20Object%20Reference :default "/Game/1_Core/Inputs/IA_FollowHero.IA_FollowHero"))
  ;[0.15 0.15 0.15 0.5] SimpleInput
  (if (Class|Operator|IsFocusHero)
    (Class|Operator|ResetCameraRotation)
    (else
      (Class|Operator|SetFollowingHero true)))
  (if (not (Class|Operator|IsOnlySelectHero))
    (Class|Operator|SelectActor (Variables|Default|GetHeroActor) true)))

(event EventBeginPlay
  ;[0.15 0.15 0.15 0.5] Initiate
  (Utilities|FlowControl|Sequence
    (:then_0
      (Variables|/Script/Engine.SpringArmComponent|SetTargetArmLength (Variables|Default|GetCameraArm) (Variables|Default|GetCameraLength))
      (Variables|Default|SetSelectorCamera (Variables|Default|GetCameraMain)))
    (:then_1
      (Class|Operator|SpawnHero (Transformation|GetActorLocation))
      (Class|Operator|SetFollowingHero true))))

(event EventOnPlayerConnected
  (params (NewPlayer :type Ingame%20Controller%20Object%20Reference))
  ;[0.15 0.15 0.15 0.5] Control Link
  (|CallParentFunction NewPlayer)
  (CallFunction|InitiateController NewPlayer)
  (CallFunction|CreateIngameWidget (Variables|Default|GetPlayerController))
  (CallFunction|InitiateDragArea))

(event EventSetCameraLength
  (params (Value :type Float%20%28single-precision%29))
  (bind _result (CallFunction|GetCameraZoomLimitMin))
  ;[0.15 0.15 0.15 0.5] Zoom
  (|CallParentFunction Value)
  (bind _output_get (Variables|/Script/Engine.SpringArmComponent|SetTargetArmLength (Variables|Default|GetCameraArm) Value))
  (Transformation|SetRelativeRotation (Variables|Default|GetCameraArm) (Math|Rotator|MakeRotator 0.0 (Math|Float|Lerp -3e+01 -65.0 (Math|Float|Clamp(Float) (/ (- _output_get _result) (- 6e+02 _result)))) 0.0) false false))

(event EventTick
  (params (DeltaSeconds :type Float%20%28single-precision%29))
  (bind (_offset _position _viewportsize) (CallFunction|GetMousePositiononViewport))
  (bind _playercontroller (Variables|Default|GetPlayerController))
  (bind _wheelstartposition (Variables|Default|GetWheelStartPosition))
  (bind (_locationx _locationy) (Game|Player|GetMousePosition _playercontroller))
  (|CallParentFunction DeltaSeconds)
  (Utilities|FlowControl|Sequence
    (:then_0
      (if (Variables|Default|GetMouseWheel)
        (Variables|Default|SetClaimedWheelMove (+ (Variables|Default|GetClaimedWheelMove) (Math|Vector|MakeVector (- _locationx (.x _wheelstartposition)) (- (.y _wheelstartposition) _locationy) 0.0)))
        (Class|PlayerController|SetMouseLocation (Variables|Default|GetPlayerController) (Math|Float|Truncate (.x _wheelstartposition)) (Math|Float|Truncate (.y _wheelstartposition)))
        (else
          (Variables|Default|GetFocusActor
            (:then)
            (:else
              (Variables|Default|SetCurrentMousePosition _position)
              (Variables|Default|SetCurrentViewportSize _viewportsize)
              (Class|Operator|EdgeScroll (Variables|Default|GetCurrentMousePosition) (Variables|Default|GetCurrentViewportSize) (* (CallFunction|GetCameraMoveSpeedEdge) DeltaSeconds)))))))
    (:then_1
      (if (Variables|Default|GetDragMove)
        (CallFunction|CameraWheelMove DeltaSeconds)
        (else
          (CallFunction|CameraWheelRotate DeltaSeconds))))))

(event EventOnPlayerDisconnected
  (params (OldPlayer :type Ingame%20Controller%20Object%20Reference))
  ;[0.15 0.15 0.15 0.5] Control Link
  (|CallParentFunction OldPlayer)
  (Input|RemoveMappingContext OldPlayer "/Game/1_Core/Inputs/IMC_Operator.IMC_Operator" "(bIgnoreAllPressedKeysUntilRelease=True,bForceImmediately=False,bNotifyUserSettings=False)"))

(event Input|KeyboardEvents|AnyKey
  (params (Key :type Key%20Structure))
  (:Pressed
    (CallFunction|OnHotKeyDown Key)))

(fn ConstructionScript
  (|CallParentFunction)
  (Variables|Default|SetIndicator (Variables|Default|GetIndicatorInstance)))

(fn CreateIngameWidget
  (params (OwningPlayer :type Ingame%20Controller%20Object%20Reference))
  (bind _returnvalue (UserInterface|CreateWidget "/Game/1_Core/Widgets/Main/WB_Ingame.WB_Ingame_C" OwningPlayer))
  (bind _output_get (Variables|Default|SetIngameWidget _returnvalue))
  (Class|PlayerConnectable|OnPlayerConnected(Message) _output_get OwningPlayer)
  (UserInterface|Viewport|AddtoPlayerScreen (Variables|Default|GetIngameWidget))
  (return (Variables|Default|GetIngameWidget)))

(fn SetInputModeDefault
  (bind _playercontroller (Variables|Default|GetPlayerController)
    (:then
      (Input|SetInputModeGameandUI _playercontroller 0 "LockAlways" false true))
    (:else)))

(fn InitiateDragArea
  (bind _self self)
  (Variables|Default|GetDragAreaActor
    (:then)
    (:else
      (bind _returnvalue (Game|SpawnActorfromClass "/Game/1_Core/Blueprints/Actors/Players/BP_AreaSquare.BP_AreaSquare_C" (Math|Transform|MakeTransform "0, 0, 0" "-90.000000,0.000000,0.000000" "1.000000,1.000000,1.000000") "Undefined" "MultiplyWithRoot" _self _self))
      (bind _output_get (Variables|Default|SetDragAreaActor _returnvalue))
      (Rendering|SetActorHiddenInGame _output_get true))))

(fn InitiateController
  (params (NewController :type Ingame%20Controller%20Object%20Reference))
  (if (Pawn|IsLocalPlayerController NewController)
    (Input|AddMappingContext (PlayerController|LocalPlayerSubsystems|GetEnhancedInputLocalPlayerSubsystem NewController) "/Game/1_Core/Inputs/IMC_Operator.IMC_Operator" 0 "(bIgnoreAllPressedKeysUntilRelease=True,bForceImmediately=False,bNotifyUserSettings=False)")
    (CallFunction|SetInputModeDefault)))

(fn GetConnectedPlayerController
  (return (Variables|Default|GetPlayerController)))

(fn SpawnEffectonLocation
  (params (ShowOnlyOwner :type Boolean) (SystemTemplate :type Niagara%20System%20Object%20Reference) (InTransform :type Transform%20%28by%20ref%29) (Instigator :type Controller%20Object%20Reference))
  (bind (_location _rotation _scale) (Math|Transform|BreakTransform InTransform))
  (Utilities|IsValid SystemTemplate
    (:Is%20Valid
      (if (and (Utilities|IsValid SystemTemplate) (or (not ShowOnlyOwner) (and ShowOnlyOwner (Pawn|IsLocalPlayerController Instigator))))
        (Niagara|SpawnSystematLocation SystemTemplate _location _rotation _scale)))))

(fn OnHotKeyDown
  (params (TargetKey :type Key%20Structure :default "None"))
  (bind _array_element (Utilities|Array|ForEachLoopwithBreak (Class|Operator|GetAvaliableActionfromKey TargetKey) :!label _label)
    (:LoopBody
      (if (Variables|Default|GetbIsReservationMode)
        (Utilities|Array|Clear (LocalVariables|GetTargetActors))
        (for _array_element_2 (.components _array_element)
          (Utilities|IsValid (Components|GetOwner _array_element_2)
            (:Is%20Valid
              (Utilities|Array|AddUnique (LocalVariables|GetTargetActors) 0))))
        (Class|Operator|ReservationAction (.action _array_element) (LocalVariables|GetTargetActors) (Variables|Default|GetCurrentInputPackage) (Class|Operator|IsSmartKey (.action _array_element)))
        (else
          (Class|Operator|CommandAction (.action _array_element) (.components _array_element) (Class|Operator|IsSmartKey (.action _array_element)))
          (goto _label Break))))))

(fn CameraWheelMove
  (params (DeltaSeconds :type Float%20%28double-precision%29))
  (bind _output_get (LocalVariables|SetMoveAmount (Math|Vector|VectorLength (Variables|Default|GetClaimedWheelMove))))
  (if (> _output_get 0.0)
    (LocalVariables|SetMoveInDeltaSeconds (* DeltaSeconds (CallFunction|GetCameraMoveSpeedWheel)))
    (Class|Operator|RemoveFocusActor)
    (Class|Operator|CameraMove (Math|Vector|MakeVector (.X (Math|Vector|BreakVector (Math|Vector|SelectVector (* (Math|Vector|Normalize (Variables|Default|GetClaimedWheelMove)) (LocalVariables|GetMoveInDeltaSeconds)) (Variables|Default|GetClaimedWheelMove) (> (LocalVariables|GetMoveAmount) (LocalVariables|GetMoveInDeltaSeconds))))) (.Y (Math|Vector|BreakVector (Math|Vector|SelectVector (* (Math|Vector|Normalize (Variables|Default|GetClaimedWheelMove)) (LocalVariables|GetMoveInDeltaSeconds)) (Variables|Default|GetClaimedWheelMove) (> (LocalVariables|GetMoveAmount) (LocalVariables|GetMoveInDeltaSeconds))))) 0.0) (LocalVariables|GetMoveInDeltaSeconds))
    (Variables|Default|SetClaimedWheelMove (- (Variables|Default|GetClaimedWheelMove) (Math|Vector|SelectVector (* (Math|Vector|Normalize (Variables|Default|GetClaimedWheelMove)) (LocalVariables|GetMoveInDeltaSeconds)) (Variables|Default|GetClaimedWheelMove) (> (LocalVariables|GetMoveAmount) (LocalVariables|GetMoveInDeltaSeconds)))))))

(fn CameraWheelRotate
  (params (DeltaSeconds :type Float%20%28double-precision%29))
  (bind _output_get (LocalVariables|SetMoveAmount (Math|Vector|VectorLength (Variables|Default|GetClaimedWheelMove))))
  (if (> _output_get 0.0)
    (LocalVariables|SetMoveInDeltaSeconds (* DeltaSeconds (CallFunction|GetCameraRotateSpeedWheel)))
    (bind _output_get_2 (LocalVariables|SetMoveInCurrent (Math|Float|SelectFloat (* (Math|Float|Sign(Float) (* (.x (Variables|Default|GetClaimedWheelMove)) (CallFunction|GetCameraRotateMultiplyWheel))) (LocalVariables|GetMoveInDeltaSeconds)) (* (.x (Variables|Default|GetClaimedWheelMove)) (CallFunction|GetCameraRotateMultiplyWheel)) (> (Math|Float|Absolute(Float) (* (.x (Variables|Default|GetClaimedWheelMove)) (CallFunction|GetCameraRotateMultiplyWheel))) (Math|Float|Absolute(Float) (LocalVariables|GetMoveInDeltaSeconds))))))
    (Class|Actor|AddActorWorldRotation (Math|Rotator|MakeRotator 0.0 0.0 _output_get_2))
    (Variables|Default|SetClaimedWheelMove (Math|Vector|MakeVector (- (* (.x (Variables|Default|GetClaimedWheelMove)) (CallFunction|GetCameraRotateMultiplyWheel)) (LocalVariables|GetMoveInCurrent)) 0.0 0.0))))