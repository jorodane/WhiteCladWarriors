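; Fillable value Blueprint representing a unit's HP, extending a parent fillable value class.
; When a container connects, it binds to the current unit's die event and sets the value to zero on death.
; Its simplified fill color reflects the unit's ally color relative to the local operator, falling back to the parent color if either is invalid.
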(event Custom|OnUnitDie
  (params (TargetUnit :type Unit%20Main%20Component%20Object%20Reference) (LastAttackDamageInfo :type Damage%20Info%20Structure%20%28by%20ref%29))
  (Class|FloatValue|SetValue 0.0))

(event EventOnContainerConnected
  (params (NewContainer :type Value%20Container%20Object%20Reference))
  (|CallParentFunction NewContainer)
  (bind _currentunit (Variables|Default|GetCurrentUnit)
    (:then
      (EventDispatchers|BindEventtoOnUnitDie _currentunit (delegate Custom|OnUnitDie)))
    (:else)))

(fn GetSimplifiedFillColor
  (bind _output_get (LocalVariables|SetOperator (Class|Operator|GetLocalOperator)))
  (Utilities|IsValid _output_get
    (:Is%20Valid
      (bind _currentunit (Variables|Default|GetCurrentUnit)
        (:then
          (return (Utilities|GetAllyColorfromOperator _currentunit (LocalVariables|GetOperator))))
        (:else
          _)))
    (:Is%20Not%20Valid
      _))
  (return (|CallParentFunction)))