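; BP_FillableValue is a value with a current and maximum amount that presents itself as a fill bar in info UI.
; On container connection it creates ordered widget claims for a simple bar and a detail bar with centered text, and caches the owning unit.
; Connect and update callbacks push colors, values and percentage text through widget messages, and BroadcastDirty refreshes both bars.
; GetInfoWidget serves the simple bar for Minimal, the detail bar for Hover and Detail.
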(event Custom|ValueUpdate
  (params (NewWidget :type Generic%20Widget%20Base%20Object%20Reference))
  (bind _currentvalue (Variables|Default|GetCurrentValue))
  (bind _maxvalue (Variables|Default|GetMaxValue))
  (Class|ContainFloat2Value|SetFloat2(Message) NewWidget _currentvalue _maxvalue)
  (Class|ContainTextValue|SetText(Message) NewWidget (Utilities|Text|FormatText "{Current} / {Max} ({Percent}%)" _currentvalue _maxvalue (* (Math|Float|SafeDivide _currentvalue _maxvalue) 1e+02))))

(event Custom|SimpleBarConnect
  (params (NewParam :type Generic%20Widget%20Base%20Object%20Reference))
  (CallFunction|ValueUpdate NewParam)
  (Class|ContainBackgroundColorPaint|SetBackgroundColor(Message) NewParam (Variables|Default|GetBackgroundColor_Simple))
  (Class|ContainFillColorPaint|SetFillColor(Message) NewParam (Variables|Default|GetFillColor)))

(event Custom|DetailBarConnect
  (params (NewParam :type Generic%20Widget%20Base%20Object%20Reference))
  (CallFunction|ValueUpdate NewParam)
  (Class|ContainBackgroundColorPaint|SetBackgroundColor(Message) NewParam (Variables|Default|GetBackgroundColor_Detail))
  (Class|ContainFillColorPaint|SetFillColor(Message) NewParam (Variables|Default|GetFillColor)))

(event EventOnContainerConnected
  (params (NewContainer :type Value%20Container%20Object%20Reference))
  (CallFunction|CreateWidgetClaimers)
  (bind _outresult (Class|UnitMainComponent|TryGetUnit (Components|GetOwner NewContainer))
    (:True
      (Variables|Default|SetCurrentUnit _outresult))))

(fn BroadcastDirty
  (bind _returnvalue (|CallParentFunction))
  (bind _simplebar (Variables|Default|GetSimpleBar)
    (:then
      (Class|GenericWidgetClaim|UpdateWidgetRecursive _simplebar))
    (:else
      _))
  (bind _detailbar (Variables|Default|GetDetailBar)
    (:then
      (Class|GenericWidgetClaim|UpdateWidgetRecursive _detailbar))
    (:else
      _))
  (return _returnvalue))

(fn CreateWidgetClaimers
  (bind _returnvalue (Utilities|CreateWidgetClaimwithUpdater (Variables|Default|GetTextWidgetName) 0 (EventDispatchers|CreateEvent :!event Custom|ValueUpdate)))
  (Variables|/Script/WhiteCladWarriors.GenericWidgetClaim|SetWidgetTransform _returnvalue (Utilities|Map|MakeMap "HorizontalAlignment" 0.5 "VerticalAlignment" 0.5))
  (bind _returnvalue_2 (Utilities|CreateOrderedWidgetClaimwithEvent (Variables|Default|GetUIOrder) (Variables|Default|GetDetailBarWidgetName) (Utilities|Array|MakeArray _returnvalue) (EventDispatchers|CreateEvent :!event Custom|DetailBarConnect) (EventDispatchers|CreateEvent :!event Custom|ValueUpdate)))
  (bind _output_get (Variables|Default|SetDetailBar _returnvalue_2))
  (Variables|/Script/WhiteCladWarriors.GenericWidgetClaim|SetWidgetTransform _output_get (Utilities|Map|MakeMap "VerticalSize" (Variables|Default|GetDetailHeight)))
  (bind _returnvalue_3 (Utilities|CreateOrderedWidgetClaimwithEvent (Variables|Default|GetUIOrder) "FillBar" 0 (EventDispatchers|CreateEvent :!event Custom|SimpleBarConnect) (EventDispatchers|CreateEvent :!event Custom|ValueUpdate)))
  (bind _output_get_2 (Variables|Default|SetSimpleBar _returnvalue_3))
  (Variables|/Script/WhiteCladWarriors.GenericWidgetClaim|SetWidgetTransform _output_get_2 (Utilities|Map|MakeMap "VerticalSize" (Variables|Default|GetSimpleHeight))))

(fn GetInfoWidget
  (params (WantType :type EInfoWidgetType%20Enum :default "Minimal") (Operator :type Operator%20Object%20Reference))
  (bind _detailbar (Variables|Default|GetDetailBar))
  (return (Utilities|Array|MakeArray (Utilities|Select :Index WantType :Minimal (Variables|Default|GetSimpleBar) :Hover _detailbar :Detail _detailbar :Inspector 0))))

(fn GetInfoWorldPosition
  (return "0, 0, 0"))