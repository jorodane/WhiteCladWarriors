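; Experience value, a fillable value that levels up its owner each time it fills.
; It finds or adds a level number object by tag on its container; filling resets EXP to zero, grows the maximum by 25% and adds a level, while overflow is added back.
; A widget-claim text and bar, with level in the text, serves the Detail view, hidden when the unit is not the operator's own.
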(event EventOnContainerConnected
  (params (NewContainer :type Value%20Container%20Object%20Reference))
  (|CallParentFunction NewContainer)
  (bind _returnvalue (Class|ValueContainer|FindorAddNumberObject NewContainer (Variables|Default|GetLevelTag) (Variables|Default|GetStartLevel) "/Script/WhiteCladWarriors.FloatValue"))
  (Variables|Default|SetLevelValue _returnvalue))

(fn GetInfoWidget
  (params (WantType :type EInfoWidgetType%20Enum :default "Minimal") (Operator :type Operator%20Object%20Reference))
  (bind _currentunit (Variables|Default|GetCurrentUnit)
    (:then
      (if (Utilities|Enum|Equal(Enum) (Class|UnitMainComponent|GetAllyTypefromOperator _currentunit Operator) "Own")
        _
        (else
          (return 0))))
    (:else
      _))
  (return (Utilities|Array|MakeArray (Utilities|Select :Index WantType :Minimal 0 :Hover 0 :Detail (Variables|Default|GetDetailBar) :Inspector 0))))

(fn OnValueFull
  (|CallParentFunction)
  (bind _returnvalue (Class|FillableValue|SetFillValue 0.0 (* (Variables|Default|GetMaxValue) 1.25)))
  (CallFunction|LevelUp 1)
  (return _returnvalue))

(fn LevelUp
  (params (Amount :type Integer))
  (bind _levelvalue (Variables|Default|GetLevelValue)
    (:then
      (Class|FloatValue|AddValue _levelvalue (Math|Conversions|ToFloat(Integer) Amount)))
    (:else)))

(fn OnValueOverflow
  (params (AbsoluteValue :type Float%20%28single-precision%29))
  (bind _returnvalue (|CallParentFunction AbsoluteValue))
  (bind _returnvalue_2 (Class|FloatValue|AddValue _returnvalue))
  (return _returnvalue_2))

(fn CreateWidgetClaimers
  (bind _returnvalue (Utilities|CreateWidgetClaimwithUpdater (Variables|Default|GetTextWidgetName) 0 (EventDispatchers|CreateEvent :!event ValueUpdate)))
  (Variables|/Script/WhiteCladWarriors.GenericWidgetClaim|SetWidgetTransform _returnvalue (Utilities|Map|MakeMap "HorizontalAlignment" 0.5 "Padding_Vertical" -5.0))
  (bind _returnvalue_2 (Utilities|CreateWidgetClaimwithEvent (Variables|Default|GetDetailBarWidgetName) 0 (EventDispatchers|CreateEvent :!event DetailBarConnect) (EventDispatchers|CreateEvent :!event ValueUpdate)))
  (Variables|/Script/WhiteCladWarriors.GenericWidgetClaim|SetWidgetTransform _returnvalue_2 (Utilities|Map|MakeMap "VerticalSize" (Variables|Default|GetDetailHeight)))
  (bind _returnvalue_3 (Utilities|CreateOrderedWidgetClaim (Variables|Default|GetUIOrder) "VerticalBox" (Utilities|Array|MakeArray _returnvalue _returnvalue_2)))
  (Variables|Default|SetDetailBar _returnvalue_3))

(fn GetValueText
  (bind _levelvalue (Variables|Default|GetLevelValue)
    (:then
      (return (Utilities|Text|FormatText (Variables|Default|GetTextFormat) (Variables|Default|GetCurrentValue) (CallFunction|GetPercentText) (Class|FloatValue|GetValue _levelvalue))))
    (:else
      (return (|CallParentFunction)))))