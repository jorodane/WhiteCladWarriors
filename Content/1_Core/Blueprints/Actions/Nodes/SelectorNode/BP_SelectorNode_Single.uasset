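; BP_SelectorNode_Single is an action-graph selector node that requests a single input, such as a position, direction or actor, for an action cursor.
; On execute it sends an input claim with executor components, descriptions, cursor type and ready montage to the cursor's operator.
; Received values pass separate Check functions before being written to the cursor by tag.
; Default checks accept any position, spawning a check effect, any direction, and any valid actor.
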(event EventClaimExecute
  (params (WantCursor :type Action%20Cursor%20Finder%20Structure%20%28by%20ref%29))
  (bind (_currentaction _currentoperator _currentexecutorid) (Utilities|Struct|BreakActionCursorFinder WantCursor))
  (Utilities|IsValid _currentoperator
    (:Is%20Valid
      (Class|Operator|ClaimInput _currentoperator (CallFunction|GetInputClaim (Class|ActionExecutor|GetComponentArray (Class|ActionExecutor|GetExecutorfromID _currentexecutorid)) _currentaction _currentexecutorid)))))

(event EventClaimExecutewithInput
  (params (WantCursor :type Action%20Cursor%20Finder%20Structure%20%28by%20ref%29) (Input :type Input%20Package%20Structure%20%28by%20ref%29))
  (Class|ActionSelectorNode|ReceiveInput WantCursor Input))

(fn OnReceivePosition
  (params (WantCursor :type Action%20Cursor%20Finder%20Structure%20%28by%20ref%29) (TargetTag :type Name%20%28by%20ref%29 :default "None") (TargetPosition :type Vector%20%28by%20ref%29 :default "0, 0, 0"))
  (bind _returnvalue (CallFunction|CheckPosition WantCursor TargetTag TargetPosition))
  (if _returnvalue
    (Class|ActionExecutor|SetVectortoCursor WantCursor TargetTag TargetPosition)
    (return true)
    (else
      (return false))))

(fn OnReceiveDirection
  (params (WantCursor :type Action%20Cursor%20Finder%20Structure%20%28by%20ref%29) (TargetTag :type Name%20%28by%20ref%29 :default "None") (TargetDirection :type Vector%20%28by%20ref%29 :default "0, 0, 0"))
  (LocalVariables|SetWantTag TargetTag)
  (LocalVariables|SetWantDirection TargetDirection)
  (bind _returnvalue (CallFunction|CheckDirection WantCursor (LocalVariables|GetWantTag) (LocalVariables|GetWantDirection)))
  (if _returnvalue
    (Class|ActionExecutor|SetVectortoCursor WantCursor (LocalVariables|GetWantTag) (LocalVariables|GetWantDirection))
    (return true)
    (else
      (return false))))

(fn OnReceiveActor
  (params (WantCursor :type Action%20Cursor%20Finder%20Structure%20%28by%20ref%29) (TargetTag :type Name%20%28by%20ref%29 :default "None") (TargetActor :type Actor%20Object%20Reference))
  (bind _returnvalue (CallFunction|CheckActor WantCursor TargetTag TargetActor))
  (if _returnvalue
    (Utilities|IsValid TargetActor
      (:Is%20Valid
        (Class|ActionExecutor|SetActortoCursor WantCursor TargetTag TargetActor)
        (return true))
      (:Is%20Not%20Valid
        _)))
  (return false))

(fn CheckActor
  (params (WantCursor :type Action%20Cursor%20Finder%20Structure%20%28by%20ref%29) (TargetTag :type Name%20%28by%20ref%29 :default "None") (TargetActor :type Actor%20Object%20Reference))
  (return (Utilities|IsValid TargetActor)))

(fn CheckPosition
  (params (WantCursor :type Action%20Cursor%20Finder%20Structure%20%28by%20ref%29) (TargetTag :type Name%20%28by%20ref%29 :default "None") (TargetPosition :type Vector%20%28by%20ref%29 :default "0, 0, 0"))
  (bind (_currentaction _currentoperator) (Utilities|Struct|BreakActionCursorFinder WantCursor))
  (Class|ActionBase|SpawnCheckEffect _currentaction true _currentoperator (Utilities|Struct|MakeInputPackage TargetPosition TargetPosition 0 0 0) "Position" (Utilities|Text|FormatText ""))
  (return true))

(fn CheckDirection
  (params (WantCursor :type Action%20Cursor%20Finder%20Structure%20%28by%20ref%29) (TargetTag :type Name%20%28by%20ref%29 :default "None") (TargetDirection :type Vector%20%28by%20ref%29 :default "0, 0, 0"))
  (return true))

(fn GetInputClaim
  (params (TargetComponent :type Array%20of%20Unit%20Action%20Component%20Object%20References) (TargetAction :type Action%20Base%20Object%20Reference) (ExecutorID :type Integer64))
  (return (Utilities|Struct|MakeInputClaim (Utilities|Struct|MakeActionCursorFinder TargetAction 0 ExecutorID) TargetComponent self (Variables|Default|GetDescription) (Variables|Default|GetCursorDescription) (Variables|Default|GetCursorType) (Variables|Default|GetReadyMontage))))