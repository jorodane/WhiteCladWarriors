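; Action node that requests a position from an executor's Operator and sends the executor's targets there.
; On execution it claims input from a valid Operator, passing itself, the executor, a location tag and a description.
; When a position arrives, it enters the node on the executor, then issues AI MoveTo to each target's owning Character without waiting for arrival.
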(event EventClaimExecute
  (params (Executor :type Action%20Executor%20Object%20Reference))
  (bind _operator (Variables|/Script/WhiteCladWarriors.ActionExecutor|GetOperator Executor)
    (:then
      (Class|Operator|ClaimInput _operator (Utilities|Struct|MakeInputClaim "Position" self Executor (Variables|Default|GetLocationTag) (Variables|Default|GetDescription))))
    (:else)))

(event EventOnPositionInput
  (params (Executor :type Action%20Executor%20Object%20Reference) (Position :type Vector :default "0, 0, 0"))
  (Class|ActionExecutor|EnterNode Executor)
  (for _array_element (Variables|/Script/WhiteCladWarriors.ActionExecutor|GetTarget Executor)
    (bind _as캐릭터 (Utilities|Casting|CastToCharacter (Components|GetOwner _array_element)))
    (AI|AIMoveTo _as캐릭터 _as캐릭터 Position 0 5.0 false)))