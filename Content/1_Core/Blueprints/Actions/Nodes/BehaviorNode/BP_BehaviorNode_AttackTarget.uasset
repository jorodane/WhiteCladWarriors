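; A behavior node in the action system that orders a unit's attack component to attack a target and shows an attack range indicator.
; On execute it passes the target actor resolved from the cursor to the attack component, cancelling if either is invalid.
; Complete or failed messages advance or cancel the cursor; ending the node closes sub-nodes and sets a stop message.
; It claims one range indicator per targeted component, sized by the unit's AttackRange value.
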(event EventClaimExecute
  (params (WantCursor :type Action%20Cursor%20Finder%20Structure%20%28by%20ref%29))
  (bind _asbp_action_attack_component (Utilities|Casting|CastToBP_ActionAttackComponent (.CurrentComponent (Utilities|Struct|BreakActionCursorFinder WantCursor)))
    (:then
      (bind _attacktarget (Variables|Default|GetAttackTarget)
        (:then
          (Class|UnitAttackComponent|BeginAttackTarget _asbp_action_attack_component (Class|ActorClaimer|GetActor _attacktarget WantCursor) WantCursor))
        (:else
          (Class|ActionNode|MoveExecutortoCancel WantCursor :!label _label))))
    (:CastFailed
      (goto _label))))

(event EventUpdateIndicatorSingle
  (params (TargetNode :type Action%20Behavior%20Node%20Object%20Reference) (TargetInput :type Input%20Claim%20Structure%20%28by%20ref%29) (InputPackage :type Input%20Package%20Structure%20%28by%20ref%29) (TargetComponent :type Unit%20Action%20Component%20Object%20Reference) (TargetShower :type Action%20Indicator%20Shower%20Base%20Object%20Reference) (TargetUnit :type Unit%20Main%20Component%20Object%20Reference) (Index :type Integer) (bIsIconPreview :type Boolean))
  (Utilities|IsValid TargetUnit
    (:Is%20Valid
      (bind _valuemap (Variables|/Script/WhiteCladWarriors.UnitMainComponent|GetValueMap TargetUnit)
        (:then
          (bind _returnvalue (Class|ValueContainer|GetNumber _valuemap "AttackRange" 0.0))
          (Class|ActionIndicatorShowerBase|Drawat TargetShower (Class|UnitComponentBase|GetLocation TargetUnit) _returnvalue))
        (:else)))))

(event EventOnActionMessageSimple
  (params (WantCursor :type Action%20Cursor%20Finder%20Structure%20%28by%20ref%29) (Message :type Name%20%28by%20ref%29 :default "None"))
  (switch name Message
    (:AttackComplete
      (Class|ActionNode|MoveExecutortoNext WantCursor))
    (:AttackFailed
      (Class|ActionNode|MoveExecutortoCancel WantCursor))))

(event EventOnComplete
  (params (WantCursor :type Action%20Cursor%20Finder%20Structure%20%28by%20ref%29))
  (Class|ActionNode|EndAllSubNodes WantCursor)
  (Class|Stoppable|SetStop(Message) (.CurrentComponent (Utilities|Struct|BreakActionCursorFinder WantCursor))))

(event EventOnCancel
  (params (WantCursor :type Action%20Cursor%20Finder%20Structure%20%28by%20ref%29))
  (Class|ActionNode|EndAllSubNodes WantCursor)
  (Class|Stoppable|SetStop(Message) (.CurrentComponent (Utilities|Struct|BreakActionCursorFinder WantCursor))))

(fn GetIndicatorClaim
  (params (TargetInput :type Input%20Claim%20Structure%20%28by%20ref%29))
  (return (Utilities|Map|MakeMap self (Utilities|Struct|MakeIndicatorClaim "Range" (Utilities|Array|Length (.targetcomponentarray TargetInput))))))