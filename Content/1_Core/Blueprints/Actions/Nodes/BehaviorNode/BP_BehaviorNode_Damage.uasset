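; Behavior node that deals damage to a target actor as one step of an action's behavior flow.
; Target, Damage and Direction providers resolve from the cursor into a damage info, sent via message after a damageable check.
; Positive damage notifies the current operator and owner unit, then advances the executor.
; Non-damageable targets branch to OnNotDamageable as canceled, while invalid inputs or zero damage cancel.
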(event EventClaimExecute
  (params (WantCursor :type Action%20Cursor%20Finder%20Structure%20%28by%20ref%29))
  (bind (_currentaction _currentoperator _currentexecutorid _currentcomponent) (Utilities|Struct|BreakActionCursorFinder WantCursor))
  (bind _damage (Variables|Default|GetDamage))
  (bind _target (Variables|Default|GetTarget))
  (bind _direction (Variables|Default|GetDirection))
  (bind _returnvalue (Class|UnitComponentBase|GetOwnerUnit _currentcomponent))
  (bind _returnvalue_2 (Class|FloatClaimer|GetValue _damage WantCursor 0.0))
  (bind _returnvalue_3 (Components|GetOwner _currentcomponent))
  (bind _returnvalue_4 (Class|ActorClaimer|GetActor _target WantCursor))
  (bind _returnvalue_5 (Transformation|GetActorLocation _returnvalue_3))
  (bind _returnvalue_6 (Transformation|GetActorForwardVector _returnvalue_3))
  (bind _returnvalue_7 (Class|DirectionClaimer|GetDirection _direction WantCursor _returnvalue_5 _returnvalue_6))
  (bind _damageinfo (Utilities|Struct|MakeDamageInfo _returnvalue_2 _returnvalue_7 _returnvalue_3 _returnvalue))
  (Utilities|IsValid _returnvalue_3
    (:Is%20Valid
      (if (Math|Boolean|ANDBoolean (Utilities|IsValid (Variables|Default|GetTarget)) (Utilities|IsValid (Variables|Default|GetDamage)) (Utilities|IsValid (Variables|Default|GetDirection)))
        (Utilities|IsValid _returnvalue_4
          (:Is%20Valid
            (bind _returnvalue_8 (Class|Damageable|GetIsDamageable(Message) _returnvalue_4 _returnvalue))
            (if _returnvalue_8
              (bind (_biskill _returnvalue_9) (Class|Damageable|TakeDamage(Message) _returnvalue_4 _damageinfo))
              (if (> _returnvalue_9 0.0)
                (Utilities|IsValid _currentoperator
                  (:Is%20Valid
                    (Default|CallOnSuccessDamage _currentoperator _returnvalue_4 _biskill _returnvalue_9 _damageinfo))
                  (:Is%20Not%20Valid
                    _))
                (Utilities|IsValid _returnvalue
                  (:Is%20Valid
                    (Default|CallOnSuccessDamage _returnvalue _returnvalue_4 _biskill _returnvalue_9 _damageinfo))
                  (:Is%20Not%20Valid
                    _))
                (Class|ActionNode|MoveExecutortoNext WantCursor)
                (else
                  (Class|ActionNode|MoveExecutortoCancel WantCursor :!label _label)))
              (else
                (Class|ActionNode|MoveExecutortoWantNode WantCursor (Variables|Default|GetOnNotDamageable) true))))
          (:Is%20Not%20Valid
            (Class|ActionNode|MoveExecutortoCancel WantCursor)))
        (else
          (goto _label))))
    (:Is%20Not%20Valid
      (goto _label))))