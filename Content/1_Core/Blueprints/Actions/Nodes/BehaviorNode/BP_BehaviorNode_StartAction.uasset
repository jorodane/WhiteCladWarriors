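; BP_BehaviorNode_StartAction is a behavior node, apparently meant to start a unit action from a behavior cursor.
; ClaimExecute advances the cursor when it has a valid operator and its component resolves an owner unit, otherwise cancels it.
; The ExecuteActionWithInput call, fed by the unit's action components and target position and actor, is disconnected, so no action is actually started.
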(event EventClaimExecute
  (params (WantCursor :type Action%20Cursor%20Finder%20Structure%20%28by%20ref%29))
  (bind (_currentaction _currentoperator _currentexecutor _currentcomponent) (Utilities|Struct|BreakActionCursorFinder WantCursor))
  (Utilities|IsValid _currentoperator
    (:Is%20Valid
      (bind _resultunit (Class|UnitComponentBase|TryGetOwnerUnit _currentcomponent)
        (:True
          (Class|ActionNode|MoveExecutortoNext WantCursor))
        (:False
          (Class|ActionNode|MoveExecutortoCancel WantCursor :!label _label))))
    (:Is%20Not%20Valid
      (goto _label))))