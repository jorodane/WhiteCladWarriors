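; Behavior node that spawns visual effects for an action, then advances the executor to the next node.
; It casts the cursor's operator to BP_Operator and has it spawn an optional effect at a position claimed from the current executor.
; It also loops over claimed actors, optionally spawning an effect at each location and playing a selection effect that flags whether only one actor is selected.
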(event EventClaimExecute
  (params (WantCursor :type Action%20Cursor%20Finder%20Structure%20%28by%20ref%29))
  (CallFunction|SpawnEffect WantCursor)
  (Class|ActionNode|MoveExecutortoNext WantCursor))

(fn SpawnEffect
  (params (Cursor :type Action%20Cursor%20Finder%20Structure))
  (bind _output_get (LocalVariables|SetCurrentCursor Cursor))
  (bind _asbp_operator (Utilities|Casting|CastToBP_Operator (.CurrentOperator (Utilities|Struct|BreakActionCursorFinder _output_get))))
  (LocalVariables|SetCurrentOperator _asbp_operator)
  (Utilities|FlowControl|Sequence
    (:then_0
      (bind _effectonposition (Variables|Default|GetEffectOnPosition)
        (:then
          (Default|SpawnEffectonLocation (LocalVariables|GetCurrentOperator) (Variables|Default|GetShow%20Only%20Owner) _effectonposition (Math|Transform|MakeTransform (Class|ActionExecutor|GetPosition (.currentexecutor (LocalVariables|GetCurrentCursor)) (LocalVariables|GetCurrentCursor) (Variables|Default|GetEffectPosition)) "0, 0, 0" "1.000000,1.000000,1.000000") (Pawn|GetController (LocalVariables|GetCurrentOperator))))
        (:else)))
    (:then_1
      (LocalVariables|SetSingleSelected (== (Utilities|Array|Length (Class|ActionExecutor|GetActorArray (.currentexecutor (LocalVariables|GetCurrentCursor)) (LocalVariables|GetCurrentCursor) (Variables|Default|GetEffectActors))) 1))
      (for _array_element (Class|ActionExecutor|GetActorArray (.currentexecutor (LocalVariables|GetCurrentCursor)) (LocalVariables|GetCurrentCursor) (Variables|Default|GetEffectActors))
        (Utilities|FlowControl|Sequence
          (:then_0
            (bind _effectonactor (Variables|Default|GetEffectOnActor)
              (:then
                (Default|SpawnEffectonLocation (LocalVariables|GetCurrentOperator) (Variables|Default|GetShow%20Only%20Owner) _effectonactor (Math|Transform|MakeTransform (Transformation|GetActorLocation _array_element) "0, 0, 0" "1.000000,1.000000,1.000000")))
              (:else)))
          (:then_1
            (if (Variables|Default|GetActorSelectEffect)
              (Class|Selectable|PlaySelectEffect(Message) _array_element (LocalVariables|GetCurrentOperator) (LocalVariables|GetSingleSelected)))))))))