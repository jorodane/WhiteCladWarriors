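; Base-style behavior node that starts unit movement as a step in an action, with placeholder destination, target actor and move-start hooks.
; On execute it claims movement on the cursor's owner unit, using an optional acceptance radius with a fallback.
; Move success or failure messages advance or cancel the executor, and a failed claim also cancels.
; It also claims range indicators, drawn at valid target units at the acceptance radius's width.
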(event EventClaimExecute
  (params (WantCursor :type Action%20Cursor%20Finder%20Structure%20%28by%20ref%29))
  (bind _currentcomponent (Utilities|Struct|BreakActionCursorFinder WantCursor))
  (bind _resultunit (Class|UnitActionComponent|TryGetOwnerUnit _currentcomponent)
    (:True
      (bind _returnvalue (Class|UnitMainComponent|ClaimStartMovement _resultunit (CallFunction|GetDestination WantCursor (Transformation|GetActorLocation (Components|GetOwner _currentcomponent))) (CallFunction|GetTargetActor WantCursor) (CallFunction|GetAcceptanceRadius) WantCursor))
      (if _returnvalue
        (CallFunction|StartMove WantCursor)
        (else
          (CallFunction|FailtoMove WantCursor))))))

(event EventUpdateIndicatorSingle
  (params (TargetNode :type Action%20Behavior%20Node%20Object%20Reference) (TargetInput :type Input%20Claim%20Structure%20%28by%20ref%29) (InputPackage :type Input%20Package%20Structure%20%28by%20ref%29) (TargetComponent :type Unit%20Action%20Component%20Object%20Reference) (TargetShower :type Action%20Indicator%20Shower%20Base%20Object%20Reference) (TargetUnit :type Unit%20Main%20Component%20Object%20Reference) (Index :type Integer) (bIsIconPreview :type Boolean))
  (Utilities|IsValid TargetUnit
    (:Is%20Valid
      (Class|ActionIndicatorShowerBase|Drawat TargetShower (Transformation|GetActorLocation (Components|GetOwner TargetUnit)) (CallFunction|GetAcceptanceRadius)))))

(event EventOnActionMessageSimple
  (params (WantCursor :type Action%20Cursor%20Finder%20Structure%20%28by%20ref%29) (Message :type Name%20%28by%20ref%29 :default "None"))
  (if (== Message (Class|ReservedActionMessage|GetActionMessageMoveSucceed))
    (Class|ActionNode|OnComplete WantCursor)
    (CallFunction|CompleteMove WantCursor)
    (elif (== Message (Class|ReservedActionMessage|GetActionMessageMoveFailed))
      (CallFunction|FailtoMove WantCursor))))

(fn GetIndicatorClaim
  (params (TargetInput :type Input%20Claim%20Structure%20%28by%20ref%29))
  (return (Utilities|Map|MakeMap self (Utilities|Struct|MakeIndicatorClaim "Range" (Utilities|Array|Length (.targetcomponentarray TargetInput))))))

(fn GetAcceptanceRadius
  (bind _acceptance_radius (Variables|Default|GetAcceptance%20Radius)
    (:then
      (return (Class|FloatGetter|GetValue _acceptance_radius)))
    (:else
      (return 5.0))))

(fn GetDestination
  (params (WantCursor :type Action%20Cursor%20Finder%20Structure%20%28by%20ref%29) (DefaultValue :type Vector%20%28by%20ref%29))
  (return "0, 0, 0"))

(fn GetTargetActor
  (params (WantCursor :type Action%20Cursor%20Finder%20Structure%20%28by%20ref%29))
  (return 0))

(fn FailtoMove
  (params (WantCursor :type Action%20Cursor%20Finder%20Structure%20%28by%20ref%29))
  (Class|ActionNode|MoveExecutortoCancel WantCursor))

(fn StartMove
  (params (WantCursor :type Action%20Cursor%20Finder%20Structure%20%28by%20ref%29)))

(fn CompleteMove
  (params (WantCursor :type Action%20Cursor%20Finder%20Structure%20%28by%20ref%29))
  (Class|ActionNode|MoveExecutortoNext WantCursor))