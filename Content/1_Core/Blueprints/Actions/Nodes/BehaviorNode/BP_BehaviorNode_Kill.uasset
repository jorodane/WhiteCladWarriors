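; Behavior node that kills or removes the actor resolved from its TargetActor for the executing cursor.
; It sends the target a destroy message, then calls Die on units with damage direction and causer from the owner unit, or a fallback without one.
; Non-units are either returned to their pool through the Poolable interface or destroyed.
; The executor advances afterward, or cancels if no valid target exists.
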(event EventClaimExecute
  (params (WantCursor :type Action%20Cursor%20Finder%20Structure%20%28by%20ref%29))
  (bind (_currentaction _currentoperator _currentexecutorid _currentcomponent _claimactor) (Utilities|Struct|BreakActionCursorFinder WantCursor))
  (bind _returnvalue (Class|UnitComponentBase|GetOwnerUnit _currentcomponent))
  (bind _returnvalue_2 (Components|GetOwner _returnvalue))
  (bind _targetactor (Variables|Default|GetTargetActor)
    (:then
      (Utilities|IsValid (Class|ActorClaimer|GetActor _targetactor WantCursor _currentcomponent)
        (:Is%20Valid
          (Class|DestroyFunctionable|OnDestroyFunction(Message) (Class|ActorClaimer|GetActor _targetactor WantCursor _currentcomponent))
          (bind _outresult (Class|UnitMainComponent|TryGetUnit (Class|ActorClaimer|GetActor _targetactor WantCursor _currentcomponent))
            (:True
              (Utilities|IsValid _returnvalue
                (:Is%20Valid
                  (Class|UnitMainComponent|Die _outresult (Utilities|Struct|MakeDamageInfo 0.0 (Math|Rotator|GetRotationXVector (Math|Rotator|FindLookatRotation (Transformation|GetActorLocation (Class|ActorClaimer|GetActor _targetactor WantCursor _currentcomponent)) (Transformation|GetActorLocation _returnvalue_2))) _returnvalue_2 _returnvalue)))
                (:Is%20Not%20Valid
                  (Class|UnitMainComponent|Die _outresult (Utilities|Struct|MakeDamageInfo 0.0 (* (Transformation|GetActorForwardVector (Class|ActorClaimer|GetActor _targetactor WantCursor _currentcomponent)) -1.0) _claimactor 0)))))
            (:False
              (if (Utilities|DoesObjectImplementInterface _outresult "/Script/WhiteCladWarriors.Poolable")
                (bind _returnvalue_3 (Class|Poolable|ClaimPoolEnqueue(Message) (Class|ActorClaimer|GetActor _targetactor WantCursor _currentcomponent)))
                (if _returnvalue_3
                  _
                  (else
                    (Actor|DestroyActor (Class|ActorClaimer|GetActor _targetactor WantCursor _currentcomponent) :!label _label)))
                (else
                  (goto _label)))))
          (Class|ActionNode|MoveExecutortoNext WantCursor))
        (:Is%20Not%20Valid
          (Class|ActionNode|MoveExecutortoCancel WantCursor :!label _label_2))))
    (:else
      (goto _label_2))))