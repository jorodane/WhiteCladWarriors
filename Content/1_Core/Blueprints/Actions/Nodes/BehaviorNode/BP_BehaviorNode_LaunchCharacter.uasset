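; Action behavior node that launches a Character in a chosen direction at a set speed, overriding its velocity.
; LaunchActor and LaunchDirection resolve target and direction from the cursor and component, then execution advances to the next node.
; It claims one arrow indicator per target component, sized by Range and capsule diameter.
; The arrow's default direction points toward the mouse terrain position, or along actor forward for icon previews.
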(event EventClaimExecute
  (params (WantCursor :type Action%20Cursor%20Finder%20Structure%20%28by%20ref%29))
  (bind _currentcomponent (Utilities|Struct|BreakActionCursorFinder WantCursor))
  (bind _launchactor (Variables|Default|GetLaunchActor))
  (bind _returnvalue (Class|ActorClaimer|GetActor _launchactor WantCursor _currentcomponent))
  (Utilities|IsValid _currentcomponent
    (:Is%20Valid
      (bind _as캐릭터 (Utilities|Casting|CastToCharacter _returnvalue))
      (Character|LaunchCharacter _as캐릭터 (* (Class|DirectionClaimer|GetDirection (Variables|Default|GetLaunchDirection) WantCursor _currentcomponent (Transformation|GetActorLocation _returnvalue) (Transformation|GetActorForwardVector _returnvalue)) (Variables|Default|GetSpeed)) true true)
      (Class|ActionNode|MoveExecutortoNext WantCursor))))

(event EventUpdateIndicatorSingle
  (params (TargetNode :type Action%20Behavior%20Node%20Object%20Reference) (TargetInput :type Input%20Claim%20Structure%20%28by%20ref%29) (InputPackage :type Input%20Package%20Structure%20%28by%20ref%29) (TargetComponent :type Unit%20Action%20Component%20Object%20Reference) (TargetShower :type Action%20Indicator%20Shower%20Base%20Object%20Reference) (TargetUnit :type Unit%20Main%20Component%20Object%20Reference) (Index :type Integer) (bIsIconPreview :type Boolean))
  (bind _targetactioncursor (Utilities|Struct|BreakInputClaim TargetInput))
  (bind _launchactor (Variables|Default|GetLaunchActor))
  (bind _launchdirection (Variables|Default|GetLaunchDirection))
  (bind _returnvalue (Class|ActorClaimer|GetActor _launchactor _targetactioncursor TargetComponent))
  (bind _returnvalue_2 (Transformation|GetActorLocation _returnvalue))
  (Utilities|IsValid TargetUnit
    (:Is%20Valid
      (bind _as캐릭터 (Utilities|Casting|CastToCharacter _returnvalue))
      (Default|SetPercent TargetShower (Class|ActionNode|GetPercent _targetactioncursor))
      (Default|DrawfromDirection TargetShower (Class|DirectionClaimer|GetStartPosition _launchdirection _targetactioncursor TargetComponent _returnvalue_2) (Class|DirectionClaimer|GetDirection _launchdirection _targetactioncursor TargetComponent _returnvalue_2 (Math|Vector|SelectVector (Transformation|GetActorForwardVector _returnvalue) (Class|KismetMathLibrary|VectorNormal2D (- (.MouseTerrainPosition (Utilities|Struct|BreakInputPackage InputPackage)) _returnvalue_2) 0.0001) bIsIconPreview)) (Variables|Default|GetRange) (* (Components|Capsule|GetScaledCapsuleRadius (Variables|/Script/Engine.Character|GetCapsuleComponent _as캐릭터)) 2.0)))))

(fn GetIndicatorClaim
  (params (TargetInput :type Input%20Claim%20Structure%20%28by%20ref%29))
  (return (Utilities|Map|MakeMap self (Utilities|Struct|MakeIndicatorClaim "Arrow" (Utilities|Array|Length (.targetcomponentarray TargetInput))))))