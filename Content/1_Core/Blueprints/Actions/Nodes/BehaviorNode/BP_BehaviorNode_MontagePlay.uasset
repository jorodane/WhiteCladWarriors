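; Behavior node that plays a main action montage on the owner unit and drives the action cursor from its result.
; The focus target comes from the montage info, falling back to the node's FocusTarget; a successful start spawns the OnMontageStart sub-node.
; Completion advances the executor, while failure or interruption cancels it.
; Montage notify messages jump to linked nodes by context name, and cancelling stops the montage.
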(event EventClaimExecute
  (params (WantCursor :type Action%20Cursor%20Finder%20Structure%20%28by%20ref%29))
  (bind _playmontageinfo (Variables|Default|GetPlayMontageInfo))
  (bind _resultunit (Class|UnitComponentBase|TryGetOwnerUnit (.CurrentComponent (Utilities|Struct|BreakActionCursorFinder WantCursor)))
    (:True
      (Utilities|IsValid (.focustarget (Variables|Default|GetPlayMontageInfo))
        (:Is%20Valid
          (bind _returnvalue (Class|UnitMainComponent|PlayMainActionMontage _resultunit (Variables|Default|GetPlayMontageInfo) :!label _label))
          (if _returnvalue
            (bind _onmontagestart (Variables|Default|GetOnMontageStart :!label _label_2)
              (:then
                (Class|ActionNode|CreateSubNode WantCursor _onmontagestart))
              (:else))
            (else
              (Class|ActionNode|MoveExecutortoCancel WantCursor :!label _label_3))))
        (:Is%20Not%20Valid
          (Utilities|IsValid (Variables|Default|GetFocusTarget)
            (:Is%20Valid
              (bind _focustarget (Variables|Default|GetFocusTarget)
                (:then
                  (Utilities|IsValid (Class|ActorClaimer|GetActor _focustarget WantCursor)
                    (:Is%20Valid
                      (bind _returnvalue_2 (Class|UnitMainComponent|PlayMainActionMontage _resultunit (Utilities|Struct|MakeMontageEventInfo (.montagetoplay _playmontageinfo) (Class|ActorClaimer|GetActor _focustarget WantCursor) (.playrate _playmontageinfo) (.startingposition _playmontageinfo) (.blendintime _playmontageinfo) (.blendouttime _playmontageinfo))))
                      (if _returnvalue_2
                        (goto _label_2)
                        (else
                          (goto _label_3))))
                    (:Is%20Not%20Valid
                      (goto _label))))
                (:else
                  (goto _label))))
            (:Is%20Not%20Valid
              (goto _label))))))
    (:False
      (goto _label_3))))

(event EventOnActionMessageMontage
  (params (WantCursor :type Action%20Cursor%20Finder%20Structure%20%28by%20ref%29) (Montage :type Anim%20Montage%20Object%20Reference) (bIsStart :type Boolean) (bIsInterrupted :type Boolean))
  (if (== Montage (.montagetoplay (Variables|Default|GetPlayMontageInfo)))
    (if (not bIsStart)
      (if bIsInterrupted
        (Class|ActionNode|MoveExecutortoCancel WantCursor)
        (Variables|Default|GetEndAllSubNodeWithMontageEnd
          (:then
            (Class|ActionNode|EndAllSubNodes WantCursor))
          (:else))
        (else
          (Class|ActionNode|MoveExecutortoNext WantCursor))))))

(event EventOnActionMessageDetail
  (params (WantCursor :type Action%20Cursor%20Finder%20Structure%20%28by%20ref%29) (Message :type Name%20%28by%20ref%29 :default "None") (Context :type Name%20%28by%20ref%29 :default "None"))
  (if (or (== Message (Class|ReservedActionMessage|GetActionMessageMontageNotifyBegin)) (== Message (Class|ReservedActionMessage|GetActionMessageMontageNotifyEnd)))
    (Class|ActionNode|MoveExecutortoLinkedNode WantCursor Context)))

(event EventOnCancel
  (params (WantCursor :type Action%20Cursor%20Finder%20Structure%20%28by%20ref%29))
  (CallFunction|StopCurrentMontage WantCursor))

(fn StopCurrentMontage
  (params (ActionCursorFinder :type Action%20Cursor%20Finder%20Structure%20%28by%20ref%29))
  (bind _resultunit (Class|UnitComponentBase|TryGetOwnerUnit (.CurrentComponent (Utilities|Struct|BreakActionCursorFinder ActionCursorFinder)))
    (:True
      (Class|UnitMainComponent|StopMainActionMontage _resultunit true))))