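; Behavior node for actions that fires a projectile from the executing component, with configurable speed, range, radius and durability.
; On execute, the cursor's executor resolves start position and direction through the ShotDirection claimer, the projectile spawns, and the executor moves to the next step.
; For targeting, it claims one arrow indicator per target component and draws each along the shot, sized by range and radius, with a percent from the cursor.
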(event EventClaimExecute
  (params (WantCursor :type Action%20Cursor%20Finder%20Structure%20%28by%20ref%29))
  (CallFunction|SpawnProjectile WantCursor))

(event EventUpdateIndicatorSingle
  (params (TargetInput :type Input%20Claim%20Structure%20%28by%20ref%29) (InputPackage :type Input%20Package%20Structure%20%28by%20ref%29) (TargetComponent :type Unit%20Action%20Component%20Object%20Reference) (TargetShower :type Action%20Indicator%20Shower%20Base%20Object%20Reference) (TargetUnit :type Unit%20Base%20Object%20Reference) (Index :type Integer))
  (bind _targetactioncursor (Utilities|Struct|BreakInputClaim TargetInput))
  (bind _shotdirection (Variables|Default|GetShotDirection))
  (Utilities|IsValid TargetUnit
    (:Is%20Valid
      (bind _asbp_action_indicator_shower_base (Utilities|Casting|CastToBP_ActionIndicatorShowerBase TargetShower))
      (Default|SetPercent _asbp_action_indicator_shower_base (Class|ActionNode|GetPercent _targetactioncursor))
      (Default|DrawfromDirection _asbp_action_indicator_shower_base (Class|DirectionClaimer|GetStartPosition _shotdirection _targetactioncursor TargetComponent) (Class|DirectionClaimer|GetDirection _shotdirection _targetactioncursor TargetComponent) (Variables|Default|GetRange) (Variables|Default|GetRadius)))))

(fn SpawnProjectile
  (params (Cursor :type Action%20Cursor%20Finder%20Structure))
  (bind _shotdirection (Variables|Default|GetShotDirection))
  (bind _output_get (LocalVariables|SetCurrentCursor Cursor))
  (Utilities|SpawnProjectile (Variables|Default|GetProjectile) (.CurrentComponent (Utilities|Struct|BreakActionCursorFinder _output_get)) (.CurrentExecutor (Utilities|Struct|BreakActionCursorFinder _output_get)) (Class|ActionExecutor|GetStartPosition (.CurrentExecutor (Utilities|Struct|BreakActionCursorFinder (LocalVariables|GetCurrentCursor))) _output_get _shotdirection) (Class|ActionExecutor|GetDirection (.CurrentExecutor (Utilities|Struct|BreakActionCursorFinder (LocalVariables|GetCurrentCursor))) _output_get _shotdirection) (Variables|Default|GetSpeed) (Variables|Default|GetRange) (Variables|Default|GetRadius) (Variables|Default|GetMax%20Durability))
  (Class|ActionNode|MoveExecutortoNext (LocalVariables|GetCurrentCursor)))

(fn GetIndicatorClaim
  (params (TargetInput :type Input%20Claim%20Structure%20%28by%20ref%29))
  (return (Utilities|Struct|MakeIndicatorClaim "Arrow" (Utilities|Array|Length (.targetcomponentarray TargetInput)))))