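; Repeat node for the action system that sweeps a direction vector around the yaw axis as the loop runs.
; LoopStart takes the direction from OriginDirection or the claim/owner actor's forward, applies StartShiftAngle and stores it on the cursor under ResultDirectionTag.
; Each LoopBody rotates the stored vector by ShiftAngle and writes it back, so rotation accumulates per iteration rather than deriving from the index.
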(fn LoopBody
  (params (BaseCursor :type Action%20Cursor%20Finder%20Structure%20%28by%20ref%29) (CurrentIndex :type Integer%20%28by%20ref%29) (MaxCount :type Integer%20%28by%20ref%29))
  (bind _returnvalue (Class|ActionExecutor|GetExecutorfromCursor BaseCursor))
  (Utilities|IsValid _returnvalue
    (:Is%20Valid
      (bind _resultdirection (CallFunction|CalculateDirection (.OutResult (Class|ActionExecutor|GetVector _returnvalue BaseCursor (Variables|Default|GetResultDirectionTag) (Class|KismetMathLibrary|VectorRight))) CurrentIndex MaxCount BaseCursor))
      (Class|ActionExecutor|SetVector _returnvalue BaseCursor (Variables|Default|GetResultDirectionTag) _resultdirection)
      (return true))))

(fn CalculateDirection
  (params (OriginDirection :type Vector) (Index :type Integer) (MaxCount :type Integer) (WantCursor :type Action%20Cursor%20Finder%20Structure%20%28by%20ref%29))
  (bind _shiftangle (Variables|Default|GetShiftAngle)
    (:then
      (if (== (Class|FloatClaimer|GetValue _shiftangle WantCursor 0.0) 0.0)
        _
        (else
          (return (Math|Vector|RotateVector OriginDirection (Math|Rotator|MakeRotator 0.0 0.0 (Class|FloatClaimer|GetValue _shiftangle WantCursor 0.0)))))))
    (:else
      _))
  (return OriginDirection))

(fn LoopStart
  (params (BaseCursor :type Action%20Cursor%20Finder%20Structure%20%28by%20ref%29) (MaxCount :type Integer%20%28by%20ref%29))
  (bind _output_get (LocalVariables|SetCursor BaseCursor))
  (LocalVariables|SetMax MaxCount)
  (bind _output_get_2 (LocalVariables|SetComponent (.CurrentComponent (Utilities|Struct|BreakActionCursorFinder _output_get))))
  (Utilities|IsValid _output_get_2
    (:Is%20Valid
      (Utilities|IsValid (.ClaimActor (Utilities|Struct|BreakActionCursorFinder _output_get))
        (:Is%20Valid
          (LocalVariables|SetActor (.ClaimActor (Utilities|Struct|BreakActionCursorFinder _output_get))))
        (:Is%20Not%20Valid
          (LocalVariables|SetActor (Components|GetOwner (LocalVariables|GetComponent)))))
      (LocalVariables|SetDirection (Transformation|GetActorForwardVector (LocalVariables|GetActor)))
      (bind _origindirection (Variables|Default|GetOriginDirection)
        (:then
          (LocalVariables|SetDirection (Class|DirectionClaimer|GetDirection _origindirection (LocalVariables|GetCursor) (Transformation|GetActorLocation (LocalVariables|GetActor)) (LocalVariables|GetDirection))))
        (:else
          _))
      (bind _startshiftangle (Variables|Default|GetStartShiftAngle)
        (:then
          (if (!= (Class|FloatClaimer|GetValue _startshiftangle (LocalVariables|GetCursor) 0.0) 0.0)
            (LocalVariables|SetDirection (Math|Vector|RotateVector (LocalVariables|GetDirection) (Math|Rotator|MakeRotator 0.0 0.0 (Class|FloatClaimer|GetValue _startshiftangle (LocalVariables|GetCursor) 0.0))))))
        (:else
          _))
      (Class|ActionExecutor|SetVectortoCursor (LocalVariables|GetCursor) (Variables|Default|GetResultDirectionTag) (LocalVariables|GetDirection))
      (return))
    (:Is%20Not%20Valid
      (return))))