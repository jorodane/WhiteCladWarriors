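; BP_RepeatNode is an action-graph node that runs a linked RepeatNode a number of times, spaced by a timed interval.
; On execute it evaluates the optional Interval and RepeatTime inputs, then starts the inherited timer.
; Each timer activation creates a sub-node cursor and moves execution into RepeatNode if LoopBody returns true; completion advances to the next node.
; LoopStart, LoopBody and LoopEnd are stub hooks around the loop.
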(event Custom|OnSubNodeCreated
  (params (BaseCursor :type Action%20Cursor%20Finder%20Structure%20%28by%20ref%29) (CurrentIndex :type Integer) (MaxCount :type Integer))
  (bind _canexecute (CallFunction|LoopBody BaseCursor CurrentIndex MaxCount))
  (if _canexecute
    (Class|ActionNode|MoveExecutortoWantNode BaseCursor (Variables|Default|GetRepeatNode) false)))

(event EventOnActivated
  (params (BaseCursor :type Action%20Cursor%20Finder%20Structure%20%28by%20ref%29) (CurrentIndex :type Integer) (MaxCount :type Integer))
  (bind _repeatnode (Variables|Default|GetRepeatNode)
    (:then
      (bind _resultcursor (Class|ActionNode|CreateSubNode BaseCursor _repeatnode))
      (CallFunction|OnSubNodeCreated _resultcursor CurrentIndex MaxCount))
    (:else)))

(event EventClaimExecute
  (params (WantCursor :type Action%20Cursor%20Finder%20Structure%20%28by%20ref%29))
  (bind _interval (Variables|Default|GetInterval)
    (:then
      (bind _repeattime (Variables|Default|GetRepeatTime)
        (:then
          (Class|ActionDelayNode|StartTimer WantCursor (Class|FloatClaimer|GetValue _interval WantCursor 0.0) (Math|Float|Round (Class|FloatClaimer|GetValue _repeattime WantCursor 1.0))))
        (:else
          (Class|ActionDelayNode|StartTimer WantCursor (Class|FloatClaimer|GetValue _interval WantCursor 0.0) 1))))
    (:else
      (bind _repeattime_2 (Variables|Default|GetRepeatTime)
        (:then
          (Class|ActionDelayNode|StartTimer WantCursor 0.0 (Math|Float|Round (Class|FloatClaimer|GetValue _repeattime_2 WantCursor 1.0))))
        (:else
          (Class|ActionDelayNode|StartTimer WantCursor 0.0 1))))))

(event EventOnStartTimer
  (params (BaseCursor :type Action%20Cursor%20Finder%20Structure%20%28by%20ref%29) (MaxCount :type Integer))
  (CallFunction|LoopStart BaseCursor MaxCount))

(event EventOnFinishTimer
  (params (BaseCursor :type Action%20Cursor%20Finder%20Structure%20%28by%20ref%29))
  (CallFunction|LoopEnd BaseCursor)
  (Class|ActionNode|MoveExecutortoNext BaseCursor))

(fn LoopBody
  (params (BaseCursor :type Action%20Cursor%20Finder%20Structure%20%28by%20ref%29) (CurrentIndex :type Integer%20%28by%20ref%29) (MaxCount :type Integer%20%28by%20ref%29))
  (return true))

(fn LoopStart
  (params (BaseCursor :type Action%20Cursor%20Finder%20Structure%20%28by%20ref%29) (MaxCount :type Integer%20%28by%20ref%29)))

(fn LoopEnd
  (params (BaseCursor :type Action%20Cursor%20Finder%20Structure%20%28by%20ref%29)))