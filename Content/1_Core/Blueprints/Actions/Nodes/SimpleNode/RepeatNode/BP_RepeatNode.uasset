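; BP_RepeatNode is an action node that runs a sub-node several times across an evenly spaced yaw fan.
; On execution, it reads the executor's tagged direction and builds rotated directions centred on it, using the repeat count and angle step.
; It sets each direction on the executor before creating a sub-node from RepeatNode, then restores the original direction and advances the executor to the next node.
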(event EventClaimExecute
  (params (WantCursor :type Action%20Cursor%20Finder%20Structure%20%28by%20ref%29))
  (CallFunction|Repeat WantCursor)
  (Class|ActionNode|MoveExecutortoNext WantCursor))

(fn Repeat
  (params (WantCursor :type Action%20Cursor%20Finder%20Structure%20%28by%20ref%29))
  (bind _repeattime (Variables|Default|GetRepeatTime))
  (bind _returnvalue (Class|FloatGetter|GetValue _repeattime))
  (bind _returnvalue_2 (Class|KismetMathLibrary|Round64 _returnvalue))
  (bind _returnvalue_3 (Math|Conversions|ToInteger(Byte) _returnvalue_2))
  (bind _returnvalue_4 (+ _returnvalue_3 -1))
  (bind _output_get (LocalVariables|SetCursor WantCursor))
  (bind _output_get_2 (LocalVariables|SetExecutor (Class|ActionExecutor|GetExecutorfromCursor _output_get)))
  (Utilities|IsValid _output_get_2
    (:Is%20Valid
      (Variables|Default|GetRepeatTime
        (:then
          (Variables|Default|GetRepeatAngle
            (:then
              (Utilities|FlowControl|Sequence
                (:then_0
                  (LocalVariables|SetOriginDirection (Class|ActionExecutor|GetSavedDirection (LocalVariables|GetExecutor) (LocalVariables|GetCursor) (Variables|Default|GetOriginAngleTag)))
                  (bind _output_get_3 (LocalVariables|SetShiftAngle (Class|FloatGetter|GetValue (Variables|Default|GetRepeatAngle))))
                  (LocalVariables|SetHalfAngle (* (* _output_get_3 _returnvalue_4) -0.5))
                  (for _index (range 0 _returnvalue_4)
                    (Utilities|Array|Add (LocalVariables|GetTargetDirections) (Math|Vector|RotateVector (LocalVariables|GetOriginDirection) (Math|Rotator|MakeRotator 0.0 0.0 (+ (* _index (LocalVariables|GetShiftAngle)) (LocalVariables|GetHalfAngle)))))))
                (:then_1
                  (for _array_element (LocalVariables|GetTargetDirections)
                    (Class|ActionExecutor|SetDirection (LocalVariables|GetExecutor) (Variables|Default|GetOriginAngleTag) (LocalVariables|GetCursor) _array_element)
                    (Class|ActionNode|CreateSubNode (LocalVariables|GetCursor) (Variables|Default|GetRepeatNode)))
                  (Class|ActionExecutor|SetDirection (LocalVariables|GetExecutor) (Variables|Default|GetOriginAngleTag) (LocalVariables|GetCursor) (LocalVariables|GetOriginDirection)))))
            (:else)))
        (:else)))))