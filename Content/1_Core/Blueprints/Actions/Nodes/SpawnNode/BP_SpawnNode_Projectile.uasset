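; Action node that fires a projectile from the owning unit along a ShotDirection, using configured speed, range, radius and durability, and cancels its executor when it cannot.
; The spawned projectile is registered as an instance, and optional sub-nodes run on spawn, hit and destruction, with the projectile or hit result written into their cursors.
; It also claims an arrow targeting indicator sized by range and radius, aimed toward the mouse or unit forward in icon preview.
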(event EventClaimExecute
  (params (WantCursor :type Action%20Cursor%20Finder%20Structure%20%28by%20ref%29))
  (Variables|Default|GetShotDirection
    (:then
      (CallFunction|SpawnProjectile WantCursor))
    (:else
      (Class|ActionNode|MoveExecutortoCancel WantCursor))))

(event EventOnHitReceived
  (params (From :type Actor%20Object%20Reference) (BaseCursor :type Action%20Cursor%20Finder%20Structure%20%28by%20ref%29) (Hit :type Hit%20Result%20Structure%20%28by%20ref%29))
  (bind _onhit (Variables|Default|GetOnHit)
    (:then
      (bind _resultcursor (Class|ActionNode|CreateSubNode BaseCursor _onhit))
      (Class|ActionExecutor|SetHitResulttoCursor _resultcursor (Variables|Default|GetHitResultName) Hit)
      (Class|ActionExecutor|ExecuteCursor _resultcursor))
    (:else)))

(event EventUpdateIndicatorSingle
  (params (TargetNode :type Action%20Behavior%20Node%20Object%20Reference) (TargetInput :type Input%20Claim%20Structure%20%28by%20ref%29) (InputPackage :type Input%20Package%20Structure%20%28by%20ref%29) (TargetComponent :type Unit%20Action%20Component%20Object%20Reference) (TargetShower :type Action%20Indicator%20Shower%20Base%20Object%20Reference) (TargetUnit :type Unit%20Main%20Component%20Object%20Reference) (Index :type Integer) (bIsIconPreview :type Boolean))
  (bind _targetactioncursor (Utilities|Struct|BreakInputClaim TargetInput))
  (bind _returnvalue (Components|GetOwner TargetUnit))
  (bind _shotdirection (Variables|Default|GetShotDirection))
  (bind _returnvalue_2 (Transformation|GetActorLocation _returnvalue))
  (Variables|Default|GetShotDirection
    (:then
      (Utilities|IsValid TargetUnit
        (:Is%20Valid
          (Default|SetPercent TargetShower (Class|ActionNode|GetPercent _targetactioncursor))
          (Default|DrawfromDirection TargetShower (Class|PositionClaimer|GetPosition _shotdirection _targetactioncursor _returnvalue_2) (Class|DirectionClaimer|GetDirection _shotdirection _targetactioncursor _returnvalue_2 (Math|Vector|SelectVector (Transformation|GetActorForwardVector _returnvalue) (Class|KismetMathLibrary|VectorNormal2D (- (.MouseTerrainPosition (Utilities|Struct|BreakInputPackage InputPackage)) _returnvalue_2) 0.0001) bIsIconPreview)) (Variables|Default|GetRange) (Variables|Default|GetRadius)))))
    (:else)))

(event EventInstanceDestroyed
  (params (Instance :type Actor%20Object%20Reference) (BaseCursor :type Action%20Cursor%20Finder%20Structure%20%28by%20ref%29))
  (bind _ondestroyprojectile (Variables|Default|GetOnDestroyProjectile)
    (:then
      (bind _resultcursor (Class|ActionNode|CreateSubNode BaseCursor _ondestroyprojectile))
      (Class|ActionExecutor|ExecuteCursor _resultcursor))
    (:else)))

(fn SpawnProjectile
  (params (Cursor :type Action%20Cursor%20Finder%20Structure))
  (bind _shotdirection (Variables|Default|GetShotDirection))
  (bind _output_get (LocalVariables|SetCurrentCursor Cursor))
  (bind _output_get_2 (LocalVariables|SetCurrentExecutor (Class|ActionExecutor|GetExecutorfromID (.CurrentExecutorID (Utilities|Struct|BreakActionCursorFinder _output_get)))))
  (Utilities|IsValid _output_get_2
    (:Is%20Valid
      (bind _output_get_3 (LocalVariables|SetCurrentComponent (.CurrentComponent (Utilities|Struct|BreakActionCursorFinder _output_get))))
      (Utilities|IsValid _output_get_3
        (:Is%20Valid
          (bind _resultunit (Class|UnitActionComponent|TryGetOwnerUnit _output_get_3)
            (:True
              (LocalVariables|SetCurrentUnit _resultunit)
              (bind _returnvalue (Utilities|SpawnProjectile (LocalVariables|GetCurrentComponent) (Variables|Default|GetProjectile) (Variables|Default|GetMain%20Particle) (Class|PositionClaimer|GetPosition _shotdirection (LocalVariables|GetCurrentCursor) (Transformation|GetActorLocation (Components|GetOwner (LocalVariables|GetCurrentUnit)))) (Class|DirectionClaimer|GetDirection _shotdirection (LocalVariables|GetCurrentCursor) (Transformation|GetActorLocation (Components|GetOwner (LocalVariables|GetCurrentUnit))) (Transformation|GetActorForwardVector (Components|GetOwner (LocalVariables|GetCurrentUnit)))) (Variables|Default|GetSpeed) (Variables|Default|GetRange) (Variables|Default|GetRadius) (Variables|Default|GetMax%20Durability)))
              (Utilities|IsValid _returnvalue
                (:Is%20Valid
                  (LocalVariables|SetCurrentProjectile _returnvalue)
                  (bind _returnvalue_2 (CallFunction|InstanceCreated (LocalVariables|GetCurrentProjectile) (LocalVariables|GetCurrentCursor)))
                  (Class|ActionSpawnNode|InstanceRegistration (LocalVariables|GetCurrentProjectile) _returnvalue_2))
                (:Is%20Not%20Valid
                  (Class|ActionNode|MoveExecutortoCancel (LocalVariables|GetCurrentCursor) :!label _label))))
            (:False
              (goto _label))))
        (:Is%20Not%20Valid
          (goto _label))))
    (:Is%20Not%20Valid
      (goto _label))))

(fn GetIndicatorClaim
  (params (TargetInput :type Input%20Claim%20Structure%20%28by%20ref%29))
  (return (Utilities|Map|MakeMap self (Utilities|Struct|MakeIndicatorClaim "Arrow" (Utilities|Array|Length (.targetcomponentarray TargetInput))))))

(fn InstanceCreated
  (params (Instance :type Actor%20Object%20Reference) (BaseCursor :type Action%20Cursor%20Finder%20Structure%20%28by%20ref%29))
  (bind _onspawnprojectile (Variables|Default|GetOnSpawnProjectile)
    (:then
      (bind _resultcursor (Class|ActionNode|CreateSubNode BaseCursor _onspawnprojectile))
      (Class|ActionExecutor|SetActortoCursor _resultcursor (Variables|Default|GetProjectileName) Instance)
      (return _resultcursor))
    (:else
      (return BaseCursor))))