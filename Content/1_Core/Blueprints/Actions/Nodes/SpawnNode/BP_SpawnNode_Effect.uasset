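; Action-graph node that spawns a visual effect through the cursor's operator, then advances execution to the next node.
; On execute it casts the cursor's current operator to BP_Operator, stopping the spawn if that fails.
; Optional SpawnPosition and SpawnDirection providers resolve the location and facing from the cursor and component.
; The operator spawns the template effect with that transform, its controller as instigator and an owner-only visibility flag.
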(event EventClaimExecute
  (params (WantCursor :type Action%20Cursor%20Finder%20Structure%20%28by%20ref%29))
  (CallFunction|SpawnEffect WantCursor)
  (Class|ActionNode|MoveExecutortoNext WantCursor))

(fn SpawnEffect
  (params (ActionCursorFinder :type Action%20Cursor%20Finder%20Structure%20%28by%20ref%29))
  (bind (_currentaction _currentoperator _currentexecutorid _currentcomponent) (Utilities|Struct|BreakActionCursorFinder ActionCursorFinder))
  (LocalVariables|SetCurrentCursor ActionCursorFinder)
  (LocalVariables|SetCurrentComponent _currentcomponent)
  (bind _asbp_operator (Utilities|Casting|CastToBP_Operator _currentoperator))
  (Utilities|FlowControl|Sequence
    (:then_0
      (bind _spawnposition (Variables|Default|GetSpawnPosition)
        (:then
          (LocalVariables|SetCurrentPosition (Class|PositionClaimer|GetPosition _spawnposition (LocalVariables|GetCurrentCursor) (LocalVariables|GetCurrentComponent) (LocalVariables|GetCurrentPosition))))
        (:else)))
    (:then_1
      (bind _spawndirection (Variables|Default|GetSpawnDirection)
        (:then
          (LocalVariables|SetCurrentRotation (Class|DirectionClaimer|GetDirection _spawndirection (LocalVariables|GetCurrentCursor) (LocalVariables|GetCurrentComponent) (LocalVariables|GetCurrentPosition) (LocalVariables|GetCurrentRotation))))
        (:else)))
    (:then_2
      (Default|SpawnEffectonLocation _asbp_operator (Variables|Default|GetShow%20Only%20Owner) (Variables|Default|GetTemplateEffect) (Math|Transform|MakeTransform (LocalVariables|GetCurrentPosition) (Math|Conversions|RotationFromXVector (LocalVariables|GetCurrentRotation)) "1.000000,1.000000,1.000000") (Pawn|GetController _asbp_operator)))))