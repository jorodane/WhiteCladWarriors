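; Action preset for a basic attack, built at BeginPlay as a tree of behavior nodes.
; A single-target selector with an attack cursor picks the tagged target and leads to a LookAt node, then a main-action montage that stops movement on start.
; The montage's "Shot" link triggers a damage sub-node on that target.
; The LookAt chain also serves as the sub-node root, skipping selection.
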(event EventBeginPlay
  (|CallParentFunction)
  (Variables|Default|SetAttackRadius (Class|ValueGetterLibrary|MakeSimpleFloat 0 5e+02))
  (Variables|Default|SetAttackDamage (Class|ValueGetterLibrary|MakeSimpleFloat 0 1e+01))
  (Variables|Default|SetTargetActor (Class|ValueClaimerLibrary|MakeActorClaimerSavedActor 0 (Variables|Default|GetTargetTag)))
  (Variables|Default|SetTargetDirection (Class|ValueClaimerLibrary|MakeDirectionClaimertoPosition 0 (Class|ValueClaimerLibrary|ClaimSelfPosition) (Class|ValueClaimerLibrary|MakePositionClaimerActorPosition 0 (Variables|Default|GetTargetActor) "Self")))
  (bind _returnvalue (Game|ConstructObjectfromClass "/Game/1_Core/Blueprints/Actions/Nodes/BehaviorNode/BP_BehaviorNode_Damage.BP_BehaviorNode_Damage_C" (Variables|Default|GetTargetActor) (Variables|Default|GetAttackDamage) (Variables|Default|GetTargetDirection) 0 (Utilities|Struct|MakeActionExecuteSettingContainer false true false false) 0 0 0))
  (bind _returnvalue_2 (Game|ConstructObjectfromClass "/Game/1_Core/Blueprints/Actions/Nodes/BehaviorNode/BP_BehaviorNode_MontagePlay.BP_BehaviorNode_MontagePlay_C" (Variables|Default|GetAttackMontage) (Variables|Default|GetTargetActor) 0 false (Utilities|Struct|MakeActionExecuteSettingContainer true true true false) 0 0 0 (Utilities|Map|MakeMap "Shot" (Utilities|Struct|MakeLinkedNodeInfo _returnvalue true))))
  (bind _returnvalue_3 (Game|ConstructObjectfromClass :Class "/Game/1_Core/Blueprints/Actions/Nodes/BehaviorNode/BP_BehaviorNode_LookAt.BP_BehaviorNode_LookAt_C" :LookDirection (Variables|Default|GetTargetDirection) :NextNode _returnvalue_2 :CanceledNode 0 :BlockedNode 0))
  (Variables|Default|SetRootAsSubNode _returnvalue_3)
  (bind _returnvalue_4 (Game|ConstructObjectfromClass :Class "/Game/1_Core/Blueprints/Actions/Nodes/SelectorNode/BP_SelectorNode_Single.BP_SelectorNode_Single_C" :Description "공격할 대상을 선택하세요" :CursorDescription "공격" :CursorType "Attack" :PositionEffect "/Game/1_Core/VisualEffects/Single/NS_MoveEffect.NS_MoveEffect" :InputTypes (Utilities|Array|MakeArray (Utilities|Struct|MakeSelectorInput "SingleTarget" (Variables|Default|GetTargetTag) _returnvalue_3)) :NextNode 0 :CanceledNode 0 :BlockedNode 0))
  (Variables|Default|SetRootNode _returnvalue_4))

(fn ConstructionScript
  (|CallParentFunction))