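; BP_Action_Move is a preset action that moves to either a targeted actor or a position.
; On BeginPlay it builds its node tree in code, with a single crosshair selector as the root node.
; The selector pairs single-target input with a move-to-actor behavior and position input with a move-to-location behavior, linked through claimers on a shared destination tag.
; Its simple action order is a constant, independent of input and target.
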(event EventBeginPlay
  (bind _destination_tag (Variables|Default|GetDestination%20Tag))
  (|CallParentFunction)
  (bind _returnvalue (Game|ConstructObjectfromClass "/Game/1_Core/Blueprints/Actions/Nodes/BehaviorNode/BP_BehaviorNode_MoveToActor.BP_BehaviorNode_MoveToActor_C" (Class|ValueClaimerLibrary|MakeActorClaimer 0 (Variables|Default|GetDestination%20Tag)) (Class|ValueGetterLibrary|MakeSimpleFloat 0 5e+01) 0 0 0))
  (bind _returnvalue_2 (Game|ConstructObjectfromClass "/Game/1_Core/Blueprints/Actions/Nodes/BehaviorNode/BP_BehaviorNode_MoveToLocation.BP_BehaviorNode_MoveToLocation_C" (Class|ValueClaimerLibrary|MakePositionClaimer 0 (Variables|Default|GetDestination%20Tag) "SavedPosition" "World") 0 0 0 0))
  (bind _returnvalue_3 (Game|ConstructObjectfromClass "/Game/1_Core/Blueprints/Actions/Nodes/SelectorNode/BP_SelectorNode_Single.BP_SelectorNode_Single_C" (Variables|Default|GetDescription) "Crosshairs" (Utilities|Array|MakeArray (Utilities|Struct|MakeSelectorInput "SingleTarget" _destination_tag _returnvalue) (Utilities|Struct|MakeSelectorInput "Position" _destination_tag _returnvalue_2)) 0 0 0 0))
  (Variables|Default|SetRootNode _returnvalue_3))

(fn ConstructionScript
  (|CallParentFunction))

(fn GetSimpleActionOrder
  (params (CurrentInput :type Input%20Package%20Structure%20%28by%20ref%29) (CurrentTarget :type Unit%20Action%20Component%20Object%20Reference))
  (return 100))