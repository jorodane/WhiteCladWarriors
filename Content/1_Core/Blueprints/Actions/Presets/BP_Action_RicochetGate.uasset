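; Ricochet action preset: the player aims a shot that, on hit, splits into two stronger projectiles.
; BeginPlay builds the node tree leaf-first, ending in a single direction selector as RootNode, with the first projectile as its indicator.
; That projectile's hit-damage node chains into a parallel node firing both secondary shots, angled either side of the hit normal.
; The two branches differ in additive space (World versus Self) as well as angle sign.
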(event EventBeginPlay
  (bind _returnvalue (Class|ValueGetterLibrary|MakeSimpleFloat 0 -6e+01))
  (bind _returnvalue_2 (Class|ValueClaimerLibrary|MakeDirectionClaimerSavedDirection 0 0 "ThrowDirection"))
  (bind _returnvalue_3 (Class|ValueGetterLibrary|MakeSimpleFloat 0 6e+01))
  (bind _hittag (Variables|Default|GetHitTag))
  (bind _hittag_2 (Variables|Default|GetHitTag))
  (bind _returnvalue_4 (Class|ValueClaimerLibrary|MakeDirectionClaimerHitNormal 0 _hittag _returnvalue_3 "Self"))
  (bind _returnvalue_5 (Class|ValueClaimerLibrary|MakeDirectionClaimerHitNormal 0 _hittag_2 _returnvalue "World"))
  (Utilities|FlowControl|Sequence
    (:then_0
      (bind _returnvalue_6 (Utilities|MakeProjectileHitDamage 0 "Projectile" (Variables|Default|GetHitTag) "/Game/Projectiles_Spells_VFX/Effects/Projectile_01/Lvl_1/NS_Impact_01_Lvl_1.NS_Impact_01_Lvl_1" (Class|ValueClaimerLibrary|MakeFloatClaimerSimpleFloat 0 (Class|ValueGetterLibrary|MakeSimpleFloat 0 3e+01)) _returnvalue_5 true))
      (bind _returnvalue_7 (Utilities|MakeSimpleProjectile 0 _returnvalue_6 3e+03 1.5e+03 5e+01 -1.0 _returnvalue_5 _returnvalue_5 "/Game/Projectiles_Spells_VFX/Effects/Projectile_01/Lvl_1/NS_Cast_01_Lvl_1.NS_Cast_01_Lvl_1" "/Game/Projectiles_Spells_VFX/Effects/Projectile_01/Lvl_1/NS_Projectile_01_Lvl_1.NS_Projectile_01_Lvl_1" (Variables|Default|GetHitTag) "Projectile")))
    (:then_1
      (bind _returnvalue_8 (Utilities|MakeProjectileHitDamage 0 "Projectile" (Variables|Default|GetHitTag) "/Game/Projectiles_Spells_VFX/Effects/Projectile_01/Lvl_1/NS_Impact_01_Lvl_1.NS_Impact_01_Lvl_1" (Class|ValueClaimerLibrary|MakeFloatClaimerSimpleFloat 0 (Class|ValueGetterLibrary|MakeSimpleFloat 0 3e+01)) _returnvalue_4 true))
      (bind _returnvalue_9 (Utilities|MakeSimpleProjectile 0 _returnvalue_8 3e+03 1.5e+03 5e+01 -1.0 _returnvalue_4 _returnvalue_4 "/Game/Projectiles_Spells_VFX/Effects/Projectile_01/Lvl_1/NS_Cast_01_Lvl_1.NS_Cast_01_Lvl_1" "/Game/Projectiles_Spells_VFX/Effects/Projectile_01/Lvl_1/NS_Projectile_01_Lvl_1.NS_Projectile_01_Lvl_1" (Variables|Default|GetHitTag) "Projectile")))
    (:then_2
      (bind _returnvalue_10 (Game|ConstructObjectfromClass "/Game/1_Core/Blueprints/Actions/Nodes/SimpleNode/Branchs/BP_SimpleNode_ParallelExecution.BP_SimpleNode_ParallelExecution_C" (Utilities|Array|MakeArray _returnvalue_7 _returnvalue_9) 0 0 0))
      (bind _returnvalue_11 (Utilities|MakeProjectileHitDamage _returnvalue_10 "Projectile" (Variables|Default|GetHitTag) "/Game/Projectiles_Spells_VFX/Effects/Projectile_01/Lvl_1/NS_Impact_01_Lvl_1.NS_Impact_01_Lvl_1" (Class|ValueClaimerLibrary|MakeFloatClaimerSimpleFloat 0 (Class|ValueGetterLibrary|MakeSimpleFloat 0 15.0)) _returnvalue_2 true))
      (bind _returnvalue_12 (Utilities|MakeSimpleProjectile 0 _returnvalue_11 3e+03 1.5e+03 5e+01 -1.0 _returnvalue_2 (Class|ValueClaimerLibrary|ClaimSelfPosition) "/Game/Projectiles_Spells_VFX/Effects/Projectile_01/Lvl_1/NS_Cast_01_Lvl_1.NS_Cast_01_Lvl_1" "/Game/Projectiles_Spells_VFX/Effects/Projectile_01/Lvl_1/NS_Projectile_01_Lvl_1.NS_Projectile_01_Lvl_1" (Variables|Default|GetHitTag) "Projectile"))
      (bind _returnvalue_13 (Game|ConstructObjectfromClass "/Game/1_Core/Blueprints/Actions/Nodes/SelectorNode/BP_SelectorNode_Single.BP_SelectorNode_Single_C" 0 "발사할 방향 선택" "" "Target" "/Game/1_Core/VisualEffects/Single/NS_MoveEffect.NS_MoveEffect" (Utilities|Struct|MakeMontageEventInfo "/Game/1_Core/Animations/AM_PrepareShooting.AM_PrepareShooting") (Utilities|Array|MakeArray (Utilities|Struct|MakeSelectorInput "Direction" "ThrowDirection" _returnvalue_12)) (Utilities|Array|MakeArray _returnvalue_12) false 0 0 0))
      (Variables|Default|SetRootNode _returnvalue_13))))

(fn ConstructionScript
  (|CallParentFunction))