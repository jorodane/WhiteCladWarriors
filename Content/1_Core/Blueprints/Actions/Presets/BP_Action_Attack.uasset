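; Attack command preset that builds its behavior node tree in BeginPlay under a single-selection selector with an attack cursor.
; A picked target leads to moving within attack radius, then stopping to start the unit's "Attack"-tagged action, while a picked position is a plain move.
; GetSimpleActionOrder gives priority only when the hovered unit is an enemy.
; A disconnected look-at and fireball projectile chain remains unused.
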(event EventBeginPlay
  (bind _targettag (Variables|Default|GetTargetTag))
  (|CallParentFunction)
  (Variables|Default|SetAttackRadius (Class|ValueGetterLibrary|MakeSimpleFloat 0 5e+02))
  (Variables|Default|SetTargetActor (Class|ValueClaimerLibrary|MakeActorClaimer 0 (Variables|Default|GetTargetTag)))
  (bind _returnvalue (Game|ConstructObjectfromClass "/Game/1_Core/Blueprints/Actions/Nodes/BehaviorNode/BP_BehaviorNode_StartAction.BP_BehaviorNode_StartAction_C" (Class|ValueClaimerLibrary|MakeActionClaimerUnitTagged 0 "Attack") (Variables|Default|GetTargetActor) (Class|ValueClaimerLibrary|MakePositionClaimerActorPosition 0 (Variables|Default|GetTargetActor) "Self") 0 0 0 0 true false true))
  (bind _returnvalue_2 (Game|ConstructObjectfromClass "/Game/1_Core/Blueprints/Actions/Nodes/BehaviorNode/BP_BehaviorNode_MoveToActor.BP_BehaviorNode_MoveToActor_C" (Variables|Default|GetTargetActor) (Variables|Default|GetAttackRadius) _returnvalue 0 0))
  (bind _returnvalue_3 (Game|ConstructObjectfromClass "/Game/1_Core/Blueprints/Actions/Nodes/BehaviorNode/BP_BehaviorNode_MoveToLocation.BP_BehaviorNode_MoveToLocation_C" (Class|ValueClaimerLibrary|MakePositionClaimerSavedPosition 0 (Variables|Default|GetTargetTag) "Self") 0 0 0 0))
  (bind _returnvalue_4 (Game|ConstructObjectfromClass :Class "/Game/1_Core/Blueprints/Actions/Nodes/SelectorNode/BP_SelectorNode_Single.BP_SelectorNode_Single_C" :Description "공격할 대상을 선택하세요" :CursorType "Attack" :PositionEffect "/Game/1_Core/VisualEffects/Single/NS_MoveEffect.NS_MoveEffect" :InputTypes (Utilities|Array|MakeArray (Utilities|Struct|MakeSelectorInput "SingleTarget" _targettag _returnvalue_2) (Utilities|Struct|MakeSelectorInput "Position" _targettag _returnvalue_3)) :IndicatorNodes (Utilities|Array|MakeArray _returnvalue_2) :NextNode 0 :CanceledNode 0 :BlockedNode 0))
  (Variables|Default|SetRootNode _returnvalue_4))

(fn ConstructionScript
  (|CallParentFunction))

(fn GetSimpleActionOrder
  (params (CurrentInput :type Input%20Package%20Structure%20%28by%20ref%29) (CurrentTarget :type Unit%20Action%20Component%20Object%20Reference))
  (bind _returnvalue (Actor|GetComponentbyClass (.mousehitactor CurrentInput) "/Script/WhiteCladWarriors.UnitMainComponent"))
  (Utilities|IsValid (.mousehitactor CurrentInput)
    (:Is%20Valid
      (Utilities|IsValid _returnvalue
        (:Is%20Valid
          (return (Utilities|Select :Index (Class|UnitMainComponent|GetAllyType _returnvalue (Class|Operator|GetLocalOperator)) :Normal 0 :Own 0 :Enemy 200 :Ally 0)))
        (:Is%20Not%20Valid
          _)))
    (:Is%20Not%20Valid
      _))
  (return 0))