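; Dash action preset that builds its node graph on BeginPlay and stores the selector as the root node.
; A single selector prompts for a dash direction, saved under the "DashDirection" tag and claimed from the actor's own position.
; The selection chains into look-at, a fixed-range character launch as the main action, then a cancelable quick-shift montage.
; The launch node also serves as the selector's indicator.
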(event EventBeginPlay
  (|CallParentFunction)
  (Variables|Default|SetThrowDirection (Class|ValueClaimerLibrary|MakeDirectionClaimerSavedDirection 0 (Class|ValueClaimerLibrary|ClaimSelfPosition) "DashDirection"))
  (bind _returnvalue (Game|ConstructObjectfromClass "/Game/1_Core/Blueprints/Actions/Nodes/BehaviorNode/BP_BehaviorNode_MontagePlay.BP_BehaviorNode_MontagePlay_C" (Utilities|Struct|MakeMontageEventInfo "/Game/1_Core/Animations/AM_QuickShift.AM_QuickShift" 1.0 0.3 0.0) 0 0 0 0 true true true))
  (bind _returnvalue_2 (Game|ConstructObjectfromClass "/Game/1_Core/Blueprints/Actions/Nodes/BehaviorNode/BP_BehaviorNode_LaunchCharacter.BP_BehaviorNode_LaunchCharacter_C" 4e+03 4e+02 (Variables|Default|GetThrowDirection) _returnvalue 0 0 0 true true true))
  (bind _returnvalue_3 (Game|ConstructObjectfromClass "/Game/1_Core/Blueprints/Actions/Nodes/BehaviorNode/BP_BehaviorNode_LookAt.BP_BehaviorNode_LookAt_C" (Variables|Default|GetThrowDirection) _returnvalue_2 0 0))
  (bind _returnvalue_4 (Game|ConstructObjectfromClass :Class "/Game/1_Core/Blueprints/Actions/Nodes/SelectorNode/BP_SelectorNode_Single.BP_SelectorNode_Single_C" :Description "대시할 방향을 정해주세요" :CursorType "Target" :PositionEffect "/Game/1_Core/VisualEffects/Single/NS_MoveEffect.NS_MoveEffect" :InputTypes (Utilities|Array|MakeArray (Utilities|Struct|MakeSelectorInput "Direction" "DashDirection" _returnvalue_3)) :IndicatorNodes (Utilities|Array|MakeArray _returnvalue_2) :NextNode 0 :CanceledNode 0 :BlockedNode 0))
  (Variables|Default|SetRootNode _returnvalue_4))

(fn ConstructionScript
  (|CallParentFunction))