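; Area attack action preset that builds its node tree on BeginPlay and sprays damaging projectiles around the user, stopping movement on start.
; Nested ShiftAngle repeat nodes form a rotating four-way pattern: the outer steps the angle at short intervals, the inner fans shots at right angles via the saved "ShiftedDirection".
; Each slow outward projectile chains through NextNode into a fast one thrown from the trigger actor's position toward the user.
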(event EventBeginPlay
  (bind _returnvalue (Class|ValueClaimerLibrary|ClaimSelfPosition))
  (bind _returnvalue_2 (Class|ValueClaimerLibrary|ClaimTriggerActor))
  (bind _returnvalue_3 (Class|ValueClaimerLibrary|MakePositionClaimerActorPosition 0 _returnvalue_2 "Self"))
  (bind _returnvalue_4 (Class|ValueClaimerLibrary|MakeDirectionClaimertoPosition 0 _returnvalue_3 _returnvalue))
  (|CallParentFunction)
  (Variables|Default|SetThrowDirection 0)
  (Variables|Default|SetSpreadDirection (Class|ValueClaimerLibrary|MakeDirectionClaimerSavedDirection 0 0 "ShiftedDirection"))
  (Variables|Default|SetDamageValue (Class|ValueClaimerLibrary|MakeFloatClaimerSimpleFloat 0 (Class|ValueGetterLibrary|MakeSimpleFloat 0 15.0)))
  (bind _returnvalue_5 (Utilities|MakeProjectileHitDamage 0 "Projectile" (Variables|Default|GetHit%20Tag) "/Game/Projectiles_Spells_VFX/Effects/Projectile_18/Lvl_1/NS_Impact_18_Lvl_1.NS_Impact_18_Lvl_1" (Variables|Default|GetDamageValue) _returnvalue_4 true))
  (bind _returnvalue_6 (Utilities|MakeSimpleProjectile 0 _returnvalue_5 5e+03 1.5e+03 7e+01 -1.0 _returnvalue_4 _returnvalue_3 0 "/Game/Projectiles_Spells_VFX/Effects/Projectile_18/Lvl_1/NS_Projectile_18_Lvl_1.NS_Projectile_18_Lvl_1" (Variables|Default|GetHit%20Tag) "Projectile"))
  (bind _output_get (Variables|Default|SetProjectile _returnvalue_6))
  (bind _returnvalue_7 (Utilities|MakeProjectileHitDamage 0 "Projectile" (Variables|Default|GetHit%20Tag) "/Game/Projectiles_Spells_VFX/Effects/Projectile_18/Lvl_1/NS_Impact_18_Lvl_1.NS_Impact_18_Lvl_1" (Variables|Default|GetDamageValue) (Variables|Default|GetSpreadDirection) true))
  (bind _returnvalue_8 (Utilities|MakeSimpleProjectile _output_get _returnvalue_7 5e+02 1.5e+03 7e+01 -1.0 (Variables|Default|GetSpreadDirection) (Class|ValueClaimerLibrary|ClaimSelfPosition) 0 "/Game/Projectiles_Spells_VFX/Effects/Projectile_18/Lvl_1/NS_Projectile_18_Lvl_1.NS_Projectile_18_Lvl_1" (Variables|Default|GetHit%20Tag) "Projectile"))
  (Variables|Default|SetStartDirection (Class|ValueClaimerLibrary|MakeDirectionClaimerSimpleDirection 0 (Class|ValueClaimerLibrary|ClaimSelfPosition) (Class|ValueGetterLibrary|GetSimpleForwardVector) "Self"))
  (Variables|Default|SetShiftAngle (Class|ValueClaimerLibrary|MakeFloatClaimerSimpleFloat 0 (Class|ValueGetterLibrary|MakeSimpleFloat 0 9e+01)))
  (Variables|Default|SetRepeatTime (Class|ValueClaimerLibrary|MakeFloatClaimerSimpleFloat 0 (Class|ValueGetterLibrary|MakeSimpleFloat 0 4.0)))
  (bind _returnvalue_9 (Game|ConstructObjectfromClass :Class "/Game/1_Core/Blueprints/Actions/Nodes/DelayNode/BP_RepeatNode_ShiftAngle.BP_RepeatNode_ShiftAngle_C" :OriginDirection (Class|ValueClaimerLibrary|MakeDirectionClaimerSavedDirection 0 (Class|ValueClaimerLibrary|ClaimSelfPosition) "ShiftedDirection") :StartShiftAngle 0 :ShiftAngle (Variables|Default|GetShiftAngle) :ResultDirectionTag "ShiftedDirection" :RepeatTime (Variables|Default|GetRepeatTime) :RepeatNode _returnvalue_8 :Interval 0 :NextNode 0 :CanceledNode 0 :BlockedNode 0))
  (bind _returnvalue_10 (Game|ConstructObjectfromClass "/Game/1_Core/Blueprints/Actions/Nodes/DelayNode/BP_RepeatNode_ShiftAngle.BP_RepeatNode_ShiftAngle_C" (Variables|Default|GetStartDirection) 0 (Class|ValueClaimerLibrary|MakeFloatClaimerSimpleFloat 0 (Class|ValueGetterLibrary|MakeSimpleFloat 0 17.125)) "ShiftedDirection" (Class|ValueClaimerLibrary|MakeFloatClaimerSimpleFloat 0 (Class|ValueGetterLibrary|MakeSimpleFloat 0 9e+01)) _returnvalue_9 (Class|ValueClaimerLibrary|MakeFloatClaimerSimpleFloat 0 (Class|ValueGetterLibrary|MakeSimpleFloat 0 0.1)) (Utilities|Struct|MakeActionExecuteSettingContainer true true true false) 0 0 0))
  (Variables|Default|SetRootNode _returnvalue_10))

(fn ConstructionScript
  (|CallParentFunction))