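; Player-issued attack command action that targets either a unit or a location.
; BeginPlay builds a single-selector root whose actor input feeds an AttackTarget behavior node and whose position input feeds AttackLocation with a chase range, both reading saved values by tag.
; Simple-order scoring favors this action only when the unit under the cursor is an enemy of the local operator.
; Inspector targets include itself plus selected units' "Attack"-tagged actions.
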(event EventBeginPlay
  (bind _targettag (Variables|Default|GetTargetTag))
  (|CallParentFunction)
  (Variables|Default|SetTargetDestination (Class|ValueClaimerLibrary|MakePositionClaimerSavedPosition 0 (Variables|Default|GetTargetTag) "Self"))
  (Variables|Default|SetTargetActor (Class|ValueClaimerLibrary|MakeActorClaimerSavedActor 0 (Variables|Default|GetTargetTag)))
  (Variables|Default|SetTarget%20Chase%20Range (Class|ValueGetterLibrary|MakeSimpleFloat 0 (Variables|Default|GetChaseRangeValue)))
  (bind _returnvalue (Game|ConstructObjectfromClass "/Game/1_Core/Blueprints/Actions/Nodes/BehaviorNode/BP_BehaviorNode_AttackTarget.BP_BehaviorNode_AttackTarget_C" (Variables|Default|GetTargetActor) 0 0 0 0 0 (Utilities|Struct|MakeActionExecuteSettingContainer true true false true)))
  (bind _returnvalue_2 (Game|ConstructObjectfromClass "/Game/1_Core/Blueprints/Actions/Nodes/BehaviorNode/BP_BehaviorNode_AttackLocation.BP_BehaviorNode_AttackLocation_C" (Variables|Default|GetTargetDestination) (Variables|Default|GetTarget%20Chase%20Range) 0 0 0 0 (Utilities|Struct|MakeActionExecuteSettingContainer true true false true)))
  (bind _returnvalue_3 (Game|ConstructObjectfromClass :Class "/Game/1_Core/Blueprints/Actions/Nodes/SelectorNode/BP_SelectorNode_Single.BP_SelectorNode_Single_C" :Description "공격할 대상을 선택하세요" :CursorDescription "공격" :CursorType "Attack" :PositionEffect "/Game/1_Core/VisualEffects/Single/NS_MoveEffect.NS_MoveEffect" :InputTypes (Utilities|Array|MakeArray (Utilities|Struct|MakeSelectorInput "SingleTarget" _targettag _returnvalue) (Utilities|Struct|MakeSelectorInput "Position" _targettag _returnvalue_2)) :IndicatorNodes (Utilities|Array|MakeArray _returnvalue) :NextNode 0 :CanceledNode 0 :BlockedNode 0 :Settings (Utilities|Struct|MakeActionExecuteSettingContainer false true false false)))
  (Variables|Default|SetRootNode _returnvalue_3))

(fn ConstructionScript
  (|CallParentFunction))

(fn GetSimpleActionOrder
  (params (CurrentInput :type Input%20Package%20Structure%20%28by%20ref%29) (CurrentTarget :type Unit%20Action%20Component%20Object%20Reference))
  (bind _returnvalue (Actor|GetComponentbyClass (.mousehitactor CurrentInput) "/Script/WhiteCladWarriors.UnitMainComponent"))
  (Utilities|IsValid (.mousehitactor CurrentInput)
    (:Is%20Valid
      (Utilities|IsValid _returnvalue
        (:Is%20Valid
          (return (Utilities|Select :Index (Class|UnitMainComponent|GetAllyTypefromOperator _returnvalue (Class|Operator|GetLocalOperator)) :Normal 0 :Own 0 :Enemy 200 :Ally 0)))
        (:Is%20Not%20Valid
          _)))
    (:Is%20Not%20Valid
      _))
  (return 0))

(fn GetInspectorTargets
  (Utilities|Array|Add (LocalVariables|GetResult) self)
  (for _array_element (.selectedactors (Class|Operator|GetLocalInputPackage))
    (Utilities|IsValid (Actor|GetComponentbyClass _array_element "/Script/WhiteCladWarriors.UnitMainComponent")
      (:Is%20Valid
        (bind _returnvalue (Class|ActionSetting|GetAction (Class|UnitMainComponent|GetActionfromTag (Actor|GetComponentbyClass _array_element "/Script/WhiteCladWarriors.UnitMainComponent") "Attack")))
        (Utilities|IsValid _returnvalue
          (:Is%20Valid
            (Utilities|Array|AddUnique (LocalVariables|GetResult) _returnvalue))))))
  (return (LocalVariables|GetResult)))