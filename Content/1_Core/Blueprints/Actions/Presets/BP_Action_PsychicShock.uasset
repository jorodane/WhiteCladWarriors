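; BP_Action_PsychicShock is an action preset for a single-target damage attack.
; On BeginPlay it builds a behavior node tree, rooted in a selector that prompts the player to pick a target.
; The selection feeds a montage node that stops movement, focuses the target and plays a sped-up shot animation.
; Its "Shot" event triggers a linked damage sub-node, directed from the caster toward the target.
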(event EventBeginPlay
  (|CallParentFunction)
  (Variables|Default|SetAttackRadius (Class|ValueGetterLibrary|MakeSimpleFloat 0 5e+02))
  (Variables|Default|SetAttackDamage (Class|ValueGetterLibrary|MakeSimpleFloat 0 1e+01))
  (Variables|Default|SetTargetActor (Class|ValueClaimerLibrary|MakeActorClaimerSavedActor 0 (Variables|Default|GetTargetTag)))
  (bind _returnvalue (Game|ConstructObjectfromClass "/Game/1_Core/Blueprints/Actions/Nodes/BehaviorNode/BP_BehaviorNode_Damage.BP_BehaviorNode_Damage_C" (Variables|Default|GetTargetActor) (Variables|Default|GetAttackDamage) (Class|ValueClaimerLibrary|MakeDirectionClaimertoPosition 0 (Class|ValueClaimerLibrary|ClaimSelfPosition) (Class|ValueClaimerLibrary|MakePositionClaimerActorPosition 0 (Variables|Default|GetTargetActor) "Self")) 0 0 0 0 (Utilities|Struct|MakeActionExecuteSettingContainer false true false false true true)))
  (bind _returnvalue_2 (Game|ConstructObjectfromClass "/Game/1_Core/Blueprints/Actions/Nodes/BehaviorNode/BP_BehaviorNode_MontagePlay.BP_BehaviorNode_MontagePlay_C" (Utilities|Struct|MakeMontageEventInfo "/Game/1_Core/Animations/AM_SampleShotFloating_Montage.AM_SampleShotFloating_Montage" 0 2.0) (Variables|Default|GetTargetActor) 0 0 0 (Utilities|Map|MakeMap "Shot" (Utilities|Struct|MakeLinkedNodeInfo _returnvalue true)) (Utilities|Struct|MakeActionExecuteSettingContainer true true false true true true)))
  (bind _returnvalue_3 (Game|ConstructObjectfromClass :Class "/Game/1_Core/Blueprints/Actions/Nodes/SelectorNode/BP_SelectorNode_Single.BP_SelectorNode_Single_C" :Description "공격할 대상을 선택하세요" :CursorDescription "공격" :CursorType "Attack" :PositionEffect "/Game/1_Core/VisualEffects/Single/NS_MoveEffect.NS_MoveEffect" :InputTypes (Utilities|Array|MakeArray (Utilities|Struct|MakeSelectorInput "SingleTarget" (Variables|Default|GetTargetTag) _returnvalue_2)) :IndicatorNodes (Utilities|Array|MakeArray _returnvalue_2) :NextNode 0 :CanceledNode 0 :BlockedNode 0 :Settings (Utilities|Struct|MakeActionExecuteSettingContainer false true false false true true)))
  (Variables|Default|SetRootNode _returnvalue_3))

(fn ConstructionScript
  (|CallParentFunction))