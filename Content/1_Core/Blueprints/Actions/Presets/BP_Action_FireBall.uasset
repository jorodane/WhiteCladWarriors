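; Fireball action preset that builds its behavior node graph on BeginPlay from a player-selected throw direction.
; The caster turns to that direction and plays a shot montage; after a short delay, two parallel angle-shift repeaters sweep damaging projectiles inward from both sides.
; A follow-up repeater fires a short burst along the aim with slight random spread.
; The burst projectile also serves as the targeting indicator.
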(event EventBeginPlay
  (bind _returnvalue (Class|ValueClaimerLibrary|ClaimTriggerActor))
  (bind _returnvalue_2 (Class|ValueClaimerLibrary|MakePositionClaimerActorPosition 0 _returnvalue "Self"))
  (|CallParentFunction)
  (Variables|Default|SetThrowDirection (Class|ValueClaimerLibrary|MakeDirectionClaimerSavedDirection 0 (Class|ValueClaimerLibrary|MakePositionClaimerSelfPosition 0 "Self" (Class|ValueGetterLibrary|MakeSimpleVector 0 "0.000000,0.000000,20.000000")) "ThrowDirection"))
  (Variables|Default|SetRepeatDirection (Class|ValueClaimerLibrary|MakeDirectionClaimerSavedDirection 0 0 "ThrowDirection" (Class|ValueGetterLibrary|MakeRandomFloat 0 -5.0 5.0)))
  (Variables|Default|SetSpreadDirection (Class|ValueClaimerLibrary|MakeDirectionClaimerSavedDirection 0 0 "ShiftedDirection"))
  (Variables|Default|SetDamageValue (Class|ValueClaimerLibrary|MakeFloatClaimerSimpleFloat 0 (Class|ValueGetterLibrary|MakeSimpleFloat 0 15.0)))
  (bind _returnvalue_3 (Utilities|MakeProjectileHitDamage 0 "Projectile" (Variables|Default|GetHit%20Tag) "/Game/Projectiles_Spells_VFX/Effects/Projectile_18/Lvl_1/NS_Impact_18_Lvl_1.NS_Impact_18_Lvl_1" (Variables|Default|GetDamageValue) (Variables|Default|GetRepeatDirection) true))
  (bind _returnvalue_4 (Utilities|MakeSimpleProjectile 0 _returnvalue_3 5e+03 1.5e+03 7e+01 -1.0 (Variables|Default|GetRepeatDirection) _returnvalue_2 0 "/Game/Projectiles_Spells_VFX/Effects/Projectile_18/Lvl_1/NS_Projectile_18_Lvl_1.NS_Projectile_18_Lvl_1" (Variables|Default|GetHit%20Tag) "Projectile"))
  (Variables|Default|SetProjectile _returnvalue_4)
  (bind _returnvalue_5 (Utilities|MakeProjectileHitDamage 0 "Projectile" (Variables|Default|GetHit%20Tag) "/Game/Projectiles_Spells_VFX/Effects/Projectile_18/Lvl_1/NS_Impact_18_Lvl_1.NS_Impact_18_Lvl_1" (Variables|Default|GetDamageValue) (Variables|Default|GetSpreadDirection) true))
  (bind _returnvalue_6 (Utilities|MakeSimpleProjectile 0 _returnvalue_5 5e+03 1.5e+03 7e+01 -1.0 (Variables|Default|GetSpreadDirection) _returnvalue_2 0 "/Game/Projectiles_Spells_VFX/Effects/Projectile_18/Lvl_1/NS_Projectile_18_Lvl_1.NS_Projectile_18_Lvl_1" (Variables|Default|GetHit%20Tag) "Projectile"))
  (Utilities|FlowControl|Sequence
    (:then_0
      (bind _returnvalue_7 (Game|ConstructObjectfromClass "/Game/1_Core/Blueprints/Actions/Nodes/DelayNode/BP_RepeatNode.BP_RepeatNode_C" (Class|ValueClaimerLibrary|MakeFloatClaimerSimpleFloat 0 (Class|ValueGetterLibrary|MakeSimpleFloat 0 3.0)) (Variables|Default|GetProjectile) (Class|ValueClaimerLibrary|MakeFloatClaimerSimpleFloat 0 (Class|ValueGetterLibrary|MakeSimpleFloat 0 0.1)) (Utilities|Struct|MakeActionExecuteSettingContainer true true false false) 0 0 0)))
    (:then_1
      (bind _returnvalue_8 (Game|ConstructObjectfromClass :Class "/Game/1_Core/Blueprints/Actions/Nodes/DelayNode/BP_RepeatNode_ShiftAngle.BP_RepeatNode_ShiftAngle_C" :OriginDirection (Variables|Default|GetThrowDirection) :StartShiftAngle (Class|ValueClaimerLibrary|MakeFloatClaimerSimpleFloat 0 (Class|ValueGetterLibrary|MakeSimpleFloat 0 -9e+01)) :ShiftAngle (Class|ValueClaimerLibrary|MakeFloatClaimerSimpleFloat 0 (Class|ValueGetterLibrary|MakeSimpleFloat 0 5.0)) :ResultDirectionTag "ShiftedDirection" :RepeatTime (Class|ValueClaimerLibrary|MakeFloatClaimerSimpleFloat 0 (Class|ValueGetterLibrary|MakeSimpleFloat 0 18.0)) :RepeatNode _returnvalue_6 :Interval (Class|ValueClaimerLibrary|MakeFloatClaimerSimpleFloat 0 (Class|ValueGetterLibrary|MakeSimpleFloat 0 0.01)) :NextNode 0 :CanceledNode 0 :BlockedNode 0)))
    (:then_2
      (bind _returnvalue_9 (Game|ConstructObjectfromClass :Class "/Game/1_Core/Blueprints/Actions/Nodes/DelayNode/BP_RepeatNode_ShiftAngle.BP_RepeatNode_ShiftAngle_C" :OriginDirection (Variables|Default|GetThrowDirection) :StartShiftAngle (Class|ValueClaimerLibrary|MakeFloatClaimerSimpleFloat 0 (Class|ValueGetterLibrary|MakeSimpleFloat 0 9e+01)) :ShiftAngle (Class|ValueClaimerLibrary|MakeFloatClaimerSimpleFloat 0 (Class|ValueGetterLibrary|MakeSimpleFloat 0 -5.0)) :ResultDirectionTag "ShiftedDirection" :RepeatTime (Class|ValueClaimerLibrary|MakeFloatClaimerSimpleFloat 0 (Class|ValueGetterLibrary|MakeSimpleFloat 0 18.0)) :RepeatNode _returnvalue_6 :Interval (Class|ValueClaimerLibrary|MakeFloatClaimerSimpleFloat 0 (Class|ValueGetterLibrary|MakeSimpleFloat 0 0.01)) :NextNode 0 :CanceledNode 0 :BlockedNode 0)))
    (:then_3
      (bind _returnvalue_10 (Game|ConstructObjectfromClass "/Game/1_Core/Blueprints/Actions/Nodes/SimpleNode/Branchs/BP_SimpleNode_ParallelExecution.BP_SimpleNode_ParallelExecution_C" (Utilities|Array|MakeArray _returnvalue_8 _returnvalue_9) _returnvalue_7 0 0))
      (bind _returnvalue_11 (Game|ConstructObjectfromClass :Class "/Game/1_Core/Blueprints/Actions/Nodes/DelayNode/BP_DelayNode.BP_DelayNode_C" :Interval (Class|ValueGetterLibrary|MakeSimpleFloat 0 0.3) :NextNode _returnvalue_10 :CanceledNode 0 :BlockedNode 0))
      (bind _returnvalue_12 (Game|ConstructObjectfromClass "/Game/1_Core/Blueprints/Actions/Nodes/BehaviorNode/BP_BehaviorNode_MontagePlay.BP_BehaviorNode_MontagePlay_C" (Utilities|Struct|MakeMontageEventInfo "/Game/1_Core/Animations/AM_SampleShotFloating_Montage.AM_SampleShotFloating_Montage" 0 2.0) 0 _returnvalue_11 true (Utilities|Struct|MakeActionExecuteSettingContainer true true true false) 0 0 0))
      (bind _returnvalue_13 (Game|ConstructObjectfromClass :Class "/Game/1_Core/Blueprints/Actions/Nodes/BehaviorNode/BP_BehaviorNode_LookAt.BP_BehaviorNode_LookAt_C" :LookDirection (Variables|Default|GetThrowDirection) :NextNode _returnvalue_12 :CanceledNode 0 :BlockedNode 0))
      (bind _returnvalue_14 (Game|ConstructObjectfromClass "/Game/1_Core/Blueprints/Actions/Nodes/SelectorNode/BP_SelectorNode_Single.BP_SelectorNode_Single_C" 0 "파이어볼을 발사할 방향을 정해주세요" "" "Target" "/Game/1_Core/VisualEffects/Single/NS_MoveEffect.NS_MoveEffect" (Utilities|Struct|MakeMontageEventInfo "/Game/1_Core/Animations/AM_PrepareShooting.AM_PrepareShooting") (Utilities|Array|MakeArray (Utilities|Struct|MakeSelectorInput "Direction" "ThrowDirection" _returnvalue_13)) (Utilities|Array|MakeArray (Variables|Default|GetProjectile)) false 0 0 0))
      (Variables|Default|SetRootNode _returnvalue_14))))

(fn ConstructionScript
  (|CallParentFunction))