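; Blueprint function library that supplies camera control tuning values as hardcoded constants.
; It has separate getters for keyboard, screen-edge and mouse move speeds, zoom speed with minimum and maximum limits, and rotation speed, multiplier and start length.
; Each function simply returns a fixed float, with no stored state or saved user settings behind it.
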(fn GetCameraMoveSpeedKeyboard
  (return 6e+01))

(fn GetCameraMoveSpeedEdge
  (return 6e+03))

(fn GetCameraMoveSpeedMouse
  (return 2e+04))

(fn GetCameraZoomSpeed
  (return 5e+01))

(fn GetCameraZoomLimitMin
  (return 2e+02))

(fn GetCameraZoomLimitMax
  (return 9e+03))

(fn GetCameraRotateSpeed
  (return 3.6e+02))

(fn GetCameraRotateMultiply
  (return 0.5))

(fn GetCameraRotateStartLength
  (params (__WorldContext :type Object%20Object%20Reference))
  (return 3.6e+02))