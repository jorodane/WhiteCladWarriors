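; Function library of viewport and UI helpers for mouse position, click detection, world-to-screen projection, visibility tests and info widget building.
; Visibility checks project actor locations through view-projection matrices and range-test the perspective-divided result.
; ClaimInfoWidgetsFromActor passes an actor's widget claims to ClaimWidgets, which adds generic widgets sorted by UIOrder to a panel, then any others.
; CreateInfoWidget resolves classes through DT_GenericWidget and recursively attaches child widgets.
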(fn GetMousePositiononViewport
  (bind _returnvalue (Viewport|GetViewportSize))
  (bind _returnvalue_2 (Class|WidgetLayoutLibrary|GetMousePositiononViewport))
  (return (Math|Vector2D|MakeVector2D (.x (- (/ (* _returnvalue_2 (Class|WidgetLayoutLibrary|GetViewportScale)) _returnvalue) "(X=0.500000,Y=0.500000)")) (* (.y (- (/ (* _returnvalue_2 (Class|WidgetLayoutLibrary|GetViewportScale)) _returnvalue) "(X=0.500000,Y=0.500000)")) -1.0)) (* _returnvalue_2 (Class|WidgetLayoutLibrary|GetViewportScale)) _returnvalue))

(fn IsMouseClick
  (params (SquaredLength :type Float%20%28double-precision%29) (DownPosition :type Vector) (UpPosition :type Vector))
  (return (< (Class|KismetMathLibrary|VSizeXYSquared (- DownPosition UpPosition)) SquaredLength)))

(fn IsVisibleonViewport
  (params (Camera :type Camera%20Component%20Object%20Reference) (Target :type Actor%20Object%20Reference))
  (bind _desiredview (Class|CameraComponent|GetCameraView Camera 0.0))
  (return (Math|Boolean|ANDBoolean (Math|Float|InRange(Float) (/ (.x (Class|KismetMathLibrary|MatrixTransformPosition (.ViewProjectionMatrix (Class|GameplayStatics|GetViewProjectionMatrix _desiredview)) (Transformation|GetActorLocation Target))) (.w (Class|KismetMathLibrary|MatrixTransformPosition (.ViewProjectionMatrix (Class|GameplayStatics|GetViewProjectionMatrix _desiredview)) (Transformation|GetActorLocation Target)))) -1.0 1.0) (Math|Float|InRange(Float) (/ (.y (Class|KismetMathLibrary|MatrixTransformPosition (.ViewProjectionMatrix (Class|GameplayStatics|GetViewProjectionMatrix _desiredview)) (Transformation|GetActorLocation Target))) (.w (Class|KismetMathLibrary|MatrixTransformPosition (.ViewProjectionMatrix (Class|GameplayStatics|GetViewProjectionMatrix _desiredview)) (Transformation|GetActorLocation Target)))) -1.0 1.0) (Math|Float|InRange(Float) (/ (.z (Class|KismetMathLibrary|MatrixTransformPosition (.ViewProjectionMatrix (Class|GameplayStatics|GetViewProjectionMatrix _desiredview)) (Transformation|GetActorLocation Target))) (.w (Class|KismetMathLibrary|MatrixTransformPosition (.ViewProjectionMatrix (Class|GameplayStatics|GetViewProjectionMatrix _desiredview)) (Transformation|GetActorLocation Target)))) -1.0 1.0) (> (.w (Class|KismetMathLibrary|MatrixTransformPosition (.ViewProjectionMatrix (Class|GameplayStatics|GetViewProjectionMatrix _desiredview)) (Transformation|GetActorLocation Target))) 0.0))))

(fn IsVisibleonProjectionMatrix
  (params (Matrix :type Matrix%20Structure%20%28by%20ref%29) (Target :type Actor%20Object%20Reference))
  (bind _returnvalue (Math|Vector2D|MakeVector2D -1.2 1.2))
  (bind _returnvalue_2 (Transformation|GetActorLocation Target))
  (bind _returnvalue_3 (Class|KismetMathLibrary|MatrixTransformPosition Matrix _returnvalue_2))
  (return (Math|Boolean|ANDBoolean (Math|Float|InRange(Float) (/ (.x _returnvalue_3) (.w _returnvalue_3)) (.x _returnvalue) (.y _returnvalue)) (Math|Float|InRange(Float) (/ (.y _returnvalue_3) (.w _returnvalue_3)) (.x _returnvalue) (.y _returnvalue)) (Math|Float|InRange(Float) (/ (.z _returnvalue_3) (.w _returnvalue_3)) (.x _returnvalue) (.y _returnvalue)) (> (.w _returnvalue_3) 0.0))))

(fn GetScreentoLocalOffset
  (params (ScreenPos :type Vector%202D%20Structure) (Geometry :type Geometry%20Structure))
  (bind _returnvalue (Class|SlateBlueprintLibrary|GetLocalSize Geometry))
  (return (/ (- ScreenPos (Class|SlateBlueprintLibrary|LocaltoAbsolute Geometry (* _returnvalue 0.5))) _returnvalue)))

(fn ClaimWidgets
  (params (Claim :type BPS%20Widget%20Claimer%20Structure) (InfoType :type EInfoWidgetType%20Enum :default "Minimal"))
  (LocalVariables|SetCurrentType InfoType)
  (Utilities|FlowControl|Sequence
    (:then_0
      (bind _output_get (LocalVariables|SetCurrentClaim Claim))
      (for _array_element (.claimwidgets _output_get)
        (Utilities|IsValid _array_element
          (:Is%20Valid
            (bind (_result _uiorder) (CallFunction|CreateInfoWidget _array_element (LocalVariables|GetCurrentType) (.claimer _output_get)))
            (Utilities|IsValid _result
              (:Is%20Valid
                (bind _output_get_2 (LocalVariables|SetCurrentCreatedWidget _result))
                (bind _aswb_generic_widget_base (Utilities|Casting|CastToWB_GenericWidgetBase _output_get_2)
                  (:then
                    (LocalVariables|SetCurrentCreatedGeneric _aswb_generic_widget_base)
                    (LocalVariables|SetCurrentOrder _uiorder)
                    (if (Utilities|Array|IsEmpty (LocalVariables|GetCreatedWidgets_Ordered))
                      (Utilities|Array|Add (LocalVariables|GetCreatedWidgets_Ordered) (LocalVariables|GetCurrentCreatedGeneric) :!label _label)
                      (else
                        (LocalVariables|SetAdded false)
                        (bind (_array_element_2 _array_index) (Utilities|Array|ForEachLoopwithBreak (LocalVariables|GetCreatedWidgets_Ordered) :!label _label_2)
                          (:LoopBody
                            (Utilities|IsValid _array_element_2
                              (:Is%20Valid
                                (if (> (Variables|/Game/1_Core/Widgets/Generics/WB_GenericWidgetBase.WB_GenericWidgetBase_C|GetUIOrder _array_element_2) (LocalVariables|GetCurrentOrder))
                                  (Utilities|Array|Insert (LocalVariables|GetCreatedWidgets_Ordered) (LocalVariables|GetCurrentCreatedGeneric) _array_index :!label _label_3)
                                  (LocalVariables|SetAdded true)
                                  (goto _label_2 Break)))
                              (:Is%20Not%20Valid
                                (goto _label_3))))
                          (:Completed
                            (if (not (LocalVariables|GetAdded))
                              (goto _label)))))))
                  (:CastFailed
                    (Utilities|Array|AddUnique (LocalVariables|GetCreatedWidgets) (LocalVariables|GetCurrentCreatedWidget))))))))))
    (:then_1
      (for _array_element_3 (LocalVariables|GetCreatedWidgets_Ordered)
        (Widget|Panel|AddChild (.claimedpanel (LocalVariables|GetCurrentClaim)) _array_element_3))
      (for _array_element_4 (LocalVariables|GetCreatedWidgets)
        (Widget|Panel|AddChild (.claimedpanel (LocalVariables|GetCurrentClaim)) _array_element_4)))))

(fn ClearWidgetList
  (params (TargetList :type Panel%20Widget%20Object%20Reference))
  (while (> (Class|PanelWidget|GetChildrenCount TargetList) 0)
    (Class|PanelWidget|RemoveChildat TargetList)))

(fn ClaimInfoWidgetsfromActor
  (params (GoalPanel :type Vertical%20Box%20Object%20Reference) (타깃 :type Object%20Object%20Reference) (WantType :type EInfoWidgetType%20Enum :default "Minimal"))
  (LocalVariables|SetCurrentPanel GoalPanel)
  (LocalVariables|SetCurrentTarget 타깃)
  (bind _output_get (LocalVariables|SetCurrentType WantType))
  (bind _returnvalue (Class|InfoConnectable|GetInfoWidget(Message) (LocalVariables|GetCurrentTarget) _output_get))
  (CallFunction|ClaimWidgets (Utilities|Struct|MakeBPS_WidgetClaimer _returnvalue (LocalVariables|GetCurrentPanel) (LocalVariables|GetCurrentTarget)) (LocalVariables|GetCurrentType)))

(fn GetWorldtoScreenPosition
  (params (WorldPosition :type Vector%20%28by%20ref%29))
  (bind _returnvalue (Class|GameplayStatics|GetPlayerControllerfromID))
  (bind (_screenposition _returnvalue_2) (Class|GameplayStatics|ProjectWorldtoScreen _returnvalue WorldPosition true))
  (return (/ _screenposition (Class|WidgetLayoutLibrary|GetViewportScale)) _returnvalue_2))

(fn CreateInfoWidget
  (params (Claimer :type Generic%20Widget%20Claim%20Object%20Reference) (InfoType :type EInfoWidgetType%20Enum :default "Minimal") (Instigator :type Object%20Object%20Reference))
  (bind _output_get (LocalVariables|SetCurrentClaim Claimer))
  (bind _asordered_generic_widget_claim (Utilities|Casting|CastToOrderedGenericWidgetClaim _output_get)
    (:then
      (LocalVariables|SetCurrentOrder (Variables|/Script/WhiteCladWarriors.OrderedGenericWidgetClaim|GetUIOrder _asordered_generic_widget_claim)))
    (:CastFailed
      _))
  (LocalVariables|SetCurrentWidgetType (Variables|/Script/WhiteCladWarriors.GenericWidgetClaim|GetWidgetType (LocalVariables|GetCurrentClaim)))
  (LocalVariables|SetCurrentInfoType InfoType)
  (LocalVariables|SetCurrentObject Instigator)
  (LocalVariables|SetCurrentChildren (Variables|/Script/WhiteCladWarriors.GenericWidgetClaim|GetChildren (LocalVariables|GetCurrentClaim)))
  (bind _returnvalue (Class|DataTableFunctionLibrary|DoesDataTableRowExist "/Game/1_Core/DataTables/DT_GenericWidget.DT_GenericWidget" (LocalVariables|GetCurrentWidgetType)))
  (if _returnvalue
    (bind _returnvalue_2 (Utilities|GetDataTableRow "/Game/1_Core/DataTables/DT_GenericWidget.DT_GenericWidget" (LocalVariables|GetCurrentWidgetType))
      (:then
        (bind _returnvalue_3 (UserInterface|CreateWidget (.widgetclass _returnvalue_2) 0 (LocalVariables|GetCurrentOrder)))
        (Utilities|IsValid _returnvalue_3
          (:Is%20Valid
            (bind _output_get_2 (LocalVariables|SetCurrentWidget _returnvalue_3))
            (Default|OnConnected _output_get_2 (LocalVariables|GetCurrentClaim))
            (for _array_element (LocalVariables|GetCurrentChildren)
              (bind _result (CallFunction|CreateInfoWidget _array_element (LocalVariables|GetCurrentInfoType) (LocalVariables|GetCurrentObject)))
              (Utilities|IsValid _result
                (:Is%20Valid
                  (Default|AddChildWidget (LocalVariables|GetCurrentWidget) _result))))
            (return (LocalVariables|GetCurrentWidget) (LocalVariables|GetCurrentOrder)))
          (:Is%20Not%20Valid
            _)))
      (:RowNotFound
        _))
    (return (LocalVariables|GetCurrentWidget) (LocalVariables|GetCurrentOrder))))