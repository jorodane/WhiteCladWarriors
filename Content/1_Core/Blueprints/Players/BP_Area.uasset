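; BP_Area is a base for area selection that gathers the selectable actors inside an area for a given operator.
; GetObjectsInArea takes hits from HitTraceArea, asks each valid hit actor whether that operator can select it, and collects unique matches.
; It also returns an AllTheSame flag by comparing each match's class with the first one found.
; HitTraceArea is an empty stub here, so this file defines no trace shape.
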(event EventBeginPlay)

(event EventTick
  (params (DeltaSeconds :type Float%20%28single-precision%29)))

(fn ConstructionScript)

(fn GetObjectsinArea
  (params (Operator :type Operator%20Object%20Reference))
  (bind _results (CallFunction|HitTraceArea))
  (for _array_element _results
    (Utilities|IsValid (.HitActor (Collision|BreakHitResult _array_element))
      (:Is%20Valid
        (Class|Selectable|IsSelectable(Message) (.HitActor (Collision|BreakHitResult _array_element)) Operator
          (:True
            (Utilities|Array|AddUnique (LocalVariables|GetResultArray) (.HitActor (Collision|BreakHitResult _array_element)))
            (bind _lastactorclass (LocalVariables|GetLastActorClass)
              (:then
                (LocalVariables|SetAllSame (and (== _lastactorclass (Utilities|GetClass (.HitActor (Collision|BreakHitResult _array_element)))) (LocalVariables|GetAllSame))))
              (:else
                (LocalVariables|SetLastActorClass (Utilities|GetClass (.HitActor (Collision|BreakHitResult _array_element)))))))))))
  (return (LocalVariables|GetResultArray) (LocalVariables|GetAllSame)))

(fn HitTraceArea
  (return 0))