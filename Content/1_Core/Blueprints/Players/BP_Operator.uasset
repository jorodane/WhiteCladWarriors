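; BP_Operator is an RTS-style player pawn that handles camera control and object selection, setting up input and the in-game widget when possessed.
; Tick traces under the cursor for terrain position and hover messages, and drives edge scroll and speed-capped middle-mouse panning.
; Left-click or a world-space BP_AreaSquare drag sends select/deselect messages, with Shift for additive selection.
; Ctrl-click or double-click selects on-screen same-class actors via view-projection matrix.
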(event Input|EnhancedActionEvents|EnhancedInputActionIA_MouseLeft
  (params (ActionValue :type Boolean) (ElapsedSeconds :type Float%20%28double-precision%29) (TriggeredSeconds :type Float%20%28double-precision%29) (InputAction :type Input%20Action%20Object%20Reference :default "/Game/1_Core/Inputs/IA_MouseLeft.IA_MouseLeft"))
  (bind _mouseterrainposition (Variables|Default|GetMouseTerrainPosition))
  ;[0.15 0.15 0.15 0.5] Click
  (:Triggered
    (CallFunction|DrawDragArea (Variables|Default|GetDragStartPosition) _mouseterrainposition))
  (:Started
    (Variables|Default|SetDragStartPosition _mouseterrainposition)
    (bind _dragarea (Variables|Default|GetDragArea)
      (:then
        (Rendering|SetActorHiddenInGame _dragarea (not ActionValue) :!label _label))
      (:else)))
  (:Completed
    (Utilities|FlowControl|Sequence
      (:then_0
        (CallFunction|ClickTrigger))
      (:then_1
        (goto _label)))))

(event Input|EnhancedActionEvents|EnhancedInputActionIA_Zoom
  (params (ActionValue :type Float%20%28double-precision%29) (ElapsedSeconds :type Float%20%28double-precision%29) (TriggeredSeconds :type Float%20%28double-precision%29) (InputAction :type Input%20Action%20Object%20Reference :default "/Game/1_Core/Inputs/IA_Zoom.IA_Zoom"))
  ;[0.15 0.15 0.15 0.5] Zoom
  (Class|Operator|CameraZoom ActionValue (CallFunction|GetCameraZoomLimitMin) (CallFunction|GetCameraZoomLimitMax) (CallFunction|GetCameraZoomSpeed)))

(event Input|EnhancedActionEvents|EnhancedInputActionIA_Shift
  (params (ActionValue :type Boolean) (ElapsedSeconds :type Float%20%28double-precision%29) (TriggeredSeconds :type Float%20%28double-precision%29) (InputAction :type Input%20Action%20Object%20Reference :default "/Game/1_Core/Inputs/IA_Shift.IA_Shift"))
  ;[0.15 0.15 0.15 0.5] SimpleInput
  (:Started
    (Variables|Default|SetAdditiveMode ActionValue :!label _label))
  (:Completed
    (goto _label)))

(event Input|EnhancedActionEvents|EnhancedInputActionIA_KeyboardArrow
  (params (ActionValue :type Vector%202D%20Structure) (ElapsedSeconds :type Float%20%28double-precision%29) (TriggeredSeconds :type Float%20%28double-precision%29) (InputAction :type Input%20Action%20Object%20Reference :default "/Game/1_Core/Inputs/IA_KeyboardArrow.IA_KeyboardArrow"))
  ;[0.15 0.15 0.15 0.5] CameraMove By Keyboard
  (Class|Operator|CameraMove ActionValue (CallFunction|GetCameraMoveSpeedKeyboard)))

(event Input|EnhancedActionEvents|EnhancedInputActionIA_MouseWheelButton
  (params (ActionValue :type Boolean) (ElapsedSeconds :type Float%20%28double-precision%29) (TriggeredSeconds :type Float%20%28double-precision%29) (InputAction :type Input%20Action%20Object%20Reference :default "/Game/1_Core/Inputs/IA_MouseWheelButton.IA_MouseWheelButton"))
  (bind _playercontoller (Variables|Default|GetPlayerContoller))
  (bind (_locationx _locationy) (Game|Player|GetMousePosition _playercontoller))
  ;[0.15 0.15 0.15 0.5] SimpleInput
  (:Started
    (Variables|Default|SetMouseWheel true)
    (Variables|Default|SetWheelStartPosition (Math|Vector2D|MakeVector2D _locationx _locationy))
    (Variables|/Script/Engine.PlayerController|SetbShowMouseCursor (Variables|Default|GetPlayerContoller) (not (Variables|Default|GetMouseWheel)) :!label _label))
  (:Completed
    (Variables|Default|SetMouseWheel false)
    (goto _label)))

(event Input|EnhancedActionEvents|EnhancedInputActionIA_Control
  (params (ActionValue :type Boolean) (ElapsedSeconds :type Float%20%28double-precision%29) (TriggeredSeconds :type Float%20%28double-precision%29) (InputAction :type Input%20Action%20Object%20Reference :default "/Game/1_Core/Inputs/IA_Control.IA_Control"))
  ;[0.15 0.15 0.15 0.5] SimpleInput
  (:Started
    (Variables|Default|SetSelectAllMode ActionValue :!label _label))
  (:Completed
    (goto _label)))

(event EventSetCameraLength
  (params (Value :type Float%20%28single-precision%29))
  ;[0.15 0.15 0.15 0.5] Zoom
  (|CallParentFunction Value)
  (Variables|/Script/Engine.SpringArmComponent|SetTargetArmLength (Variables|Default|GetCameraArm) Value))

(event EventTick
  (params (DeltaSeconds :type Float%20%28single-precision%29))
  (bind (_offset _position _viewportsize) (CallFunction|GetMousePositiononViewport))
  (bind _result (CallFunction|GetCameraMoveSpeedWheel))
  (bind _wheelstartposition (Variables|Default|GetWheelStartPosition))
  (bind _playercontoller (Variables|Default|GetPlayerContoller))
  (bind _playercontoller_2 (Variables|Default|GetPlayerContoller))
  (bind _hitresult (Game|Player|GetHitResultUnderCursorbyChannel _playercontoller_2 "TraceTypeQuery3" false))
  (bind (_locationx _locationy) (Game|Player|GetMousePosition _playercontoller))
  (bind _returnvalue (* _result DeltaSeconds))
  (bind _hitactor (Collision|BreakHitResult _hitresult))
  (Utilities|FlowControl|Sequence
    (:then_0
      (bind _playercontoller_3 (Variables|Default|GetPlayerContoller)
        (:then
          (Variables|Default|SetMouseTerrainPosition (.Location (Collision|BreakHitResult (.HitResult (Game|Player|GetHitResultUnderCursorbyChannel _playercontoller_3 "TraceTypeQuery4" false)))))
          (if (!= (Variables|Default|GetMouseHitActor) _hitactor)
            (bind _mousehitactor (Variables|Default|GetMouseHitActor)
              (:then
                (Class|Selectable|MouseHoverEnd(Message) _mousehitactor))
              (:else
                _))
            (bind _output_get (Variables|Default|SetMouseHitActor _hitactor))
            (Utilities|IsValid _output_get
              (:Is%20Valid
                (Class|Selectable|MouseHoverBegin(Message) _output_get))
              (:Is%20Not%20Valid
                _)))
          (if (Variables|Default|GetMouseWheel)
            (Variables|Default|SetClaimedWheelMove (+ (Variables|Default|GetClaimedWheelMove) (Math|Vector|MakeVector (- _locationx (.x _wheelstartposition)) (- (.y _wheelstartposition) _locationy) 0.0)))
            (Class|PlayerController|SetMouseLocation (Variables|Default|GetPlayerContoller) (Math|Float|Truncate (.x _wheelstartposition)) (Math|Float|Truncate (.y _wheelstartposition)))
            (else
              (Variables|Default|SetCurrentMousePosition _position)
              (Variables|Default|SetCurrentViewportSize _viewportsize)
              (Class|Operator|EdgeScroll (Variables|Default|GetCurrentMousePosition) (Variables|Default|GetCurrentViewportSize) (* (CallFunction|GetCameraMoveSpeedEdge) DeltaSeconds)))))
        (:else)))
    (:then_1
      (if (> (Math|Vector|VectorLength (Variables|Default|GetClaimedWheelMove)) 0.0)
        (Class|Operator|CameraMove (Math|Vector2D|MakeVector2D (.X (Math|Vector|BreakVector (Math|Vector|SelectVector (* (Math|Vector|Normalize (Variables|Default|GetClaimedWheelMove)) _returnvalue) (Variables|Default|GetClaimedWheelMove) (> (Math|Vector|VectorLength (Variables|Default|GetClaimedWheelMove)) _returnvalue)))) (.Y (Math|Vector|BreakVector (Math|Vector|SelectVector (* (Math|Vector|Normalize (Variables|Default|GetClaimedWheelMove)) _returnvalue) (Variables|Default|GetClaimedWheelMove) (> (Math|Vector|VectorLength (Variables|Default|GetClaimedWheelMove)) _returnvalue))))) _returnvalue)
        (Variables|Default|SetClaimedWheelMove (- (Variables|Default|GetClaimedWheelMove) (Math|Vector|SelectVector (* (Math|Vector|Normalize (Variables|Default|GetClaimedWheelMove)) _returnvalue) (Variables|Default|GetClaimedWheelMove) (> (Math|Vector|VectorLength (Variables|Default|GetClaimedWheelMove)) _returnvalue))))))))

(event EventPossessed
  (params (NewController :type Controller%20Object%20Reference))
  ;[0.15 0.15 0.15 0.5] Control Link
  (CallFunction|InitiateController NewController)
  (CallFunction|CreateIngameWidget (Variables|Default|GetPlayerContoller))
  (CallFunction|InitiateDragArea))

(event EventUnpossessed
  (params (OldController :type Controller%20Object%20Reference))
  ;[0.15 0.15 0.15 0.5] Control Link
  (Utilities|FlowControl|Sequence
    (:then_0
      (bind _as플레이어_컨트롤러 (Utilities|Casting|CastToPlayerController OldController))
      (Input|RemoveMappingContext _as플레이어_컨트롤러 "/Game/1_Core/Inputs/IMC_Operator.IMC_Operator" "(bIgnoreAllPressedKeysUntilRelease=True,bForceImmediately=False,bNotifyUserSettings=False)"))
    (:then_1
      (bind _dragarea (Variables|Default|GetDragArea)
        (:then
          (Rendering|SetActorHiddenInGame _dragarea true))
        (:else)))
    (:then_2
      (CallFunction|DeselectObjects)
      (bind _mousehitactor (Variables|Default|GetMouseHitActor)
        (:then
          (Class|Selectable|MouseHoverEnd(Message) _mousehitactor)
          (Variables|Default|SetMouseHitActor 0))
        (:else)))))

(fn ConstructionScript)

(fn CreateIngameWidget
  (params (OwningPlayer :type Player%20Controller%20Object%20Reference))
  (bind _returnvalue (UserInterface|CreateWidget "/Game/1_Core/Blueprints/Widgets/WB_Ingame.WB_Ingame_C" OwningPlayer))
  (bind _output_get (Variables|Default|SetIngameWidget _returnvalue))
  (Default|PlayerConnect _output_get self)
  (UserInterface|Viewport|AddtoPlayerScreen (Variables|Default|GetIngameWidget))
  (return (Variables|Default|GetIngameWidget)))

(fn SetInputModeDefault
  (bind _playercontoller (Variables|Default|GetPlayerContoller)
    (:then
      (Input|SetInputModeGameandUI _playercontoller 0 "LockAlways" false true))
    (:else)))

(fn InitiateDragArea
  (bind _self self)
  (Variables|Default|GetDragArea
    (:then)
    (:else
      (bind _returnvalue (Game|SpawnActorfromClass "/Game/1_Core/Blueprints/Players/BP_AreaSquare.BP_AreaSquare_C" (Math|Transform|MakeTransform "0, 0, 0" "-90.000000,0.000000,0.000000" "1.000000,1.000000,1.000000") "Undefined" "MultiplyWithRoot" _self _self))
      (bind _output_get (Variables|Default|SetDragArea _returnvalue))
      (Rendering|SetActorHiddenInGame _output_get true))))

(fn InitiateController
  (params (NewController :type Controller%20Object%20Reference))
  (bind (_as플레이어_컨트롤러 _bsuccess) (Utilities|Casting|CastToPlayerController NewController))
  (if (and (Pawn|IsLocalPlayerController NewController) _bsuccess)
    (Variables|Default|SetPlayerContoller _as플레이어_컨트롤러)
    (Input|AddMappingContext (PlayerController|LocalPlayerSubsystems|GetEnhancedInputLocalPlayerSubsystem (Variables|Default|GetPlayerContoller)) "/Game/1_Core/Inputs/IMC_Operator.IMC_Operator" 0 "(bIgnoreAllPressedKeysUntilRelease=True,bForceImmediately=False,bNotifyUserSettings=False)")
    (CallFunction|SetInputModeDefault)))

(fn SelectObjects
  (params (ObjectArray :type Array%20of%20Actor%20Object%20References) (bIsSingleSelection :type Boolean))
  (for _array_element ObjectArray
    (CallFunction|SelectObject _array_element bIsSingleSelection)))

(fn SelectObject
  (params (Target :type Actor%20Object%20Reference) (SingleSelect :type Boolean))
  (Utilities|Array|AddUnique (Variables|Default|GetSelectedActors) Target)
  (Class|Selectable|Select(Message) Target self SingleSelect))

(fn DeselectObjects
  (bind _selectedactors (Variables|Default|GetSelectedActors))
  (for _array_element _selectedactors
    (Class|Selectable|Deselect(Message) _array_element))
  (Utilities|Array|Clear _selectedactors))

(fn DeselectObject
  (params (Target :type Actor%20Object%20Reference))
  (bind _returnvalue (Utilities|Array|RemoveItem (Variables|Default|GetSelectedActors) Target))
  (if _returnvalue
    (Class|Selectable|Deselect(Message) Target)))

(fn SelectToggle
  (params (Target :type Actor%20Object%20Reference))
  (LocalVariables|SetCurrentTarget Target)
  (if (Utilities|Array|ContainsItem (Variables|Default|GetSelectedActors) Target)
    (CallFunction|DeselectObject (LocalVariables|GetCurrentTarget))
    (else
      (CallFunction|SelectObject (LocalVariables|GetCurrentTarget) true))))

(fn DrawDragArea
  (params (Begin :type Vector) (End :type Vector))
  (bind _returnvalue (- Begin End))
  (bind _dragarea (Variables|Default|GetDragArea))
  (bind _returnvalue_2 (Math|Vector|VectorGetAbs _returnvalue))
  (bind _returnvalue_3 (/ _returnvalue_2 2.0))
  (Transformation|SetActorLocation _dragarea (/ (+ Begin End) 2.0) false false)
  (Transformation|SetActorScale3D _dragarea (Math|Vector|MakeVector 1e+04 (.y _returnvalue_3) (.x _returnvalue_3)))
  (Rendering|SetActorHiddenInGame _dragarea false))

(fn GetFocusObjects
  (params (IsClick :type Boolean) (IsDoubleClick :type Boolean))
  (Utilities|FlowControl|Sequence
    (:then_0
      (if IsClick
        (bind _mousehitactor (Variables|Default|GetMouseHitActor)
          (:then
            (if (or (Variables|Default|GetSelectAllMode) IsDoubleClick)
              (bind _result (CallFunction|GetVisibleSameObjects _mousehitactor))
              (LocalVariables|SetContainer _result)
              (bind _output_get (LocalVariables|SetNumValid (> (Utilities|Array|Length (stale _output_get_2)) 0) :!label _label))
              (if _output_get
                (LocalVariables|SetSingle (Utilities|Array|Get(acopy) (LocalVariables|GetContainer))))
              (else
                (Utilities|Array|Add (LocalVariables|GetContainer) _mousehitactor)
                (LocalVariables|SetAllSame true)
                (LocalVariables|SetOnlySingle true)
                (LocalVariables|SetSingle _mousehitactor)
                (LocalVariables|SetNumValid true))))
          (:else))
        (else
          (bind _dragarea (Variables|Default|GetDragArea)
            (:then
              (bind (_result_2 _allthesame _singleselect) (Default|GetObjectsinArea _dragarea self))
              (LocalVariables|SetAllSame _allthesame)
              (LocalVariables|SetOnlySingle _singleselect)
              (bind _output_get_2 (LocalVariables|SetContainer _result_2))
              (goto _label))
            (:else)))))
    (:then_1
      (return (LocalVariables|GetNumValid) (LocalVariables|GetContainer) (LocalVariables|GetSingle) (LocalVariables|GetAllSame) (LocalVariables|GetOnlySingle)))))

(fn GetVisibleSameObjects
  (params (Template :type Actor%20Object%20Reference))
  (Utilities|IsValid Template
    (:Is%20Valid
      (bind _desiredview (Class|CameraComponent|GetCameraView (Variables|Default|GetCameraMain) 0.0))
      (LocalVariables|SetCurrentMatrix (.ViewProjectionMatrix (Class|GameplayStatics|GetViewProjectionMatrix _desiredview)))
      (bind _outactors (Actor|GetAllActorsOfClass (Utilities|GetClass Template)))
      (for _array_element _outactors
        (if (CallFunction|IsVisibleonProjectionMatrix (LocalVariables|GetCurrentMatrix) _array_element)
          (Utilities|Array|Add (LocalVariables|GetResultArray) _array_element)))
      (return (LocalVariables|GetResultArray)))))

(fn ClickTrigger
  (bind _returnvalue (Utilities|Time|GetTimeSeconds))
  (bind _mouseterrainposition (Variables|Default|GetMouseTerrainPosition))
  (bind _dragstartposition (Variables|Default|GetDragStartPosition))
  (bind _mousehitactor (Variables|Default|GetMouseHitActor))
  (bind _returnvalue_2 (CallFunction|IsMouseClick 8e+02 _dragstartposition _mouseterrainposition))
  (LocalVariables|SetDoubleClicked (Math|Boolean|ANDBoolean (< (- _returnvalue (Variables|Default|GetLastSelectSeconds)) 0.3) (== (Variables|Default|GetMouseClickedActor) _mousehitactor) (Utilities|IsValid _mousehitactor)))
  (Variables|Default|SetLastSelectSeconds _returnvalue)
  (Variables|Default|SetMouseClickedActor (Variables|Default|GetMouseHitActor))
  (bind (_valid _resultarray _resultsingle _allthesame _singleselect) (CallFunction|GetFocusObjects _returnvalue_2 (LocalVariables|GetDoubleClicked)))
  (if _valid
    (if (Variables|Default|GetAdditiveMode)
      (if _returnvalue_2
        (if (or (Variables|Default|GetSelectAllMode) (LocalVariables|GetDoubleClicked))
          (CallFunction|SelectObjects _resultarray _singleselect :!label _label)
          (else
            (CallFunction|SelectToggle _resultsingle)))
        (else
          (goto _label)))
      (else
        (CallFunction|DeselectObjects)
        (goto _label)))
    (elif (not (Variables|Default|GetAdditiveMode))
      (CallFunction|DeselectObjects))))